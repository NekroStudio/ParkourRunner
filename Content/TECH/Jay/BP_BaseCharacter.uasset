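; Base player character for a parkour game, routing movement, jump, crouch/slide, mantle and grapple inputs to parkour and grapple components.
; Timelines drive crouch height, camera tilt and mantling, while slide jumps launch with speed-scaled height.
; Limited air dashes follow the camera; holding the key slows time with a tinted fade until release or timeout.
; Any damage kills, ramping time down and saving death count and phantom-runner data until checkpoint respawn.
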(event Custom|ResetDashes
  (bind _numberofdashes (Variables|DashVariables|GetNumberOfDashes))
  (bind _charactermovement (Variables|Character|GetCharacterMovement))
  ;[0 0.2846 1] Dash functionality
  (Utilities|FlowControl|Delay 0.5)
  (Variables|TimeDilationVariables|SetTempRemainingDashes (Variables|DashVariables|GetNumberOfDashes))
  (Utilities|FlowControl|DoN _numberofdashes) ; enters at Reset
)

(event Custom|CheckCrouch
  ;[0.07998 1 0] Crouch slide
  ;;[0 0.2846 1] If key is pressed while in air, crouch will be activated on land
  (if (not (AI|Components|NavMovement|IsFalling (Variables|Character|GetCharacterMovement)))
    (Class|BPiParkour|ICrouch(Message) (Variables|Default|GetBP_ParkourMovement) (stale EventICrouchSlide Key))
    (Utilities|Time|ClearandInvalidateTimerbyHandle (Variables|CrouchSlideVariables|GetCheckCrouchHandle))
    (Utilities|Time|ClearandInvalidateTimerbyHandle (Variables|Default|GetCrouchJumpTimer))))

(event Custom|Reset%20Dialiation%20color%20once
  ;[0 0.2846 1] Dash functionality
  (Utilities|FlowControl|DoOnce false) ; enters at Reset
)

(event Custom|CheckTimeSlow
  (bind _returnvalue (Game|GetPlayerController 0))
  (bind _numberofdashes (Variables|DashVariables|GetNumberOfDashes))
  (bind _charactermovement (Variables|Character|GetCharacterMovement))
  (bind _charactermovement_2 (Variables|Character|GetCharacterMovement))
  (bind _returnvalue_2 (AI|Components|NavMovement|IsFalling _charactermovement_2))
  ;[0 0.2846 1] Dash functionality
  (if (Math|Boolean|ANDBoolean (>= (Class|PlayerController|GetInputKeyTimeDown _returnvalue (stale EventIDash Key)) (Variables|TimeDilationVariables|GetKeyHoldTimeTillDilation)) (Game|Player|IsInputKeyDown _returnvalue (stale EventIDash Key)) _returnvalue_2)
    (Utilities|FlowControl|DoOnce false
      (:Completed
        (if _returnvalue_2
          (if (>= (Variables|TimeDilationVariables|GetTempRemainingDashes) (Variables|DashVariables|GetNumberOfDashes))
            (Class|MovementComponent|SetPlaneConstraintNormal (Variables|Character|GetCharacterMovement) "0.000000,0.000000,1.000000")
            (Variables|DashVariables|SetDashDilationActive true)
            (Utilities|Time|SetGlobalTimeDilation 0.25)
            (Variables|Default|SetCustomTimeDilation 1.7)
            (bind _returnvalue_3 (Utilities|Time|SetTimerbyFunctionName 0 "F_DurationOfTimeDilation" 0.0025 true))
            (Variables|TimeDilationVariables|SetDilationDurationLoopingHandle _returnvalue_3)
            (Utilities|FlowControl|DoOnce false
              (:Completed
                (CameraFades|StartCameraFade (Game|GetPlayerCameraManager 0) 0.0 0.7 0.2 "(R=0.000000,G=0.047977,B=0.859375,A=1.000000)" false true))))
          (else
            (bind _counter (Utilities|FlowControl|DoN _numberofdashes)
              (:Exit
                (Math|Integer|DecrementInt (Variables|TimeDilationVariables|GetTempRemainingDashes)
                  (:%20%20
                    (Utilities|FlowControl|Sequence
                      (:then_0
                        (CallFunction|FDirectionDash)
                        (Utilities|MDashDuration)
                        ;;[1 1 1] Clamp Velocity
                        (Variables|/Script/Engine.MovementComponent|SetVelocity _charactermovement (/ (Variables|/Script/Engine.MovementComponent|GetVelocity _charactermovement) (Variables|DashVariables|GetVelocityCapAfterDash)))
                        (Variables|/Script/Engine.CharacterMovementComponent|SetGroundFriction _charactermovement (Variables|DashVariables|GetDefaultGroundFriction))
                        (if (< (Variables|TimeDilationVariables|GetTempRemainingDashes) (Variables|DashVariables|GetNumberOfDashes))
                          (Utilities|FlowControl|Delay 0.75)
                          (CallFunction|FCheckResetDash)))
                      (:then_1
                        (if (== _counter _numberofdashes)
                          (bind _returnvalue_4 (Utilities|Time|SetTimerbyFunctionName 0 "F_CheckResetDash" 0.0025 true))
                          (Variables|DashVariables|SetResetDashTimerHandle _returnvalue_4))))))))))))))

(event Custom|ResetDashDoOnce
  (bind _numberofdashes (Variables|DashVariables|GetNumberOfDashes))
  (bind _charactermovement (Variables|Character|GetCharacterMovement))
  ;[0 0.2846 1] Dash functionality
  (Utilities|FlowControl|DoOnce false) ; enters at Reset
)

(event Custom|DeathTimeDilation
  ;[0 0.176 1] Damage System
  ;;[0 0.02679 1] Take damage = Trigger death system + Slowdown time
  (Variables|SpawnVariables|SetTempGlobalTimeDilation (- (Variables|SpawnVariables|GetTempGlobalTimeDilation) 0.0075))
  (if (<= (Variables|SpawnVariables|GetTempGlobalTimeDilation) 0.0)
    (Utilities|Time|ClearandInvalidateTimerbyHandle (Variables|SpawnVariables|GetDeathTimeDilationHandle))
    (Variables|SpawnVariables|SetTempGlobalTimeDilation 1.0)
    (else
      (Utilities|Time|SetGlobalTimeDilation (Variables|SpawnVariables|GetTempGlobalTimeDilation)))))

(event Custom|TriggerDash
  (bind _numberofdashes (Variables|DashVariables|GetNumberOfDashes))
  (bind _charactermovement (Variables|Character|GetCharacterMovement))
  ;[0 0.2846 1] Dash functionality
  (Variables|DashVariables|SetDashDilationActive false)
  (CallFunction|FResetDashTimeDilation)
  (if (AI|Components|NavMovement|IsFalling (Variables|Character|GetCharacterMovement))
    (bind _counter (Utilities|FlowControl|DoN _numberofdashes)
      (:Exit
        (Math|Integer|DecrementInt (Variables|TimeDilationVariables|GetTempRemainingDashes)
          (:%20%20
            (Utilities|FlowControl|Sequence
              (:then_0
                (CallFunction|FDirectionDash)
                (Utilities|MDashDuration)
                ;;[1 1 1] Clamp Velocity
                (Variables|/Script/Engine.MovementComponent|SetVelocity _charactermovement (/ (Variables|/Script/Engine.MovementComponent|GetVelocity _charactermovement) (Variables|DashVariables|GetVelocityCapAfterDash)))
                (Variables|/Script/Engine.CharacterMovementComponent|SetGroundFriction _charactermovement (Variables|DashVariables|GetDefaultGroundFriction))
                (if (< (Variables|TimeDilationVariables|GetTempRemainingDashes) (Variables|DashVariables|GetNumberOfDashes))
                  (Utilities|FlowControl|Delay 0.75)
                  (CallFunction|FCheckResetDash)))
              (:then_1
                (if (== _counter _numberofdashes)
                  (bind _returnvalue (Utilities|Time|SetTimerbyFunctionName 0 "F_CheckResetDash" 0.0025 true))
                  (Variables|DashVariables|SetResetDashTimerHandle _returnvalue))))))))))

(event Custom|FireDispatchersFromRestartLevel
  ;[0 0.2846 1] Update the dispatchers (UI components) from restarting through the gamemode
  (bind _savegameref (Variables|Default|GetSaveGameRef :!label _label)
    (:then
      (Default|CallEDUpdateDeath (Utilities|Struct|BreakS_LevelData (Variables|/Game/TECH/Mitz/Blueprints/BP_SaveGame.BP_SaveGame_C|GetLevelData _savegameref)) (Variables|SpawnVariables|GetRespawnInputKey)))
    (:else
      (Utilities|FlowControl|Delay 0.01)
      (goto _label))))

(event EventIMoveForwardBack
  (params (Axis :type Float%20%28single-precision%29))
  ;[0 0.2846 1] INPUTS
  ;;[1 1 1] Movement Inputs
  (Utilities|MIsDashDilationActive
    (:Active
      (CallFunction|FSlowCharacterVelocity))
    (:NotActive
      (Variables|BaseMovement|SetFBAxisMovement Axis)
      (Pawn|Input|AddMovementInput (Transformation|GetActorForwardVector) Axis false))))

(event EventISetDead
  (params (Dead? :type Boolean))
  (bind _savegameref (Variables|Default|GetSaveGameRef))
  (bind _spawn_manager (Variables|Default|GetSpawn%20Manager))
  (bind _leveldata (Variables|/Game/TECH/Mitz/Blueprints/BP_SaveGame.BP_SaveGame_C|GetLevelData _savegameref))
  (bind _currentnumberofdeaths (Utilities|Struct|BreakS_LevelData _leveldata))
  ;[0 0.176 1] Damage System
  ;;[0.0782 1 0] Death
  (bind _output_get (Variables|SpawnVariables|Setdead? Dead?))
  (if _output_get
    ;;;[0 0.2846 1] SaveDeathNumber
    (Utilities|Struct|SetmembersinS_LevelData _leveldata (+ _currentnumberofdeaths 1))
    (Default|CallEDUpdateDeath _currentnumberofdeaths (Variables|SpawnVariables|GetRespawnInputKey))
    (Default|CloseGate _spawn_manager)
    (for _array_element (Variables|/Game/TECH/Mitz/Blueprints/BP_SpawnManager.BP_SpawnManager_C|GetRecordPhantom _spawn_manager)
      (Utilities|Array|Add (Variables|/Game/TECH/Mitz/Blueprints/BP_SaveGame.BP_SaveGame_C|GetPhantomRunnerData (Variables|Default|GetSaveGameRef)) _array_element))
    (Class|ISaveGame|IUpdateLevelData(Message) (Game|GetGameMode))))

(event EventBeginPlay
  (bind _charactermovement (Variables|Character|GetCharacterMovement))
  ;[0 0.2846 1] Begin play
  (Class|BPiParkour|IInitalize(Message) (Variables|Default|GetBP_ParkourMovement) self)
  (Default|Init (Variables|Default|GetBP_GrappleComponent) self)
  (CallFunction|FStoreVariables)
  (Variables|Default|SetOringalJumpZ (Variables|/Script/Engine.CharacterMovementComponent|GetJumpZVelocity _charactermovement))
  (Variables|Default|SetOrignalWalkSpeed (Variables|/Script/Engine.CharacterMovementComponent|GetMaxWalkSpeed _charactermovement))
  (CallFunction|FireDispatchersfromRestartLevel))

(event EventOnLanded
  (params (Hit :type Hit%20Result%20Structure%20%28by%20ref%29))
  (bind _charactermovement (Variables|Character|GetCharacterMovement))
  ;[0.08022 1 0] Land events
  (Class|BPiParkour|ILandEvent(Message) (Variables|Default|GetBP_ParkourMovement))
  (Variables|/Script/Engine.CharacterMovementComponent|SetJumpZVelocity _charactermovement (Variables|Default|GetOringalJumpZ))
  (Variables|/Script/Engine.CharacterMovementComponent|SetGravityScale _charactermovement 2.0))

(event EventIMantle
  (params (TargetLocation :type Vector :default "0, 0, 0"))
  ;[0.1119 1 0.04971] Mantle
  (Variables|MantleVaribles|SetMantleTargetLocation TargetLocation)
  (Variables|MantleVaribles|SetInitalPlayerPosition (Transformation|GetActorLocation))
  (bind _alpha (Timeline|MantleTimeline PlayFromStart)
    (:Update
      (Transformation|SetActorLocation (Math|Vector|Lerp(Vector) (Variables|MantleVaribles|GetInitalPlayerPosition) (Variables|MantleVaribles|GetMantleTargetLocation) _alpha) false false))
    (:Finished
      (Class|BPiParkour|IMantleDone(Message) (Variables|Default|GetBP_ParkourMovement)))))

(event EventIDash
  (params (Pressed :type Boolean) (Key :type Key%20Structure :default "None"))
  (bind _numberofdashes (Variables|DashVariables|GetNumberOfDashes))
  (bind _charactermovement (Variables|Character|GetCharacterMovement))
  ;[0 0.2846 1] Dash functionality
  (Utilities|MCheckDead
    (:NotDead
      (if Pressed
        (Utilities|FlowControl|Sequence
          (:then_0
            (if (not (Game|Player|IsInputKeyDown (Game|GetPlayerController 0) Key))
              (bind _counter (Utilities|FlowControl|DoN _numberofdashes :!label _label)
                (:Exit
                  (Math|Integer|DecrementInt (Variables|TimeDilationVariables|GetTempRemainingDashes)
                    (:%20%20
                      (Utilities|FlowControl|Sequence
                        (:then_0
                          (CallFunction|FDirectionDash)
                          (Utilities|MDashDuration)
                          ;;[1 1 1] Clamp Velocity
                          (Variables|/Script/Engine.MovementComponent|SetVelocity _charactermovement (/ (Variables|/Script/Engine.MovementComponent|GetVelocity _charactermovement) (Variables|DashVariables|GetVelocityCapAfterDash)))
                          (Variables|/Script/Engine.CharacterMovementComponent|SetGroundFriction _charactermovement (Variables|DashVariables|GetDefaultGroundFriction))
                          (if (< (Variables|TimeDilationVariables|GetTempRemainingDashes) (Variables|DashVariables|GetNumberOfDashes))
                            (Utilities|FlowControl|Delay 0.75)
                            (CallFunction|FCheckResetDash)))
                        (:then_1
                          (if (== _counter _numberofdashes)
                            (bind _returnvalue (Utilities|Time|SetTimerbyFunctionName 0 "F_CheckResetDash" 0.0025 true))
                            (Variables|DashVariables|SetResetDashTimerHandle _returnvalue))))))))
              (elif (AI|Components|NavMovement|IsFalling (Variables|Character|GetCharacterMovement))
                (if (>= (Variables|TimeDilationVariables|GetTempRemainingDashes) (Variables|DashVariables|GetNumberOfDashes))
                  (Class|MovementComponent|SetPlaneConstraintNormal (Variables|Character|GetCharacterMovement) "0.000000,0.000000,1.000000")
                  (Variables|DashVariables|SetDashDilationActive true)
                  (Utilities|Time|SetGlobalTimeDilation 0.25)
                  (Variables|Default|SetCustomTimeDilation 1.7)
                  (bind _returnvalue_2 (Utilities|Time|SetTimerbyFunctionName 0 "F_DurationOfTimeDilation" 0.0025 true))
                  (Variables|TimeDilationVariables|SetDilationDurationLoopingHandle _returnvalue_2)
                  (Utilities|FlowControl|DoOnce false
                    (:Completed
                      (CameraFades|StartCameraFade (Game|GetPlayerCameraManager 0) 0.0 0.7 0.2 "(R=0.000000,G=0.047977,B=0.859375,A=1.000000)" false true))))
                (else
                  (goto _label)))))
          (:then_1
            (bind _returnvalue_3 (Utilities|Time|SetTimerbyEvent (delegate Custom|CheckTimeSlow) (Utilities|Time|GetWorldDeltaSeconds) true))
            (Variables|TimeDilationVariables|SetTimeSlowLoopingHandle _returnvalue_3)))
        (else
          (Variables|DashVariables|SetDashDilationActive false)
          (CallFunction|FResetDashTimeDilation)
          (if (AI|Components|NavMovement|IsFalling (Variables|Character|GetCharacterMovement))
            (goto _label)))))))

(event EventICheckpointRestart
  (params (Pressed :type Boolean) (Key :type Key%20Structure :default "None"))
  ;[0.1718 1 0] Checkpoint System
  (if Pressed
    (Variables|SpawnVariables|SetRespawnInputKey Key)
    (Utilities|MCheckDead
      (:Dead
        (Class|ISaveGame|ILoadGame(Message) (Game|GetGameMode))
        (Default|CallEDPlayerRespawned)
        (Utilities|Time|SetGlobalTimeDilation 1.0)
        (Variables|SpawnVariables|Setdead? false)
        ;;[0 0.2846 1 1 17] Reset the respawn variables
        (CallFunction|FResetVariablesonRespawn)
        (Default|NewReset (Variables|Default|GetSpawn%20Manager))
        (Default|FNullVariables (Variables|Default|GetBP_GrappleComponent))))))

(event EventIBeginCrouch
  (params (StandingCapuleHalfHeight :type Float%20%28single-precision%29) (StandingCameraOffsetZ :type Float%20%28single-precision%29))
  (bind _charactermovement (Variables|Character|GetCharacterMovement))
  (bind _camera (Variables|Default|GetCamera))
  (bind _crouchedhalfheight (Variables|/Script/Engine.CharacterMovementComponent|GetCrouchedHalfHeight _charactermovement))
  (bind _relativelocation (Variables|/Script/Engine.SceneComponent|GetRelativeLocation _camera))
  ;[0.07998 1 0] Begin crouch - timeline (tweaks half height with lerp)
  (bind _alpha (Timeline|CrouchTimeline Play)
    (:Update
      (Components|Capsule|SetCapsuleHalfHeight (Variables|Collision|GetCapsuleComponent) (Math|Float|MapRangeClamped _alpha 0.0 1.0 _crouchedhalfheight StandingCapuleHalfHeight) true)
      (Transformation|SetRelativeLocation _camera (Math|Vector|MakeVector (.x _relativelocation) (.y _relativelocation) (Math|Float|MapRangeClamped _alpha 0.0 1.0 _crouchedhalfheight StandingCameraOffsetZ)) false false))))

(event EventIEndCrouch
  (bind _charactermovement (Variables|Character|GetCharacterMovement))
  (bind _camera (Variables|Default|GetCamera))
  (bind _crouchedhalfheight (Variables|/Script/Engine.CharacterMovementComponent|GetCrouchedHalfHeight _charactermovement))
  (bind _relativelocation (Variables|/Script/Engine.SceneComponent|GetRelativeLocation _camera))
  ;[0.07998 1 0] Begin crouch - timeline (tweaks half height with lerp)
  (bind _alpha (Timeline|CrouchTimeline Reverse)
    (:Update
      (Components|Capsule|SetCapsuleHalfHeight (Variables|Collision|GetCapsuleComponent) (Math|Float|MapRangeClamped _alpha 0.0 1.0 _crouchedhalfheight (stale EventIBeginCrouch StandingCapuleHalfHeight)) true)
      (Transformation|SetRelativeLocation _camera (Math|Vector|MakeVector (.x _relativelocation) (.y _relativelocation) (Math|Float|MapRangeClamped _alpha 0.0 1.0 _crouchedhalfheight (stale EventIBeginCrouch StandingCameraOffsetZ))) false false))))

(event EventISlide
  ;[0.07998 1 0] Begin slide
  (Timeline|SlideTimeline Play))

(event EventIStopSlide
  ;[0.07998 1 0] Begin slide
  (Timeline|SlideTimeline Stop))

(event EventIBeginSlideCameraTilt
  (bind _returnvalue (Pawn|GetController))
  (bind _returnvalue_2 (Pawn|GetControlRotation _returnvalue :!class /Script/Engine.Controller))
  ;[0.07998 1 0] Tilt camera while sliding
  (Timeline|CameraTiltSlide Play
    (:Update
      (Pawn|SetControlRotation _returnvalue (Math|Rotator|MakeRotator (.roll _returnvalue_2) (.pitch _returnvalue_2) (.yaw _returnvalue_2))))))

(event EventITurnLeftRight
  (params (Axis :type Float%20%28single-precision%29))
  ;[0 0.2846 1] INPUTS
  ;;[1 1 1] Movement Inputs
  (Utilities|MCheckDead
    (:NotDead
      (Pawn|Input|AddControllerYawInput Axis))))

(event EventIEndSlideCameraTilt
  (bind _returnvalue (Pawn|GetController))
  (bind _returnvalue_2 (Pawn|GetControlRotation _returnvalue :!class /Script/Engine.Controller))
  ;[0.07998 1 0] Tilt camera while sliding
  (Timeline|CameraTiltSlide Reverse
    (:Update
      (Pawn|SetControlRotation _returnvalue (Math|Rotator|MakeRotator (.roll _returnvalue_2) (.pitch _returnvalue_2) (.yaw _returnvalue_2))))))

(event EventIMoveLeftRight
  (params (Axis :type Float%20%28single-precision%29))
  (bind _returnvalue (Transformation|GetActorRightVector))
  ;[0 0.2846 1] INPUTS
  ;;[1 1 1] Movement Inputs
  (Variables|BaseMovement|SetLRAxisMovement Axis)
  (bind _movementstate (Class|BPiParkour|IGetMovementState(Message) (Variables|Default|GetBP_ParkourMovement)))
  (switch Utilities|FlowControl|Switch|SwitchonE_MovementState _movementstate
    (:NewEnumerator0
      _)
    (:NewEnumerator2
      _)
    (:NewEnumerator3
      _))
  (if (not (Variables|DashVariables|GetDashDilationActive))
    (Pawn|Input|AddMovementInput _returnvalue Axis false)
    (else
      (Character|LaunchCharacter (* _returnvalue (* Axis (Variables|DashVariables|GetDirectionalMovDilationSpeed))) true true))))

(event Game|Damage|EventAnyDamage
  (params (Damage :type Float%20%28single-precision%29) (DamageType :type Damage%20Type%20Object%20Reference) (InstigatedBy :type Controller%20Object%20Reference) (DamageCauser :type Actor%20Object%20Reference))
  ;[0 0.176 1] Damage System
  ;;[0 0.02679 1] Take damage = Trigger death system + Slowdown time
  (if (> Damage 0.0)
    (CallFunction|ISetDead true)
    (bind _returnvalue (Utilities|Time|SetTimerbyEvent (delegate Custom|DeathTimeDilation) 0.001 true))
    (Variables|SpawnVariables|SetDeathTimeDilationHandle _returnvalue)))

(event EventIStoreSpawnManager
  (params (SpawnManager :type BP%20Spawn%20Manager%20Object%20Reference))
  ;[0 0.2846 1] Store spawn manager
  (Variables|Default|SetSpawn%20Manager SpawnManager))

(event EventILookUpDown
  (params (Axis :type Float%20%28single-precision%29))
  ;[0 0.2846 1] INPUTS
  ;;[1 1 1] Movement Inputs
  (Utilities|MCheckDead
    (:NotDead
      (Pawn|Input|AddControllerPitchInput Axis))))

(event EventIJump
  (params (Pressed :type Boolean) (Key :type Key%20Structure :default "None"))
  (bind _orignalwalkspeed (Variables|Default|GetOrignalWalkSpeed))
  ;[0.08022 1 0] Jumping tied into parkour
  ;;[0 0.2846 1] Jumping
  (if Pressed
    ;;[0.07998 1 0] Checks if the player can stand and passes through jumping and switches on state
    (bind _canstand_ (Class|BPiParkour|IGetCanStand(Message) (Variables|Default|GetBP_ParkourMovement) true))
    (if _canstand_
      (bind _movementstate (Class|BPiParkour|IGetMovementState(Message) (Variables|Default|GetBP_ParkourMovement)))
      (switch Utilities|FlowControl|Switch|SwitchonE_MovementState _movementstate
        (:NewEnumerator0
          _)
        (:NewEnumerator2
          ;;[0.08022 1 0] Stands the player up when they crouch jump
          (Class|BPiParkour|IEndCrouch(Message) self)
          (Class|BPiParkour|IUnCrouch(Message) (Variables|Default|GetBP_ParkourMovement))
          ;;[0.08022 1 0] Starts a timer to see if the player can crouch / slide when landed
          (bind _returnvalue (Utilities|Time|SetTimerbyEvent (EventDispatchers|CreateEvent :!event Custom|CheckCrouch) (Utilities|Time|GetWorldDeltaSeconds) true :!label _label))
          (Variables|Default|SetCrouchJumpTimer _returnvalue))
        (:NewEnumerator3
          ;;[0.07998 1 0] Sets jump velocity based on the slide speed
          (Variables|Default|SetSlideJumpValue%28DONTCHANGE%29 (Math|Float|MapRangeClamped (Math|Vector|VectorLength (Variables|/Script/Engine.MovementComponent|GetVelocity (Variables|Character|GetCharacterMovement))) _orignalwalkspeed (* _orignalwalkspeed 1.2) (Variables|Default|GetSlideJumpMin) (Variables|Default|GetMaxSlideJumpHeight)))
          (goto _label)))
      ;;[0.08022 1 0] Checks if the player is sliding and if they are stop it and jump
      (if (Utilities|Enum|Equal(Enum) (Variables|/Game/TECH/Mitz/Blueprints/BP_ParkourMovement.BP_ParkourMovement_C|GetMovementState (Variables|Default|GetBP_ParkourMovement)) "NewEnumerator3")
        (Utilities|FlowControl|Sequence
          (:then_0
            (CallFunction|FSlideDash))
          (:then_1
            _))
        (Class|BPiParkour|IStopSlide(Message) (Variables|Default|GetBP_ParkourMovement))
        (else
          (Character|Jump)))
      (Class|BPiParkour|IJumpEvent(Message) (Variables|Default|GetBP_ParkourMovement)))
    (else
      (Character|StopJumping))))

(event EventIAttack
  (params (Pressed :type Boolean) (Key :type Key%20Structure :default "None"))
  ;[0 0.2846 1] INPUTS
  (if Pressed
    (Development|PrintString "Attacked!")))

(event EventICrouchSlide
  (params (Pressed :type Boolean) (Key :type Key%20Structure :default "None"))
  (bind _bp_parkourmovement (Variables|Default|GetBP_ParkourMovement))
  ;[0.07998 1 0] Crouch slide
  (bind _output_get (Variables|/Game/TECH/Mitz/Blueprints/BP_ParkourMovement.BP_ParkourMovement_C|SetCrouchKeyDown? _bp_parkourmovement Pressed))
  ;;[0 0.2846 1] If key is pressed while in air, crouch will be activated on land
  (if _output_get
    (bind _returnvalue (Utilities|Time|SetTimerbyEvent (delegate Custom|CheckCrouch) (Utilities|Time|GetWorldDeltaSeconds) true))
    (Variables|CrouchSlideVariables|SetCheckCrouchHandle _returnvalue)
    (if (not (AI|Components|NavMovement|IsFalling (Variables|Character|GetCharacterMovement)))
      (Class|BPiParkour|ICrouch(Message) (Variables|Default|GetBP_ParkourMovement) Key)
      (Utilities|Time|ClearandInvalidateTimerbyHandle (Variables|CrouchSlideVariables|GetCheckCrouchHandle))
      (Utilities|Time|ClearandInvalidateTimerbyHandle (Variables|Default|GetCrouchJumpTimer)))
    (else
      (Class|BPiParkour|IUnCrouch(Message) _bp_parkourmovement))))

(event EventIInteract
  (params (Pressed :type Boolean) (Key :type Key%20Structure :default "None"))
  ;[0 0.2846 1] INPUTS
  (if Pressed
    (Development|PrintString "Interacted!")))

(event EventIGrapple
  (params (Pressed :type Boolean) (Key :type Key%20Structure :default "None"))
  ;[0 0.2846 1] Grapple Event - Tied to component
  (if Pressed
    (Default|FTrytoGrapple (Variables|Default|GetBP_GrappleComponent))))

(event EventIPause
  (params (Pressed :type Boolean) (Key :type Key%20Structure :default "None"))
  ;[0 0.2846 1] INPUTS
  (if Pressed
    (Development|PrintString "Game Paused!")))

(event Input|KeyboardEvents|M
  (params (Key :type Key%20Structure :default "None"))
  (:Pressed
    (Class|ISaveGame|IRestartLevel(Message) (Game|GetGameMode))))

(fn ConstructionScript)

(fn FStoreVariables
  (Variables|DashVariables|SetDefaultGroundFriction (Variables|/Script/Engine.CharacterMovementComponent|GetGroundFriction (Variables|Character|GetCharacterMovement)))
  (Variables|TimeDilationVariables|SetDefaultCharacterTimeDilation (Variables|Default|GetCustomTimeDilation))
  (Variables|TimeDilationVariables|SetTempRemainingDashes (Variables|DashVariables|GetNumberOfDashes)))

(fn FDirectionDash
  (bind _charactermovement (Variables|Character|GetCharacterMovement))
  (bind _velocity (Variables|/Script/Engine.MovementComponent|GetVelocity _charactermovement))
  (bind (_x _y) (Math|Vector|BreakVector _velocity))
  (if (not (AI|Components|NavMovement|IsFalling (Variables|Character|GetCharacterMovement)))
    (if (!= (Math|Vector|VectorLength (Math|Vector|MakeVector _x _y 0.0)) 0.0)
      (LocalVariables|SetCurrentDashDirVec (Pawn|Components|PawnMovement|GetLastInputVector (Variables|Character|GetCharacterMovement)))
      (else
        (LocalVariables|SetCurrentDashDirVec (Transformation|GetActorForwardVector))))
    (else
      (LocalVariables|SetCurrentDashDirVec (Math|Vector|GetForwardVector (Variables|Default|GetCamera)))))
  (Variables|/Script/Engine.CharacterMovementComponent|SetGroundFriction (Variables|Character|GetCharacterMovement) 0.0)
  (Character|LaunchCharacter (* (LocalVariables|GetCurrentDashDirVec) (Variables|DashVariables|GetSpeedOfDash)) true true)
  (return))

(fn FCheckResetDash
  (if (AI|Components|NavMovement|IsFalling (Variables|Character|GetCharacterMovement))
    (if (Variables|/Game/TECH/Mitz/Blueprints/BP_ParkourMovement.BP_ParkourMovement_C|GetWallRunning (Variables|Default|GetBP_ParkourMovement))
      (CallFunction|ResetDashes :!label _label)
      (Utilities|Time|ClearandInvalidateTimerbyHandle (Variables|DashVariables|GetResetDashTimerHandle)))
    (else
      (goto _label))))

(fn FResetDashTimeDilation
  (Utilities|Time|SetGlobalTimeDilation 1.0)
  (Utilities|FlowControl|Sequence
    (:then_0
      (CallFunction|ResetDialiationColorOnce)
      (Utilities|Time|ClearandInvalidateTimerbyHandle (Variables|TimeDilationVariables|GetTimeSlowLoopingHandle))
      (CallFunction|ResetDashDoOnce)
      (Variables|Default|SetCustomTimeDilation (Variables|TimeDilationVariables|GetDefaultCharacterTimeDilation))
      (Class|MovementComponent|SetPlaneConstraintNormal (Variables|Character|GetCharacterMovement) "0, 0, 0")
      (Variables|TimeDilationVariables|SetTempTimeDilationTime 0.0)
      (Utilities|Time|ClearandInvalidateTimerbyHandle (Variables|TimeDilationVariables|GetDilationDurationLoopingHandle))
      (Default|CallEDDashTimeDilation 0.0)
      (Default|CallEDFinishedTimeDilation))
    (:then_1
      (Utilities|MCheckDead
        (:NotDead
          (CameraFades|StopCameraFade (Game|GetPlayerCameraManager 0)))))))

(fn FDurationOfTimeDilation
  (bind _output_get (Variables|TimeDilationVariables|SetTempTimeDilationTime (+ (Variables|TimeDilationVariables|GetTempTimeDilationTime) 0.01)))
  (if (>= _output_get (Variables|TimeDilationVariables|GetMaxTimeDilationTime))
    (CallFunction|TriggerDash)
    (Utilities|Time|ClearandInvalidateTimerbyHandle (Variables|TimeDilationVariables|GetDilationDurationLoopingHandle))
    (Default|CallEDDashTimeDilation 0.0)
    (else
      (Default|CallEDDashTimeDilation _output_get))))

(fn FResetVariablesonRespawn
  (Utilities|Time|ClearandInvalidateTimerbyHandle (Variables|SpawnVariables|GetDeathTimeDilationHandle))
  (Variables|SpawnVariables|SetTempGlobalTimeDilation 1.0)
  (Components|Movement|StopMovementImmediately (Variables|Character|GetCharacterMovement)))

(fn FSlideDash
  (bind _charactermovement (Variables|Character|GetCharacterMovement))
  (bind _velocity (Variables|/Script/Engine.MovementComponent|GetVelocity _charactermovement))
  (bind (_x _y) (Math|Vector|BreakVector _velocity))
  (if (not (AI|Components|NavMovement|IsFalling (Variables|Character|GetCharacterMovement)))
    (if (!= (Math|Vector|VectorLength (Math|Vector|MakeVector _x _y 0.0)) 0.0)
      (LocalVariables|SetCurrentDashDirVec (Transformation|GetActorForwardVector))
      (else
        (LocalVariables|SetCurrentDashDirVec (Transformation|GetActorForwardVector))))
    (else
      (LocalVariables|SetCurrentDashDirVec (Math|Vector|GetForwardVector (Variables|Default|GetCamera)))))
  (Character|LaunchCharacter (Math|Vector|MakeVector (.x (* (LocalVariables|GetCurrentDashDirVec) (LocalVariables|GetDashSpeedfterSLides))) (.y (* (LocalVariables|GetCurrentDashDirVec) (LocalVariables|GetDashSpeedfterSLides))) (Variables|Default|GetSlideJumpValue%28DONTCHANGE%29)) true true)
  (return))

(fn FSlowCharacterVelocity)

(fn ICharacterRef
  (return self))

(fn IGetCamera
  (return (Variables|Default|GetCamera)))

(fn IGetCanStand
  (params (jumping? :type Boolean))
  (return false))

(fn IGetController
  (return 0))

(fn IGetMovementState
  (return "NewEnumerator0"))

(fn IMovementRef
  (return (Variables|Character|GetCharacterMovement)))