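; Player controller that relays all player input, from movement, jump, dash, grapple and crouch-slide to attack, interact, pause and checkpoint restart, to the controlled pawn.
; On BeginPlay it sets game-only input, caches the pawn and initializes the game mode with itself and that pawn.
; Each action press or release and axis value is forwarded as an interface message, leaving the gameplay logic outside the controller.
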(event EventBeginPlay
  (bind _returnvalue (Pawn|GetControlledPawn))
  ;[1 1 1] Begin play
  (Input|SetInputModeGameOnly self)
  (Variables|Default|SetControlledPawn _returnvalue)
  (Default|InitGamemode (CallFunction|FGamemode) self _returnvalue))

(event Input|ActionEvents|InputActionJump
  (params (Key :type Key%20Structure))
  (bind _controlledpawn (Variables|Default|GetControlledPawn))
  ;[1 1 1] Movements
  (:Pressed
    (Class|BPICharacterInputs|IJump(Message) _controlledpawn true Key))
  (:Released
    (Class|BPICharacterInputs|IJump(Message) _controlledpawn false Key)))

(event Input|ActionEvents|InputActionCrouchSlide
  (params (Key :type Key%20Structure))
  (bind _controlledpawn (Variables|Default|GetControlledPawn))
  ;[1 1 1] Movements
  (:Pressed
    (Class|BPICharacterInputs|ICrouchSlide(Message) _controlledpawn true Key))
  (:Released
    (Class|BPICharacterInputs|ICrouchSlide(Message) _controlledpawn false Key)))

(event Input|ActionEvents|InputActionAttack
  (params (Key :type Key%20Structure))
  (bind _controlledpawn (Variables|Default|GetControlledPawn))
  ;[1 1 1] Interactions
  (:Pressed
    (Class|BPICharacterInputs|IAttack(Message) _controlledpawn true Key))
  (:Released
    (Class|BPICharacterInputs|IAttack(Message) _controlledpawn false Key)))

(event Input|ActionEvents|InputActionGrapple
  (params (Key :type Key%20Structure))
  (bind _controlledpawn (Variables|Default|GetControlledPawn))
  ;[1 1 1] Interactions
  (:Pressed
    (Class|BPICharacterInputs|IGrapple(Message) _controlledpawn true Key))
  (:Released
    (Class|BPICharacterInputs|IGrapple(Message) _controlledpawn false Key)))

(event Input|ActionEvents|InputActionInteract
  (params (Key :type Key%20Structure))
  (bind _controlledpawn (Variables|Default|GetControlledPawn))
  ;[1 1 1] Interactions
  (:Pressed
    (Class|BPICharacterInputs|IInteract(Message) _controlledpawn true Key))
  (:Released
    (Class|BPICharacterInputs|IInteract(Message) _controlledpawn false Key)))

(event Input|ActionEvents|InputActionPauseGame
  (params (Key :type Key%20Structure))
  (bind _controlledpawn (Variables|Default|GetControlledPawn))
  ;[1 1 1] Interactions
  (:Pressed
    (Class|BPICharacterInputs|IPause(Message) _controlledpawn true Key))
  (:Released
    (Class|BPICharacterInputs|IPause(Message) _controlledpawn false Key)))

(event Input|ActionEvents|InputActionDash
  (params (Key :type Key%20Structure))
  (bind _controlledpawn (Variables|Default|GetControlledPawn))
  ;[1 1 1] Movements
  (:Pressed
    (Class|BPICharacterInputs|IDash(Message) _controlledpawn true Key))
  (:Released
    (Class|BPICharacterInputs|IDash(Message) _controlledpawn false Key)))

(event Input|ActionEvents|InputActionCheckpointRestart
  (params (Key :type Key%20Structure))
  (bind _controlledpawn (Variables|Default|GetControlledPawn))
  ;[1 1 1] Interactions
  (:Pressed
    (Class|BPICharacterInputs|ICheckpointRestart(Message) _controlledpawn true Key))
  (:Released
    (Class|BPICharacterInputs|ICheckpointRestart(Message) _controlledpawn false Key)))

(event Input|AxisEvents|InputAxisMoveForwardBackward
  (params (AxisValue :type Float%20%28single-precision%29))
  ;[1 1 1] Movements
  (Class|BPICharacterInputs|IMoveForwardBack(Message) (Variables|Default|GetControlledPawn) AxisValue))

(event Input|AxisEvents|InputAxisMoveLeftRight
  (params (AxisValue :type Float%20%28single-precision%29))
  ;[1 1 1] Movements
  (Class|BPICharacterInputs|IMoveLeftRight(Message) (Variables|Default|GetControlledPawn) AxisValue))

(event Input|AxisEvents|InputAxisTurnLeftRight
  (params (AxisValue :type Float%20%28single-precision%29))
  ;[1 1 1] Movements
  (Class|BPICharacterInputs|ITurnLeftRight(Message) (Variables|Default|GetControlledPawn) AxisValue))

(event Input|AxisEvents|InputAxisLookUpDown
  (params (AxisValue :type Float%20%28single-precision%29))
  ;[1 1 1] Movements
  (Class|BPICharacterInputs|ILookUpDown(Message) (Variables|Default|GetControlledPawn) AxisValue))

(fn ConstructionScript)