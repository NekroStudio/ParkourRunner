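; End-of-level trigger volume that stops the HUD timer and records the player's level stats when the player overlaps its resizable box.
; It searches the character's save game for an entry matching the current level name.
; A match updates that entry's stats, replacing deaths only if higher, without a save call; otherwise a new entry is added and saved to slot.
; The end screen widget creation is disconnected and never runs.
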(event OnComponentBeginOverlap(EndVolume)
  (params (OverlappedComponent :type Primitive%20Component%20Object%20Reference) (OtherActor :type Actor%20Object%20Reference) (OtherComp :type Primitive%20Component%20Object%20Reference) (OtherBodyIndex :type Integer) (bFromSweep :type Boolean) (SweepResult :type Hit%20Result%20Structure%20%28by%20ref%29))
  (Utilities|MIsPlayer OtherActor
    (:true
      (Utilities|Time|PauseTimerbyHandle (Variables|/Game/TECH/Mitz/Blueprints/W_Timer.W_Timer_C|GetTimerHandle (Variables|/Game/TECH/Jay/UI/W_BaseHUD.W_BaseHUD_C|GetW_Timer (Variables|/Game/TECH/Jay/BP_PlayerController.BP_PlayerController_C|GetHUD (Variables|Default|GetController)))))
      (bind _array_element (Utilities|Array|ForEachLoopwithBreak (Variables|/Game/TECH/Mitz/Blueprints/BP_SaveGame.BP_SaveGame_C|GetLevelData (Variables|/Game/TECH/Jay/BP_BaseCharacter.BP_BaseCharacter_C|GetSaveGameRef (Variables|Default|GetCharacter))))
        (:LoopBody
          (bind _returnvalue (Game|GetCurrentLevelName true))
          (if (Utilities|Enum|Equal(Enum) _returnvalue (Utilities|String|ToString(Name) (.LevelName (Utilities|Struct|BreakS_LevelData _array_element))))
            (Variables|Default|SetExistingData true)
            (CallFunction|BreakLoop)
            (else
              (Variables|Default|SetExistingData false))))
        (:Completed
          (if (Variables|Default|GetExistingData)
            (Development|PrintString "exists")
            ;[1 1 1] Overwrite data
            (CallFunction|FOverwriteData (.CurrentNumberOfDeaths (Utilities|Struct|BreakS_LevelData _array_element)) _array_element)
            (else
              (Development|PrintString "Doesnt exist")
              ;[1 1 1] Make new data
              (CallFunction|FMakeNewData))))))))

(event Custom|BreakLoop
  (Utilities|Array|ForEachLoopwithBreak (Variables|/Game/TECH/Mitz/Blueprints/BP_SaveGame.BP_SaveGame_C|GetLevelData (Variables|/Game/TECH/Jay/BP_BaseCharacter.BP_BaseCharacter_C|GetSaveGameRef (Variables|Default|GetCharacter)))) ; enters at Break
)

(event EventBeginPlay
  ;[1 1 1] Store character
  (|CallParentFunction)
  (bind _character (Class|BPiSpawning|ICharacterRef(Message) (Game|GetPlayerCharacter 0)))
  (Variables|Default|SetCharacter _character)
  (bind _controller (Class|ISaveGame|IGetPlayerController(Message) (Game|GetPlayerController 0)))
  (Variables|Default|SetController _controller))

(fn ConstructionScript
  (|CallParentFunction)
  (Components|Box|SetBoxExtent (Variables|Default|GetEndVolume) (Variables|Default|GetBoxExtent) true))

(fn FMakeNewData
  (bind _character (Variables|Default|GetCharacter))
  (bind _savegameref (Variables|/Game/TECH/Jay/BP_BaseCharacter.BP_BaseCharacter_C|GetSaveGameRef _character))
  (bind _returnvalue (Game|GetCurrentLevelName true))
  (Utilities|Array|Add (Variables|/Game/TECH/Mitz/Blueprints/BP_SaveGame.BP_SaveGame_C|GetLevelData _savegameref) (Utilities|Struct|MakeS_LevelData (Utilities|String|StringToName _returnvalue) (Variables|/Game/TECH/Mitz/Blueprints/BP_SaveGame.BP_SaveGame_C|GetDeaths _savegameref) (Variables|/Game/TECH/Mitz/Blueprints/BP_SaveGame.BP_SaveGame_C|GetTimer _savegameref) 0 (Variables|/Game/TECH/Mitz/Blueprints/BP_SaveGame.BP_SaveGame_C|GetKills _savegameref) (Variables|/Game/TECH/Mitz/Blueprints/BP_SaveGame.BP_SaveGame_C|GetSecretPicksFound _savegameref)))
  (SaveGame|SaveGametoSlot _savegameref "Save1"))

(fn FOverwriteData
  (params (Deaths :type Integer) (LevelData :type S%20Level%20Data%20Structure))
  (bind _character (Variables|Default|GetCharacter))
  (bind _savegameref (Variables|/Game/TECH/Jay/BP_BaseCharacter.BP_BaseCharacter_C|GetSaveGameRef _character))
  (if (> (Variables|/Game/TECH/Mitz/Blueprints/BP_SaveGame.BP_SaveGame_C|GetDeaths _savegameref) Deaths)
    (Utilities|Struct|SetmembersinS_LevelData LevelData (Variables|/Game/TECH/Mitz/Blueprints/BP_SaveGame.BP_SaveGame_C|GetDeaths _savegameref)))
  (Utilities|Struct|SetmembersinS_LevelData LevelData (Variables|/Game/TECH/Mitz/Blueprints/BP_SaveGame.BP_SaveGame_C|GetTimer _savegameref))
  (Utilities|Struct|SetmembersinS_LevelData LevelData (Variables|/Game/TECH/Mitz/Blueprints/BP_SaveGame.BP_SaveGame_C|GetKills _savegameref))
  (Utilities|Struct|SetmembersinS_LevelData LevelData (Variables|/Game/TECH/Mitz/Blueprints/BP_SaveGame.BP_SaveGame_C|GetSecretPicksFound _savegameref))
  (Utilities|Struct|SetmembersinS_LevelData LevelData (Variables|/Game/TECH/Mitz/Blueprints/BP_SaveGame.BP_SaveGame_C|GetPlayerScore _savegameref)))