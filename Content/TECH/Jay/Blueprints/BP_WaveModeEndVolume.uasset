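; BP_WaveModeEndVolume is a trigger volume that ends the player's run in Wave Runner mode.
; On player overlap, it passes the game mode to the end door's lock interface and starts a camera transition.
; It blends the view to a child-actor camera and switches input to UI-only with a visible cursor.
; A looping frame-interval timer auto-walks the character forward until it is hidden shortly afterward.
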(event OnComponentBeginOverlap(Box)
  (params (OverlappedComponent :type Primitive%20Component%20Object%20Reference) (OtherActor :type Actor%20Object%20Reference) (OtherComp :type Primitive%20Component%20Object%20Reference) (OtherBodyIndex :type Integer) (bFromSweep :type Boolean) (SweepResult :type Hit%20Result%20Structure%20%28by%20ref%29))
  ;[1 1 1] On overlap, play cam transition and reshow enhancements
  (Utilities|MIsPlayer OtherActor
    (:true
      (CallFunction|PlayCameraTransition)
      (Default|ILockDoor(WM) (Variables|Default|GetEndDoor) (Variables|Default|GetWaveModeRef)))))

(event Custom|PlayCameraTransition
  ;[1 1 1] Camera transition
  (Utilities|FlowControl|Delay 0.1)
  (Game|Player|SetViewTargetwithBlend (Variables|Default|GetController) (Variables|/Script/Engine.ChildActorComponent|GetChildActor (Variables|Default|GetMoveCamLoc)) 2.0 "VTBlend_Cubic" 4.0 true)
  (bind _returnvalue (Utilities|Time|SetTimerbyFunctionName 0 "F_EnableForwardMovement" (Utilities|Time|GetWorldDeltaSeconds) true))
  (Variables|Default|SetLoopingHandle _returnvalue)
  (Utilities|FlowControl|Sequence
    (:then_0
      (CallFunction|FDisableCharInput))
    (:then_1
      (Utilities|FlowControl|Delay 0.5)
      (Utilities|Time|ClearandInvalidateTimerbyHandle (Variables|Default|GetLoopingHandle))
      (Rendering|SetActorHiddenInGame (Variables|Default|GetCharacter) true))))

(event EventBeginPlay
  ;[1 1 1] Store refs
  (|CallParentFunction)
  (bind _character (Class|BPiSpawning|ICharacterRef(Message) (Game|GetPlayerCharacter 0)))
  (Variables|Default|SetCharacter _character)
  (bind _controller (Class|ISaveGame|IGetPlayerController(Message) (Game|GetPlayerController 0)))
  (Variables|Default|SetController _controller)
  (bind _asgm_wave_runner_mode (Utilities|Casting|CastToGM_WaveRunnerMode (Game|GetGameMode)))
  (Variables|Default|SetWaveModeRef _asgm_wave_runner_mode))

(fn ConstructionScript
  (|CallParentFunction))

(fn FDisableCharInput
  (bind _controller (Variables|Default|GetController))
  (Class|NavMovementComponent|StopActiveMovement (Variables|/Script/Engine.Character|GetCharacterMovement (Variables|Default|GetCharacter)))
  (Input|DisableInput (Variables|Default|GetCharacter) _controller)
  (Variables|/Script/Engine.PlayerController|SetbShowMouseCursor _controller true)
  (Input|SetInputModeUIOnly _controller 0 "DoNotLock"))

(fn FEnableForwardMovement
  (bind _character (Variables|Default|GetCharacter))
  (Pawn|Input|AddMovementInput _character (Transformation|GetActorForwardVector _character) 1.0 false))