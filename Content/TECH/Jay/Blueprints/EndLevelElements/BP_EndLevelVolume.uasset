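; End-of-level trigger volume that records the player's run and plays the level exit sequence.
; On player overlap it pauses the HUD timer, saves stats, then adds or updates this level's save-game entry.
; It sends the totals and next level to the EndLevelWall child actor.
; The camera blends to a child-actor view while input is disabled and a looping timer walks the character forward before hiding it.
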(event OnComponentBeginOverlap(EndVolume)
  (params (OverlappedComponent :type Primitive%20Component%20Object%20Reference) (OtherActor :type Actor%20Object%20Reference) (OtherComp :type Primitive%20Component%20Object%20Reference) (OtherBodyIndex :type Integer) (bFromSweep :type Boolean) (SweepResult :type Hit%20Result%20Structure%20%28by%20ref%29))
  (bind _character (Variables|Default|GetCharacter))
  (bind _savegameref (Variables|/Game/TECH/Jay/BP_BaseCharacter.BP_BaseCharacter_C|GetSaveGameRef _character))
  ;[1 1 1] On overlap, store data
  (Utilities|MIsPlayer OtherActor
    (:true
      (Utilities|Time|PauseTimerbyHandle (Variables|/Game/TECH/Mitz/Blueprints/W_Timer.W_Timer_C|GetTimerHandle (Variables|/Game/TECH/Jay/UI/W_BaseHUD.W_BaseHUD_C|GetW_Timer (Variables|/Game/TECH/Jay/BP_PlayerController.BP_PlayerController_C|GetHUD (Variables|Default|GetController)))))
      (CallFunction|FFinalSave)
      (bind _array_element (Utilities|Array|ForEachLoopwithBreak (Variables|/Game/TECH/Mitz/Blueprints/BP_SaveGame.BP_SaveGame_C|GetLevelData (Variables|/Game/TECH/Jay/BP_BaseCharacter.BP_BaseCharacter_C|GetSaveGameRef (Variables|Default|GetCharacter))))
        (:LoopBody
          (bind _returnvalue (Game|GetCurrentLevelName true))
          (if (Utilities|Enum|Equal(Enum) _returnvalue (Utilities|String|ToString(Name) (Utilities|Struct|BreakS_LevelData _array_element)))
            (Variables|Default|SetExistingData true)
            (CallFunction|BreakLoop)
            (else
              (Variables|Default|SetExistingData false))))
        (:Completed
          (if (Variables|Default|GetExistingData)
            (Development|PrintString "exists")
            ;;[1 1 1] Overwrite data
            (CallFunction|FOverwriteData _array_element)
            (else
              (Development|PrintString "Doesnt exist")
              ;;[1 1 1] Make new data
              (CallFunction|FMakeNewData)))
          (Class|BPIEnvironmentalInteractions|IOverlapedEndVolume(Message) (Variables|/Script/Engine.ChildActorComponent|GetChildActor (Variables|Default|GetEndLevelWall)) (Variables|/Game/TECH/Mitz/Blueprints/BP_SaveGame.BP_SaveGame_C|GetKills _savegameref) (Variables|/Game/TECH/Mitz/Blueprints/BP_SaveGame.BP_SaveGame_C|GetDeaths _savegameref) (Variables|/Game/TECH/Mitz/Blueprints/BP_SaveGame.BP_SaveGame_C|GetTimer _savegameref) (Variables|/Game/TECH/Mitz/Blueprints/BP_SaveGame.BP_SaveGame_C|GetPlayerScore _savegameref) (Variables|Default|GetLevel%20to%20Open) (Variables|Default|GetController) _character)
          (CallFunction|PlayCameraTransition))))))

(event Custom|BreakLoop
  (bind _character (Variables|Default|GetCharacter))
  (bind _savegameref (Variables|/Game/TECH/Jay/BP_BaseCharacter.BP_BaseCharacter_C|GetSaveGameRef _character))
  ;[1 1 1] On overlap, store data
  (Utilities|Array|ForEachLoopwithBreak (Variables|/Game/TECH/Mitz/Blueprints/BP_SaveGame.BP_SaveGame_C|GetLevelData (Variables|/Game/TECH/Jay/BP_BaseCharacter.BP_BaseCharacter_C|GetSaveGameRef (Variables|Default|GetCharacter)))) ; enters at Break
)

(event Custom|PlayCameraTransition
  ;[1 1 1] Camera transition
  (Utilities|FlowControl|Delay 0.1)
  (Game|Player|SetViewTargetwithBlend (Variables|Default|GetController) (Variables|/Script/Engine.ChildActorComponent|GetChildActor (Variables|Default|GetMoveCamLoc)) 1.25 "VTBlend_Cubic" 4.0 true)
  (bind _returnvalue (Utilities|Time|SetTimerbyFunctionName 0 "F_EnableForwardMovement" (Utilities|Time|GetWorldDeltaSeconds) true))
  (Variables|Default|SetLoopingHandle _returnvalue)
  (Utilities|FlowControl|Sequence
    (:then_0
      (CallFunction|FDisableCharInput))
    (:then_1
      (Utilities|FlowControl|Delay 2.0)
      (Utilities|Time|ClearandInvalidateTimerbyHandle (Variables|Default|GetLoopingHandle))
      (Rendering|SetActorHiddenInGame (Variables|Default|GetCharacter) true))))

(event EventBeginPlay
  ;[1 1 1] Store character
  (|CallParentFunction)
  (bind _character (Class|BPiSpawning|ICharacterRef(Message) (Game|GetPlayerCharacter 0)))
  (Variables|Default|SetCharacter _character)
  (bind _controller (Class|ISaveGame|IGetPlayerController(Message) (Game|GetPlayerController 0)))
  (Variables|Default|SetController _controller))

(fn ConstructionScript
  (bind _endvolume (Variables|Default|GetEndVolume))
  (|CallParentFunction)
  (Components|Box|SetBoxExtent _endvolume (Variables|Default|GetBoxExtent) true)
  (Transformation|SetWorldLocation _endvolume (+ (Transformation|GetWorldLocation _endvolume) (Variables|Default|GetBoxWorldLoc)) false false))

(fn FMakeNewData
  (bind _character (Variables|Default|GetCharacter))
  (bind _savegameref (Variables|/Game/TECH/Jay/BP_BaseCharacter.BP_BaseCharacter_C|GetSaveGameRef _character))
  (bind _returnvalue (Game|GetCurrentLevelName true))
  (Utilities|Array|Add (Variables|/Game/TECH/Mitz/Blueprints/BP_SaveGame.BP_SaveGame_C|GetLevelData _savegameref) (Utilities|Struct|MakeS_LevelData (Utilities|String|StringToName _returnvalue) (Variables|/Game/TECH/Mitz/Blueprints/BP_SaveGame.BP_SaveGame_C|GetDeaths _savegameref) (Variables|/Game/TECH/Mitz/Blueprints/BP_SaveGame.BP_SaveGame_C|GetTimer _savegameref) 0 (Variables|/Game/TECH/Mitz/Blueprints/BP_SaveGame.BP_SaveGame_C|GetKills _savegameref) (Variables|/Game/TECH/Mitz/Blueprints/BP_SaveGame.BP_SaveGame_C|GetSecretPicksFound _savegameref)))
  (SaveGame|SaveGametoSlot _savegameref "Save1"))

(fn FOverwriteData
  (params (LevelData :type S%20Level%20Data%20Structure))
  (bind _character (Variables|Default|GetCharacter))
  (bind _savegameref (Variables|/Game/TECH/Jay/BP_BaseCharacter.BP_BaseCharacter_C|GetSaveGameRef _character))
  (bind _deaths (Variables|/Game/TECH/Mitz/Blueprints/BP_SaveGame.BP_SaveGame_C|GetDeaths _savegameref))
  (if (> _deaths (.CurrentNumberOfDeaths (Utilities|Struct|BreakS_LevelData LevelData)))
    (Utilities|Struct|SetmembersinS_LevelData LevelData _deaths))
  (Utilities|Struct|SetmembersinS_LevelData LevelData (Variables|/Game/TECH/Mitz/Blueprints/BP_SaveGame.BP_SaveGame_C|GetTimer _savegameref))
  (Utilities|Struct|SetmembersinS_LevelData LevelData (Variables|/Game/TECH/Mitz/Blueprints/BP_SaveGame.BP_SaveGame_C|GetKills _savegameref))
  (Utilities|Struct|SetmembersinS_LevelData LevelData (Variables|/Game/TECH/Mitz/Blueprints/BP_SaveGame.BP_SaveGame_C|GetSecretPicksFound _savegameref))
  (Utilities|Struct|SetmembersinS_LevelData LevelData (Variables|/Game/TECH/Mitz/Blueprints/BP_SaveGame.BP_SaveGame_C|GetPlayerScore _savegameref)))

(fn FEnableForwardMovement
  (bind _character (Variables|Default|GetCharacter))
  (Pawn|Input|AddMovementInput _character (Transformation|GetActorForwardVector _character) 1.0 false))

(fn FFinalSave
  (bind _character (Variables|Default|GetCharacter))
  (bind _savegameref (Variables|/Game/TECH/Jay/BP_BaseCharacter.BP_BaseCharacter_C|GetSaveGameRef _character))
  (bind _kills (Class|BPiCombat|IGetKills(Message) _character))
  (Variables|/Game/TECH/Mitz/Blueprints/BP_SaveGame.BP_SaveGame_C|SetKills _savegameref _kills)
  (Variables|/Game/TECH/Mitz/Blueprints/BP_SaveGame.BP_SaveGame_C|SetTimer _savegameref (Variables|/Game/TECH/Mitz/Blueprints/W_Timer.W_Timer_C|GetGameTime (Variables|/Game/TECH/Jay/UI/W_BaseHUD.W_BaseHUD_C|GetW_Timer (Variables|/Game/TECH/Jay/BP_PlayerController.BP_PlayerController_C|GetHUD (Variables|Default|GetController)))))
  (Utilities|Array|Clear (Variables|/Game/TECH/Mitz/Blueprints/BP_SaveGame.BP_SaveGame_C|GetCheckPointsUsed _savegameref))
  (SaveGame|SaveGametoSlot _savegameref "Save1"))

(fn FDisableCharInput
  (bind _controller (Variables|Default|GetController))
  (Class|NavMovementComponent|StopActiveMovement (Variables|/Script/Engine.Character|GetCharacterMovement (Variables|Default|GetCharacter)))
  (Input|DisableInput (Variables|Default|GetCharacter) _controller)
  (Variables|/Script/Engine.PlayerController|SetbShowMouseCursor _controller true)
  (Input|SetInputModeUIOnly _controller 0 "DoNotLock"))