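; BP_GI_Platform is a grapple-hook interactable platform that can move along a spline, expand in scale, or both.
; Each interaction runs a FlipFlop that, based on the option booleans, starts or stops the movement and expansion timelines.
; The movement timeline sets the mesh's location and yaw from the spline, while the expansion timeline lerps its scale.
; The construction script applies start scale and makes unstoppable moving platforms start on BeginPlay.
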(event Custom|TriggerPlatformEffect
  (bind _returnvalue (Utilities|MCanbeStopped&MoveonStart))
  ;[1 1 1] Flip Flop effect for stopping platform movement
  (if (Utilities|MCheckAnOptionIsSelected)
    (Utilities|FlowControl|FlipFlop
      (:A
        (if _returnvalue
          (CallFunction|StopAllConnectedInteractions :!label _label)
          (else
            (if (Utilities|MCannotbeStopped&MoveonStart)
              _
              (elif (Variables|PlatformEffects|GetIsExpandingPlatform)
                _
                (else
                  (goto _label))))
            (CallFunction|ExpandPlatform))))
      (:B
        (if _returnvalue
          _
          (elif (Variables|PlatformEffects|GetCanBeStopped)
            (goto _label)
            (else
              _)))
        (CallFunction|ExpandPlatform)))))

(event Custom|TriggerPlatformMovement
  (bind _spline (Variables|Default|GetSpline))
  ;[1 1 1] Move platform along spline
  (bind _movement (Timeline|PlatformMovement Play)
    (:Update
      (Transformation|SetWorldLocation (Variables|Character|GetMesh) (Spline|GetLocationatDistanceAlongSpline _spline (* (* _movement (Variables|PlatformExpansion|GetPlatformMovementSpeed)) (Spline|GetSplineLength _spline)) "World") false false)
      (Transformation|SetRelativeRotation (Variables|Character|GetMesh) (Math|Rotator|MakeRotator 0.0 0.0 (.yaw (Spline|GetRotationatDistanceAlongSpline _spline (* (* _movement (Variables|PlatformExpansion|GetPlatformMovementSpeed)) (Spline|GetSplineLength _spline)) "Local"))) false false))))

(event Custom|StopAllConnectedInteractions
  (bind _spline (Variables|Default|GetSpline))
  (Utilities|FlowControl|Sequence
    (:then_0
      ;[1 1 1] Trigger platform to expand from grapple hook interaction
      (bind _increase (Timeline|DevelopmentPlatform Stop)
        (:Update
          (Transformation|SetWorldScale3D (Variables|Character|GetMesh) (Math|Vector|Lerp(Vector) (Transformation|GetWorldScale (Variables|Character|GetMesh)) (Variables|PlatformExpansion|GetPlatformExpandSize) _increase)))))
    (:then_1
      ;[1 1 1] Move platform along spline
      (bind _movement (Timeline|PlatformMovement Stop)
        (:Update
          (Transformation|SetWorldLocation (Variables|Character|GetMesh) (Spline|GetLocationatDistanceAlongSpline _spline (* (* _movement (Variables|PlatformExpansion|GetPlatformMovementSpeed)) (Spline|GetSplineLength _spline)) "World") false false)
          (Transformation|SetRelativeRotation (Variables|Character|GetMesh) (Math|Rotator|MakeRotator 0.0 0.0 (.yaw (Spline|GetRotationatDistanceAlongSpline _spline (* (* _movement (Variables|PlatformExpansion|GetPlatformMovementSpeed)) (Spline|GetSplineLength _spline)) "Local"))) false false))))))

(event Custom|ExpandPlatform
  ;[1 1 1] Trigger platform to expand from grapple hook interaction
  (if (and (Variables|PlatformEffects|GetIsMovingPlatform) (Variables|PlatformEffects|GetIsExpandingPlatform))
    (CallFunction|TriggerPlatformMovement)
    (bind _increase (Timeline|DevelopmentPlatform PlayFromStart)
      (:Update
        (Transformation|SetWorldScale3D (Variables|Character|GetMesh) (Math|Vector|Lerp(Vector) (Transformation|GetWorldScale (Variables|Character|GetMesh)) (Variables|PlatformExpansion|GetPlatformExpandSize) _increase))))
    (elif (Variables|PlatformEffects|GetIsExpandingPlatform)
      (Timeline|DevelopmentPlatform PlayFromStart)
      (else
        (CallFunction|TriggerPlatformMovement)))))

(event EventBeginPlay
  ;[1 1 1] Begin play - store references
  (|CallParentFunction)
  (Transformation|SetRelativeRotation (Variables|Character|GetMesh) (Math|Rotator|MakeRotator 0.0 0.0 (.yaw (Spline|GetRotationatDistanceAlongSpline (Variables|Default|GetSpline) 0.0 "Local"))) false false)
  (if (Variables|PlatformEffects|GetShouldMoveOnStart)
    (CallFunction|TriggerPlatformMovement)))

(fn ConstructionScript
  (|CallParentFunction)
  (Transformation|SetWorldScale3D (Variables|Character|GetMesh) (Variables|PlatformExpansion|GetPlatformStartSize))
  (if (and (Variables|PlatformEffects|GetIsMovingPlatform) (not (Variables|PlatformEffects|GetCanBeStopped)))
    (Variables|PlatformEffects|SetShouldMoveOnStart true)))

(fn FInteraction
  (CallFunction|TriggerPlatformEffect))