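; Rotating hazard puzzle piece that turns its yaw back and forth when interacted with.
; FInteraction calls TriggerRotationEffect, which ignores calls mid-rotation and flip-flops between forward and reverse timelines.
; Each timeline lerps current yaw toward its end angle, clearing the busy flag within a degree of it or on finish.
; Without AllowSeveralRotations, only the forward turn plays, through a DoOnce that resets when that turn ends.
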(event Custom|TriggerRotationEffect
  (bind _returnvalue (Transformation|GetActorRotation))
  (bind _returnvalue_2 (Transformation|GetActorRotation))
  (bind _endrotationdegrees (Variables|Default|GetEndRotationDegrees))
  (bind _revereendrotationdegrees (Variables|Default|GetRevereEndRotationDegrees))
  ;[1 1 1] Rotate Platform
  (if (not (Variables|Default|GetCurrentlyRotating))
    (Utilities|FlowControl|FlipFlop
      (:A
        (if (Variables|Default|GetAllowSeveralRotations)
          (bind _rotate (Timeline|Rotation PlayFromStart)
            (:Update
              (if (>= (.yaw _returnvalue) (- _endrotationdegrees 1.0))
                (Variables|Default|SetCurrentlyRotating false :!label _label)
                (CallFunction|ResetDoOnce)
                (else
                  (Transformation|SetActorRotation (Math|Rotator|MakeRotator (.roll _returnvalue) (.pitch _returnvalue) (Math|Float|Lerp (.yaw _returnvalue) _endrotationdegrees _rotate)))
                  (Variables|Default|SetCurrentlyRotating true))))
            (:Finished
              (goto _label)))
          (else
            (Utilities|FlowControl|DoOnce false
              (:Completed
                (Timeline|Rotation PlayFromStart))))))
      (:B
        (if (Variables|Default|GetAllowSeveralRotations)
          (bind _rotate_2 (Timeline|RotationBackwards PlayFromStart)
            (:Update
              (if (<= (.yaw _returnvalue_2) (+ _revereendrotationdegrees 1.0))
                (Variables|Default|SetCurrentlyRotating false :!label _label_2)
                (else
                  (Transformation|SetActorRotation (Math|Rotator|MakeRotator (.roll _returnvalue_2) (.pitch _returnvalue_2) (Math|Float|Lerp (.yaw _returnvalue_2) _revereendrotationdegrees _rotate_2)))
                  (Variables|Default|SetCurrentlyRotating true))))
            (:Finished
              (goto _label_2))))))))

(event Custom|ResetDoOnce
  (bind _returnvalue (Transformation|GetActorRotation))
  (bind _endrotationdegrees (Variables|Default|GetEndRotationDegrees))
  ;[1 1 1] Rotate Platform
  (Utilities|FlowControl|DoOnce false) ; enters at Reset
)

(event EventBeginPlay
  (|CallParentFunction) ; This node is disabled and will not be called.\nDrag off pins to build functionality.
)

(event Collision|EventActorBeginOverlap
  (params (OtherActor :type Actor%20Object%20Reference))
  (|CallParentFunction OtherActor) ; This node is disabled and will not be called.\nDrag off pins to build functionality.
)

(event EventTick
  (params (DeltaSeconds :type Float%20%28single-precision%29))
  (|CallParentFunction DeltaSeconds) ; This node is disabled and will not be called.\nDrag off pins to build functionality.
)

(fn ConstructionScript
  (|CallParentFunction))

(fn FInteraction
  (CallFunction|TriggerRotationEffect))