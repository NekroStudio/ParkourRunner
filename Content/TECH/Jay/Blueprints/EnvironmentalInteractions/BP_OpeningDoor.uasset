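; Two-panel sliding door that opens by interaction, or automatically on player overlap when AutoOpen is set.
; Two timelines move the meshes in opposite directions from their starting positions and reverse when the player leaves in auto mode.
; Registered enemies are removed as they are deducted, and the counter reaching zero enables AutoOpen.
; Unlocking this way also triggers brief global slow motion, which a looping timer restores to normal speed.
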(event OnComponentBeginOverlap(WalkableCollision)
  (params (OverlappedComponent :type Primitive%20Component%20Object%20Reference) (OtherActor :type Actor%20Object%20Reference) (OtherComp :type Primitive%20Component%20Object%20Reference) (OtherBodyIndex :type Integer) (bFromSweep :type Boolean) (SweepResult :type Hit%20Result%20Structure%20%28by%20ref%29))
  ;[1 1 1] Open when player walks into collision
  (Utilities|MIsPlayer OtherActor
    (:true
      (if (Variables|Default|GetAutoOpen)
        (CallFunction|TriggerOpening)))))

(event OnComponentEndOverlap(WalkableCollision)
  (params (OverlappedComponent :type Primitive%20Component%20Object%20Reference) (OtherActor :type Actor%20Object%20Reference) (OtherComp :type Primitive%20Component%20Object%20Reference) (OtherBodyIndex :type Integer))
  ;[1 1 1] Open when player walks into collision
  (Utilities|MIsPlayer OtherActor
    (:true
      (if (Variables|Default|GetAutoOpen)
        (CallFunction|ReverseOpening)))))

(event Custom|TriggerInteraction
  ;[1 1 1] Open door based on timeline
  (if (not (Variables|Default|GetAutoOpen))
    (Utilities|FlowControl|Sequence
      (:then_0
        (bind _move (Timeline|OpenDoor PlayFromStart)
          (:Update
            (Transformation|SetRelativeLocation (Variables|Character|GetMesh) (+ (* _move (Variables|Default|GetMovementAmount)) (Variables|Default|GetM1CurrentRelativeLoc)) false false))))
      (:then_1
        (bind _move_2 (Timeline|Timeline_0 PlayFromStart)
          (:Update
            (Transformation|SetRelativeLocation (Variables|Default|GetSecondMesh) (+ (* _move_2 (* (Variables|Default|GetMovementAmount) -1.0)) (Variables|Default|GetM2CurrentRelativeLoc)) false false)))))))

(event Custom|TriggerOpening
  ;[1 1 1] Open door based on timeline
  (Utilities|FlowControl|Sequence
    (:then_0
      (bind _move (Timeline|OpenDoor PlayFromStart)
        (:Update
          (Transformation|SetRelativeLocation (Variables|Character|GetMesh) (+ (* _move (Variables|Default|GetMovementAmount)) (Variables|Default|GetM1CurrentRelativeLoc)) false false))))
    (:then_1
      (bind _move_2 (Timeline|Timeline_0 PlayFromStart)
        (:Update
          (Transformation|SetRelativeLocation (Variables|Default|GetSecondMesh) (+ (* _move_2 (* (Variables|Default|GetMovementAmount) -1.0)) (Variables|Default|GetM2CurrentRelativeLoc)) false false))))))

(event Custom|ReverseOpening
  ;[1 1 1] Open door based on timeline
  (Utilities|FlowControl|Sequence
    (:then_0
      (bind _move (Timeline|OpenDoor Reverse)
        (:Update
          (Transformation|SetRelativeLocation (Variables|Character|GetMesh) (+ (* _move (Variables|Default|GetMovementAmount)) (Variables|Default|GetM1CurrentRelativeLoc)) false false))))
    (:then_1
      (bind _move_2 (Timeline|Timeline_0 Reverse)
        (:Update
          (Transformation|SetRelativeLocation (Variables|Default|GetSecondMesh) (+ (* _move_2 (* (Variables|Default|GetMovementAmount) -1.0)) (Variables|Default|GetM2CurrentRelativeLoc)) false false))))))

(event Custom|UnlockDoor
  ;[1 1 1] Unlock door
  (Variables|Default|SetAutoOpen true))

(event Custom|TriggerTimeSlow
  ;[1 1 1] Trigger time slow
  (Utilities|Time|SetGlobalTimeDilation 0.1)
  (Variables|Default|SetGlobalTime 0.1)
  (Utilities|FlowControl|Delay 0.05)
  (CallFunction|TriggerResetTime))

(event Custom|TriggerResetTime
  ;[1 1 1] Reset time slow
  (bind _returnvalue (Utilities|Time|SetTimerbyEvent (delegate Custom|ResetTime) 0.0005 true))
  (Variables|Default|SetResetTimeHandle _returnvalue))

(event Custom|ResetTime
  ;[1 1 1] Reset time slow
  (bind _output_get (Variables|Default|SetGlobalTime (+ (Variables|Default|GetGlobalTime) 0.01)))
  (Utilities|Time|SetGlobalTimeDilation 1.0)
  (if (>= _output_get (Variables|Default|GetMaxGlobalTime))
    (Utilities|Time|ClearandInvalidateTimerbyHandle (Variables|Default|GetResetTimeHandle))
    (Utilities|Time|SetGlobalTimeDilation 1.0)))

(event EventBeginPlay
  ;[1 1 1] Store starting location
  (|CallParentFunction)
  (Variables|Default|SetM1CurrentRelativeLoc (Variables|/Script/Engine.SceneComponent|GetRelativeLocation (Variables|Character|GetMesh)))
  (Variables|Default|SetM2CurrentRelativeLoc (Variables|/Script/Engine.SceneComponent|GetRelativeLocation (Variables|Default|GetSecondMesh))))

(event EventISetupDoor
  (params (ConnectedEnemy :type BP%20Base%20Enemy%20Object%20Reference))
  ;[1 1 1] Store all connected enemies
  (Utilities|Array|Add (Variables|Default|GetConnected%20Enemy) ConnectedEnemy))

(event EventIDeductEnemy
  (params (EnemyToRemove :type BP%20Base%20Enemy%20Object%20Reference))
  (bind _numofenemiestounlockdoor (Variables|Default|GetNumOfEnemiesToUnlockDoor))
  ;[1 1 1] Deduct enemy from total counter
  (if (Utilities|Array|ContainsItem (Variables|Default|GetConnected%20Enemy) EnemyToRemove)
    (Math|Integer|DecrementInt _numofenemiestounlockdoor
      (:%20%20
        (Utilities|Array|RemoveItem (Variables|Default|GetConnected%20Enemy) EnemyToRemove)
        (if (<= _numofenemiestounlockdoor 0)
          (CallFunction|UnlockDoor)
          (CallFunction|TriggerTimeSlow))))))

(fn ConstructionScript
  (|CallParentFunction))

(fn FInteraction
  (CallFunction|TriggerInteraction))

(fn IGetCheckPointActiveTime
  (return 0.0))

(fn IGetTime
  (return 0.0))

(fn IGetKilledEnemies
  (return 0))

(fn IConvertSaveSlot
  (return 0))