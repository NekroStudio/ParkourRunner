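; Player grappling hook component that pulls the character to grapple points or triggers puzzle grapple points.
; A looping timer runs a Retracted, Fired, Near Target, At Target state machine, using a camera-direction line trace to select targets.
; TryToGrapple spawns a hook with a hand-attached cable.
; Regular points drive character velocity, reducing it on release and notifying parkour for instant mantle or wall run; puzzle points receive a hit message instead.
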(event Custom|Init
  (params (OwningCharacter :type BP%20Base%20Character%20Object%20Reference))
  ;[1 1 1] Store character
  (Variables|References|SetCharacter OwningCharacter)
  (CallFunction|FStoreAllGrapplePoints)
  (CallFunction|TriggerGrappleStates))

(event Custom|Trigger%20GrappleStates
  ;[1 1 1] Grapple States Timer
  (bind _returnvalue (Utilities|Time|SetTimerbyEvent (EventDispatchers|CreateEvent :!event Custom|GrappleStates) 0.001 true))
  (Variables|CoreVariables|SetGrappleLoopingHandle _returnvalue))

(event Custom|GrappleStates
  ;[1 1 1] Switch states
  (if (Utilities|MCheckCurrentPlayerDistance)
    (switch Utilities|FlowControl|Switch|SwitchonE_CurrentGrappleState (Variables|CoreVariables|GetCurrentGrappleState)
      (:NewEnumerator0
        (CallFunction|FRetracted))
      (:NewEnumerator1
        (CallFunction|FFired))
      (:NewEnumerator2
        (CallFunction|FNearTarget))
      (:NewEnumerator3
        (CallFunction|FatTarget)))
    (else
      (bind _currentgrappletarget (Variables|References|GetCurrentGrappleTarget)
        (:then
          (Default|FToggleVisibility _currentgrappletarget "NewEnumerator0"))
        (:else
          (bind _puzzlegrappletarget (Variables|References|GetPuzzleGrappleTarget)
            (:then
              (Default|FToggleVisibility _puzzlegrappletarget "NewEnumerator0"))
            (:else
              _))))
      (CallFunction|FNullVariables))))

(fn FRetracted
  (bind (_foundgrapplepoint _puzzle_grapple_points) (CallFunction|FFindTarget))
  (if (!= _foundgrapplepoint 0)
    (CallFunction|FSetCurrentGrappleTarget _foundgrapplepoint)
    (elif (!= _puzzle_grapple_points 0)
      (CallFunction|FSetCurrentPuzzleGrappleTarget _puzzle_grapple_points))))

(fn FFired
  (if (< (Default|FDistancetoTarget (Variables|References|GetGrappleHook)) (Variables|EditableElements|GetNearTargetDistance))
    (Variables|CoreVariables|SetCurrentGrappleState "NewEnumerator2")))

(fn FNearTarget
  (if (<= (.z (Transformation|GetVelocity (Variables|References|GetCharacter))) 0.0)
    ;[1 1 1] So player is in air and then can be pulled
    (Variables|References|GetCurrentGrappleTarget
      (:then
        (Character|LaunchCharacter (Variables|References|GetCharacter) "0, 0,1.000000" true true)
        (Variables|CoreVariables|SetInitialRotationDirection (Utilities|MRotatetoTarget)))
      (:else
        _))
    (Variables|CoreVariables|SetCurrentGrappleState "NewEnumerator3")))

(fn FatTarget
  (bind _character (Variables|References|GetCharacter))
  (bind _character_2 (Variables|References|GetCharacter))
  (bind _returnvalue (Pawn|GetMovementComponent _character))
  (bind _currentgrappletarget (Variables|References|GetCurrentGrappleTarget)
    (:then
      (Utilities|FlowControl|Sequence
        (:then_0
          (if (or (< (Transformation|GetDistanceTo _character_2 _currentgrappletarget) (Variables|EditableElements|GetCloseToPointDistance)) (and (Variables|Default|GetCanDrop) (<= (.z (Transformation|GetVelocity _character_2)) (Variables|Default|GetLowVelocity))))
            (Variables|/Script/Engine.MovementComponent|SetVelocity _returnvalue (* (Utilities|MRotatetoTarget) (/ (Variables|EditableElements|GetCharacterGrappleSpeed) (Variables|EditableElements|GetMaxVelocityDivisionCap))))
            ;[1 1 1] Allows for instant mantle and wall run
            (Class|BPiParkour|IFreshGrapple(Message) (Variables|/Game/TECH/Jay/BP_BaseCharacter.BP_BaseCharacter_C|GetBP_ParkourMovement (Variables|References|GetCharacter)) true)
            (Variables|/Script/Engine.CharacterMovementComponent|SetGravityScale (Variables|/Script/Engine.Character|GetCharacterMovement (Variables|References|GetCharacter)) 2.0)
            (CallFunction|FSetCurrentGrappleTarget :!label _label)
            (CallFunction|FSetCurrentPuzzleGrappleTarget)
            (Actor|DestroyActor (Variables|References|GetGrappleCable))
            (Variables|References|SetGrappleCable 0)
            (Variables|References|SetGrappleHook 0)
            (Variables|CoreVariables|SetCurrentGrappleState "NewEnumerator0")
            (Variables|Default|SetLowVelocity 0.0)
            (Variables|Default|SetCanDrop false)
            (else
              (Variables|/Script/Engine.MovementComponent|SetVelocity _returnvalue (* (Utilities|MRotatetoTarget) (Variables|EditableElements|GetCharacterGrappleSpeed))))))))
    (:else
      (bind _puzzlegrappletarget (Variables|References|GetPuzzleGrappleTarget)
        (:then
          (if (< (Transformation|GetDistanceTo (Variables|References|GetGrappleHook) _puzzlegrappletarget) (/ (Variables|EditableElements|GetCloseToPointDistance) 2.0))
            (Class|BPIGrapplePointElements|IPuzzleGrapplePointHit(Message) _puzzlegrappletarget)
            (goto _label)))
        (:else
          (Development|PrintString "NOT VALID TARGET"))))))

(fn FFindTarget
  (bind _character (Variables|References|GetCharacter))
  (bind _returnvalue (Transformation|GetActorLocation _character))
  (bind (_x _y _z) (Math|Vector|BreakVector _returnvalue))
  (bind _returnvalue_2 (+ _z 5e+01))
  (bind _returnvalue_3 (Math|Vector|MakeVector _x _y _returnvalue_2))
  ;[1 1 1] Draw linetrace to character from target to find the closest one
  (bind (_outhit _returnvalue_4) (Collision|LineTraceByChannel _returnvalue_3 (+ _returnvalue_3 (* (Math|Vector|GetForwardVector (Transformation|GetWorldRotation (Variables|/Game/TECH/Jay/BP_BaseCharacter.BP_BaseCharacter_C|GetCamera _character))) (Variables|EditableElements|GetMaxGrappleDistance))) "TraceTypeQuery2" false (Utilities|Array|MakeArray (Variables|References|GetCharacter)) "None" true "(R=1.000000,G=0.000000,B=0.000000,A=1.000000)" "(R=0.000000,G=1.000000,B=0.000000,A=1.000000)" 0.2))
  (if _returnvalue_4
    (if (.bSuccess (Utilities|Casting|CastToBP_GrapplePoint (.HitActor (Collision|BreakHitResult _outhit))))
      (return (.AsBP%20Grapple%20Point (Utilities|Casting|CastToBP_GrapplePoint (.HitActor (Collision|BreakHitResult _outhit)))) (.AsBP%20Puzzle%20Grapple%20Points (Utilities|Casting|CastToBP_PuzzleGrapplePoints (.HitActor (Collision|BreakHitResult _outhit)))))
      (elif (.bSuccess (Utilities|Casting|CastToBP_PuzzleGrapplePoints (.HitActor (Collision|BreakHitResult _outhit))))
        (return (.AsBP%20Grapple%20Point (Utilities|Casting|CastToBP_GrapplePoint (.HitActor (Collision|BreakHitResult _outhit)))) (.AsBP%20Puzzle%20Grapple%20Points (Utilities|Casting|CastToBP_PuzzleGrapplePoints (.HitActor (Collision|BreakHitResult _outhit)))))))
    (else
      (Class|BPIGrapplePointElements|ICannotSeePoint(Message) (Variables|References|GetCurrentGrappleTarget))
      (Class|BPIGrapplePointElements|ICannotSeePoint(Message) (Variables|References|GetPuzzleGrappleTarget))
      (Variables|References|SetCurrentGrappleTarget 0)
      (Variables|References|SetPuzzleGrappleTarget 0))))

(fn FSetCurrentGrappleTarget
  (params (NewTarget :type BP%20Grapple%20Point%20Object%20Reference))
  (if (== NewTarget (Variables|References|GetCurrentGrappleTarget))
    (Class|BPIGrapplePointElements|ICanSeePoint(Message) (Variables|References|GetCurrentGrappleTarget))
    (else
      (Utilities|FlowControl|Sequence
        (:then_0
          (bind _currentgrappletarget (Variables|References|GetCurrentGrappleTarget)
            (:then
              (Class|BPIGrapplePointElements|ICannotSeePoint(Message) _currentgrappletarget))
            (:else)))
        (:then_1
          (Variables|References|SetCurrentGrappleTarget NewTarget))
        (:then_2
          (bind _currentgrappletarget_2 (Variables|References|GetCurrentGrappleTarget)
            (:then
              (Class|BPIGrapplePointElements|ICanSeePoint(Message) _currentgrappletarget_2))
            (:else)))))))

(fn FTrytoGrapple
  (switch Utilities|FlowControl|Switch|SwitchonE_CurrentGrappleState (Variables|CoreVariables|GetCurrentGrappleState)
    (:NewEnumerator0
      (bind _currentgrappletarget (Variables|References|GetCurrentGrappleTarget) ; Is grapple Valid
        (:then
          ;[1 1 1] Spawn grapple hook and cable
          (bind _returnvalue (Game|SpawnActorfromClass "/Game/TECH/Jay/Blueprints/GrappleElements/BP_GrappleHook.BP_GrappleHook_C" (Math|Transform|MakeTransform (Utilities|MPlayerLocation) "0, 0, 0" "1,1,1") "AlwaysSpawn" 0 _currentgrappletarget 5e+03 0))
          (Variables|References|SetGrappleHook _returnvalue)
          (bind _returnvalue_2 (Game|SpawnActorfromClass "/Game/TECH/Jay/Blueprints/GrappleElements/BP_GrappleCable.BP_GrappleCable_C" (Math|Transform|MakeTransform (Utilities|MPlayerLocation) "0, 0, 0" "1,1,1") "AlwaysSpawn" 0 0))
          ;[1 1 1] Attach them to the character
          (bind _output_get (Variables|References|SetGrappleCable _returnvalue_2))
          (Transformation|AttachComponentToComponent _output_get (Variables|/Script/Engine.Character|GetMesh (Variables|References|GetCharacter)) "index_03_l" "SnapToTarget" "SnapToTarget" "SnapToTarget" true)
          (Class|CableComponent|SetAttachEndto (Variables|/Script/CableComponent.CableActor|GetCableComponent (Variables|References|GetGrappleCable)) (Variables|References|GetGrappleHook) "DefaultSceneRoot" "None")
          (Transformation|SetActorRotation (Variables|References|GetCharacter) (Math|Rotator|MakeRotfromZX (Math|Vector|MakeVector 0.0 0.0 1.0) (Utilities|MRotatetoTarget)))
          (Variables|CoreVariables|SetCurrentGrappleState "NewEnumerator1"))
        (:else
          (bind _puzzlegrappletarget (Variables|References|GetPuzzleGrappleTarget)
            (:then
              ;[1 1 1] Spawn grapple hook and cable
              (bind _returnvalue_3 (Game|SpawnActorfromClass "/Game/TECH/Jay/Blueprints/GrappleElements/BP_GrappleHook.BP_GrappleHook_C" (Math|Transform|MakeTransform (Utilities|MPlayerLocation) "0, 0, 0" "1,1,1") "AlwaysSpawn" 0 _puzzlegrappletarget 5e+03 0))
              (Variables|References|SetGrappleHook _returnvalue_3)
              (bind _returnvalue_4 (Game|SpawnActorfromClass "/Game/TECH/Jay/Blueprints/GrappleElements/BP_GrappleCable.BP_GrappleCable_C" (Math|Transform|MakeTransform (Utilities|MPlayerLocation) "0, 0, 0" "1,1,1") "AlwaysSpawn" 0 0))
              ;[1 1 1] Attach them to the character
              (bind _output_get_2 (Variables|References|SetGrappleCable _returnvalue_4))
              (Transformation|AttachComponentToComponent _output_get_2 (Variables|/Script/Engine.Character|GetMesh (Variables|References|GetCharacter)) "index_03_l" "SnapToTarget" "SnapToTarget" "SnapToTarget" true)
              (Class|CableComponent|SetAttachEndto (Variables|/Script/CableComponent.CableActor|GetCableComponent (Variables|References|GetGrappleCable)) (Variables|References|GetGrappleHook) "DefaultSceneRoot" "None")
              (Variables|CoreVariables|SetCurrentGrappleState "NewEnumerator1"))
            (:else)))))))

(fn FStoreAllGrapplePoints
  (bind _outactors (Actor|GetAllActorsOfClass "/Game/TECH/Jay/Blueprints/GrappleElements/GrapplePoints/BP_GrapplePoint.BP_GrapplePoint_C"))
  (for _array_element _outactors
    (Utilities|Array|Add (Variables|References|GetAllGrapplePoints) _array_element))
  (return))

(fn FNullVariables
  (CallFunction|FSetCurrentGrappleTarget)
  (CallFunction|FSetCurrentPuzzleGrappleTarget)
  (bind _grapplecable (Variables|References|GetGrappleCable)
    (:then
      (Actor|DestroyActor _grapplecable)
      (bind _grapplehook (Variables|References|GetGrappleHook)
        (:then
          (Actor|DestroyActor _grapplehook)
          (Variables|References|SetGrappleCable 0)
          (Variables|References|SetGrappleHook 0)
          (Variables|CoreVariables|SetCurrentGrappleState "NewEnumerator0")
          (Variables|Default|SetLowVelocity 0.0)
          (Variables|Default|SetCanDrop false))
        (:else)))
    (:else)))

(fn FSetCurrentPuzzleGrappleTarget
  (params (NewPuzzleGrappleTarget :type BP%20Puzzle%20Grapple%20Points%20Object%20Reference))
  (if (== NewPuzzleGrappleTarget (Variables|References|GetPuzzleGrappleTarget))
    (Class|BPIGrapplePointElements|ICanSeePoint(Message) (Variables|References|GetPuzzleGrappleTarget))
    (else
      (Utilities|FlowControl|Sequence
        (:then_0
          (bind _puzzlegrappletarget (Variables|References|GetPuzzleGrappleTarget)
            (:then
              (Class|BPIGrapplePointElements|ICannotSeePoint(Message) _puzzlegrappletarget))
            (:else)))
        (:then_1
          (Variables|References|SetPuzzleGrappleTarget NewPuzzleGrappleTarget))
        (:then_2
          (bind _puzzlegrappletarget_2 (Variables|References|GetPuzzleGrappleTarget)
            (:then
              (Class|BPIGrapplePointElements|ICanSeePoint(Message) _puzzlegrappletarget_2))
            (:else)))))))

(fn FChangeLowVelocity
  (Variables|Default|SetLowVelocity 2e+01)
  (Variables|Default|SetCanDrop true)
  (Development|PrintString "Hello"))