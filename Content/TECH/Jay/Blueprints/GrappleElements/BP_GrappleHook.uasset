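; BP_GrappleHook is the grapple hook projectile that flies from its spawn location to a target point actor and stops there.
; BeginPlay aims the projectile movement at the target, first letting an active BP_PillarZone update the hook speed in the Wave Based Runner gamemode.
; A looping timer, set to the frame delta, compares squared travel distances to catch overshoot, then snaps the hook onto the target, zeroes velocity and clears itself.
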(event Custom|TriggerGrappleHookDistance
  ;[1 1 1] Checks to see if the current cable is at the target.
  (bind _returnvalue (Utilities|Time|SetTimerbyFunctionName 0 "F_CheckCurrentGrappleCable" (Utilities|Time|GetWorldDeltaSeconds) true))
  (Variables|Default|SetGrappleHookLoopingHandle _returnvalue))

(event EventBeginPlay
  ;[1 1 1] Store variables
  (Variables|Default|SetStartLoc (Transformation|GetActorLocation))
  (Variables|Default|SetEndLoc (Transformation|GetActorLocation (Variables|Default|GetTargetPoint)))
  (Variables|Default|SetHookDirection (Math|Vector|Normalize (- (Variables|Default|GetEndLoc) (Variables|Default|GetStartLoc))))
  (bind _currentgamemode (Class|BPIGamemodeElements|ICurrentGamemode(Message) (Game|GetGameMode)))
  (switch Utilities|FlowControl|Switch|SwitchonE_CurrentGamemode _currentgamemode
    (:NewEnumerator0
      _)
    (:NewEnumerator1
      (bind _returnvalue (Actor|GetActorOfClass "/Game/TECH/Jay/WaveMode/UpgradeEffects/BP_PillarZone.BP_PillarZone_C"))
      (Utilities|IsValid _returnvalue
        (:Is%20Valid
          (if (Variables|/Game/TECH/Jay/WaveMode/UpgradeEffects/BP_PillarZone.BP_PillarZone_C|GetIsCurrentlyActive _returnvalue)
            (Default|UpdateGrappleHookSpeed _returnvalue self)))
        (:Is%20Not%20Valid
          _)))
    (:NewEnumerator2
      _)
    (:NewEnumerator3
      _))
  (Variables|/Script/Engine.MovementComponent|SetVelocity (Variables|Default|GetProjectileMovement) (* (Variables|Default|GetHookDirection) (Variables|Default|GetGrappleHookSpeed)))
  (CallFunction|TriggerGrappleHookDistance))

(fn ConstructionScript)

(fn FDistancetoTarget
  (return (Math|Vector|Distance(Vector) (Variables|Default|GetEndLoc) (Transformation|GetActorLocation))))

(fn FCheckCurrentGrappleCable
  ;[1 1 1] Has the cable reached or gone past the grapple point.
  (if (>= (Class|KismetMathLibrary|VectorDistanceSquared (Transformation|GetActorLocation) (Variables|Default|GetStartLoc)) (Class|KismetMathLibrary|VectorDistanceSquared (Transformation|GetActorLocation (Variables|Default|GetTargetPoint)) (Variables|Default|GetStartLoc)))
    (Transformation|SetActorLocation (+ (Variables|Default|GetStartLoc) (* (Variables|Default|GetHookDirection) (Math|Vector|Distance(Vector) (Variables|Default|GetStartLoc) (Variables|Default|GetEndLoc)))) false true)
    (Variables|/Script/Engine.MovementComponent|SetVelocity (Variables|Default|GetProjectileMovement) "0, 0, 0")
    (Utilities|Time|ClearandInvalidateTimerbyHandle (Variables|Default|GetGrappleHookLoopingHandle))))