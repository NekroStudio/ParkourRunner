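; Base grapple point actor that shows a spatial UI widget and switches its visibility state by player range and sight.
; An outer sphere, sized from max grapple distance, shows or hides the widget; interface seen/unseen events alternate states through paired DoOnce gates.
; An inner collision ignores camera and visibility channels while the player overlaps, preventing re-grappling the same point.
; A helper converts the pull offset to world space.
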(event OnComponentBeginOverlap(StopGrappleCollision)
  (params (OverlappedComponent :type Primitive%20Component%20Object%20Reference) (OtherActor :type Actor%20Object%20Reference) (OtherComp :type Primitive%20Component%20Object%20Reference) (OtherBodyIndex :type Integer) (bFromSweep :type Boolean) (SweepResult :type Hit%20Result%20Structure%20%28by%20ref%29))
  (bind _stopgrapplecollision (Variables|Default|GetStopGrappleCollision))
  ;[1 1 1] Prevent player from grappling to same point when in radius
  (Utilities|MIsPlayer OtherActor
    (:true
      (Collision|SetCollisionResponsetoChannel _stopgrapplecollision "ECC_Camera" "ECR_Ignore")
      (Collision|SetCollisionResponsetoChannel _stopgrapplecollision "ECC_Visibility" "ECR_Ignore")
      (CallFunction|FToggleVisibility "NewEnumerator0"))))

(event OnComponentEndOverlap(StopGrappleCollision)
  (params (OverlappedComponent :type Primitive%20Component%20Object%20Reference) (OtherActor :type Actor%20Object%20Reference) (OtherComp :type Primitive%20Component%20Object%20Reference) (OtherBodyIndex :type Integer))
  (bind _stopgrapplecollision (Variables|Default|GetStopGrappleCollision))
  ;[1 1 1] Prevent player from grappling to same point when in radius
  (Utilities|MIsPlayer OtherActor
    (:true
      (Collision|SetCollisionResponsetoChannel _stopgrapplecollision "ECC_Camera" "ECR_Block")
      (Collision|SetCollisionResponsetoChannel _stopgrapplecollision "ECC_Visibility" "ECR_Block")
      (CallFunction|FToggleVisibility "NewEnumerator1"))))

(event OnComponentBeginOverlap(InGrappleRange)
  (params (OverlappedComponent :type Primitive%20Component%20Object%20Reference) (OtherActor :type Actor%20Object%20Reference) (OtherComp :type Primitive%20Component%20Object%20Reference) (OtherBodyIndex :type Integer) (bFromSweep :type Boolean) (SweepResult :type Hit%20Result%20Structure%20%28by%20ref%29))
  ;[1 1 1] Grapple range collision
  (Utilities|MIsPlayer OtherActor
    (:true
      (CallFunction|FToggleVisibility "NewEnumerator1"))))

(event OnComponentEndOverlap(InGrappleRange)
  (params (OverlappedComponent :type Primitive%20Component%20Object%20Reference) (OtherActor :type Actor%20Object%20Reference) (OtherComp :type Primitive%20Component%20Object%20Reference) (OtherBodyIndex :type Integer))
  ;[1 1 1] Grapple range collision
  (Utilities|MIsPlayer OtherActor
    (:true
      (CallFunction|FToggleVisibility "NewEnumerator0"))))

(event EventBeginPlay
  ;[1 1 1] Begin play - create spatial widget and toggle it off
  (bind _returnvalue (UserInterface|CreateWidget (Variables|Default|GetWidgetToCreate)))
  (Variables|Default|SetCreatedGrappleWidget _returnvalue)
  (UserInterface|SetWidget (Variables|Default|GetGrapplePointWidget) _returnvalue)
  (CallFunction|FToggleVisibility "NewEnumerator0"))

(event EventICanSeePoint
  ;[1 1 1] Point Detection for UI
  (Utilities|FlowControl|DoOnce false
    (:Completed
      (CallFunction|FToggleVisibility "NewEnumerator2")
      (Utilities|FlowControl|DoOnce false) ; enters at Reset
    )))

(event EventICannotSeePoint
  ;[1 1 1] Point Detection for UI
  (Utilities|FlowControl|DoOnce false
    (:Completed
      (CallFunction|FToggleVisibility "NewEnumerator1")
      (Utilities|FlowControl|DoOnce false) ; enters at Reset
    )))

(fn ConstructionScript
  (Components|Sphere|SetSphereRadius (Variables|Default|GetLookAtGrappleCollision) (Variables|Default|GetGP%20Hit%20Collision%20Radius) true)
  (bind _output_get (Variables|Default|SetGP%20Activate%20Radius (* (Variables|Default|GetMaxGrappleDistance) 1.3)))
  (Components|Sphere|SetSphereRadius (Variables|Default|GetInGrappleRange) _output_get true))

(fn FToggleVisibility
  (params (GrapplePointState :type E_GrapplePointState%20Enum :default "NewEnumerator0"))
  (Class|BPIGrapplePointElements|IToggleVisibility(Message) (Variables|Default|GetCreatedGrappleWidget) GrapplePointState))

(fn FGetOffsetTargetLoc
  (return (Math|Transform|TransformLocation (Transformation|GetActorTransform) (Variables|Default|GetCharacterPullOffset))))