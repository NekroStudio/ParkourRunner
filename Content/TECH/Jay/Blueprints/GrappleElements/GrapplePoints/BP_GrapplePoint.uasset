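; BP_GrapplePoint is a grapple point element that extends a parent class, which handles its construction and begin-play logic.
; An interface event sets the blocking grapple size by applying the given radius to the StopGrappleCollision sphere.
; The same event derives a proportionally smaller radius for the LookAtGrappleCollision sphere, keeping the hit and stop volumes scaled together.
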(event EventITweakBlockingGrappleSize
  (params (Radius :type Float%20%28single-precision%29))
  ;[1 1 1] Update grapple elements
  (bind _output_get (Variables|Default|SetGP%20StopGrappleCollisionRadius Radius))
  (Components|Sphere|SetSphereRadius (Variables|Default|GetStopGrappleCollision) _output_get true)
  (bind _output_get_2 (Variables|Default|SetGP%20Hit%20Collision%20Radius (/ _output_get 1.65)))
  (Components|Sphere|SetSphereRadius (Variables|Default|GetLookAtGrappleCollision) _output_get_2 true))

(event EventBeginPlay
  ;[1 1 1] Begin play
  (|CallParentFunction))

(fn ConstructionScript
  (|CallParentFunction))