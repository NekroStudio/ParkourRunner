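; BP_BaseHazard is a base actor for hazards, providing shared player-detection logic around a Collision component.
; Begin and end overlaps on that component pass through an IsPlayer macro, so only the player triggers F_EnteredCollision and F_ExitedCollision.
; Both functions are empty here, acting as hooks for child hazards to fill in, and the default BeginPlay, Tick and actor overlap events are unused.
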(event OnComponentBeginOverlap(Collision)
  (params (OverlappedComponent :type Primitive%20Component%20Object%20Reference) (OtherActor :type Actor%20Object%20Reference) (OtherComp :type Primitive%20Component%20Object%20Reference) (OtherBodyIndex :type Integer) (bFromSweep :type Boolean) (SweepResult :type Hit%20Result%20Structure%20%28by%20ref%29))
  (Utilities|MIsPlayer OtherActor
    (:true
      (CallFunction|FEnteredCollision OtherActor))))

(event OnComponentEndOverlap(Collision)
  (params (OverlappedComponent :type Primitive%20Component%20Object%20Reference) (OtherActor :type Actor%20Object%20Reference) (OtherComp :type Primitive%20Component%20Object%20Reference) (OtherBodyIndex :type Integer))
  (Utilities|MIsPlayer OtherActor
    (:true
      (CallFunction|FExitedCollision OtherActor))))

(event EventBeginPlay
  (|CallParentFunction) ; This node is disabled and will not be called.\nDrag off pins to build functionality.
)

(event Collision|EventActorBeginOverlap
  (params (OtherActor :type Actor%20Object%20Reference))
  (|CallParentFunction OtherActor) ; This node is disabled and will not be called.\nDrag off pins to build functionality.
)

(event EventTick
  (params (DeltaSeconds :type Float%20%28single-precision%29))
  (|CallParentFunction DeltaSeconds) ; This node is disabled and will not be called.\nDrag off pins to build functionality.
)

(fn ConstructionScript
  (|CallParentFunction))

(fn FEnteredCollision
  (params (Actor :type Actor%20Object%20Reference)))

(fn FExitedCollision
  (params (Actor :type Actor%20Object%20Reference)))