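; Score system that awards the player points for kills and checkpoint times, tracking them in the character's save game.
; After a delayed init binds it to the character's score event, score updates poll until the save is valid, then load the save slot to skip already-scored enemies.
; New scores and killed enemies are recorded before writing the slot.
; Checkpoint points scale with average over active time, rounded to a multiple, and print for debugging.
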(event Custom|Init
  (params (Character :type BP%20Base%20Character%20Object%20Reference))
  ;[1 1 1] Init chain
  (Utilities|FlowControl|Delay 0.3) ; Delay for init chain (for save game)
  (bind _output_get (Variables|Default|SetCharacter Character))
  (Variables|Default|SetSave%20Game (Variables|/Game/TECH/Jay/BP_BaseCharacter.BP_BaseCharacter_C|GetSaveGameRef _output_get))
  (CallFunction|FBindings))

(event Custom|UpdateScore
  (params (ScoreGained :type Integer) (KilledEnemy :type BP%20Base%20Enemy%20Object%20Reference))
  (bind _save_game (Variables|Default|GetSave%20Game))
  ;[1 1 1] Update score
  ;;[1 1 1] Check if save is valid - if not, wait till valid
  (Variables|Default|SetKilledEnemy KilledEnemy)
  (Variables|Default|GetSave%20Game :!label _label
    (:then
      (bind _returnvalue (SaveGame|LoadGamefromSlot "Save1"))
      (bind _saveslot (Class|ISaveGame|IConvertSaveSlot(Message) _returnvalue))
      ;;[1 1 1] If enemy has NOT been killed once before
      (Variables|Default|GetKilledEnemy
        (:then
          (if (not (Utilities|Array|ContainsItem (Variables|/Game/TECH/Mitz/Blueprints/BP_SaveGame.BP_SaveGame_C|Get%28Score%29KilledEnemies _saveslot) (Variables|Default|GetKilledEnemy)))
            ;;[1 1 1] Add to existing player score and store enemy just killed
            (Variables|/Game/TECH/Mitz/Blueprints/BP_SaveGame.BP_SaveGame_C|SetPlayerScore _save_game (+ (Variables|/Game/TECH/Mitz/Blueprints/BP_SaveGame.BP_SaveGame_C|GetPlayerScore _save_game) ScoreGained) :!label _label_2)
            (bind _killedenemy (Variables|Default|GetKilledEnemy)
              (:then
                (Utilities|Array|Add (Variables|/Game/TECH/Mitz/Blueprints/BP_SaveGame.BP_SaveGame_C|Get%28Score%29KilledEnemies (Variables|Default|GetSave%20Game)) _killedenemy))
              (:else
                _))
            (CallFunction|SaveSlot)))
        (:else
          (goto _label_2))))
    (:else
      (Utilities|FlowControl|Delay 0.01)
      (goto _label))))

(event Custom|SaveSlot
  ;[1 1 1] Update score
  ;;[1 1 1] Save game
  (SaveGame|SaveGametoSlot (stale Custom|UpdateScore _saveslot) "Save1"))

(event Custom|CheckpointScore
  (params (ActiveTime :type Float%20%28single-precision%29) (AverageTime :type Float%20%28single-precision%29) (CheckpointIndex :type Integer))
  ;[1 1 1] Checkpoint score math
  (bind _roundednumber (CallFunction|FRoundtoMultiple (Math|Float|Truncate (* 50 (/ AverageTime ActiveTime))) 5))
  (CallFunction|UpdateScore _roundednumber)
  (Development|PrintString (Utilities|String|Append " 
 
 
 
Player Score: " (Utilities|String|ToString(Integer) (Variables|/Game/TECH/Mitz/Blueprints/BP_SaveGame.BP_SaveGame_C|GetPlayerScore (Variables|Default|GetSave%20Game))) " Checkpoint Index: " (Utilities|String|ToString(Integer) CheckpointIndex) " Active Time: " (Utilities|String|ToString(Float) ActiveTime)) true true "(R=1.000000,G=0.000000,B=0.072517,A=1.000000)" 1e+01))

(fn FBindings
  (EventDispatchers|BindEventtoEDUpdateScore (Variables|Default|GetCharacter) (EventDispatchers|CreateEvent :!event Custom|UpdateScore)))

(fn FRoundtoMultiple
  (params (NumberToRound :type Integer) (Multiple :type Integer))
  (bind _returnvalue (Math|Integer|Absolute(Integer) NumberToRound))
  (if (== Multiple 0)
    (LocalVariables|SetRoundedNum NumberToRound :!label _label)
    (else
      (bind _output_get (LocalVariables|SetRemainder (Math|Integer|%(Integer) _returnvalue Multiple)))
      (if (== _output_get 0)
        (goto _label)
        (elif (< _output_get 0)
          (LocalVariables|SetRoundedNum (* (- _returnvalue _output_get) -1))
          (else
            (LocalVariables|SetRoundedNum (- (+ NumberToRound Multiple) _output_get)))))))
  (return (LocalVariables|GetRoundedNum)))