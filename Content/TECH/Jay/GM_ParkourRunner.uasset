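; Game mode for the parkour runner that owns the save slot and restores player progress when a level starts.
; On init it loads or creates the save, spawns the player at PlayerStart or the saved transform, and initialises enemies, checkpoints, timer, kills and audio.
; Interface events save checkpoints, timers and buffered killed enemies, and handle restarts and level changes.
; A level-name comparison detects new levels; win and lose events are empty.
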(event Custom|Win%20Condition)

(event Custom|Lose%20Condition)

(event Custom|Init
  (bind _savegame (Variables|Default|GetSaveGame))
  ;[1 1 1] Load Game
  ;;[0 0.2846 1] Allows checkpoints to be triggered
  (Utilities|FlowControl|DoOnce false
    (:Completed
      (Utilities|FlowControl|Sequence
        (:then_0
          (bind _returnvalue (Utilities|MCheckLevel))
          (if (not _returnvalue)
            (bind _outactors (Actor|GetAllActorsOfClass "/Game/TECH/Mitz/AI/BP_BaseEnemy.BP_BaseEnemy_C"))
            (for _array_element _outactors
              (Class|ISaveGame|IInitEnemies(Message) _array_element)
              (Variables|Default|SetEnemies _outactors))))
        (:then_1
          (bind _returnvalue_2 (Utilities|MCheckLevel))
          (if (not _returnvalue_2)
            (bind _outactors_2 (Actor|GetAllActorsOfClass "/Game/TECH/Mitz/Blueprints/BP_CheckPoint.BP_CheckPoint_C"))
            (for _array_element_2 _outactors_2
              (Class|ISaveGame|IInitCheckPoints(Message) _array_element_2))
            (if (Variables|/Game/TECH/Mitz/Blueprints/BP_SaveGame.BP_SaveGame_C|GetuseSavedLocation? (Variables|Default|GetSaveGame))
              (Utilities|MSpawnSetting))))
        (:then_2
          (CallFunction|SaveGameCharacter))
        (:then_3
          (Class|ISaveGame|IInitTime(Message) (Variables|/Game/TECH/Jay/BP_PlayerController.BP_PlayerController_C|GetHUD (Variables|Default|GetPlayerController))))
        (:then_4
          (CallFunction|FCheckLevel))
        (:then_5
          (Class|ISaveGame|IInitKills(Message) (Variables|Default|GetPlayerCharacter) (Variables|/Game/TECH/Mitz/Blueprints/BP_SaveGame.BP_SaveGame_C|GetKills (Variables|Default|GetSaveGame))))
        (:then_6
          (bind _currentactivecheckpoint (Variables|/Game/TECH/Mitz/Blueprints/BP_SaveGame.BP_SaveGame_C|GetcurrentActiveCheckPoint _savegame)
            (:then
              (Class|ISaveGame|IInitActiveCheckPoint(Message) _currentactivecheckpoint (Variables|/Game/TECH/Mitz/Blueprints/BP_SaveGame.BP_SaveGame_C|GetcurrentCheckPointActiveTime _savegame) (Variables|Default|GetPlayerCharacter)))
            (:else)))
        (:then_7
          (Class|ISaveGame|ISettings(Message) (Variables|Default|GetPlayerCharacter) (Variables|/Game/TECH/Mitz/Blueprints/BP_SaveGame.BP_SaveGame_C|GetSettings (Variables|Default|GetSaveGame))))
        (:then_8
          (CallFunction|FAudio))
        (:then_9
          (CallFunction|SaveCurrentLevel))))))

(event Custom|CreateSaveFile
  ;[0.1714 1 0] Save Game
  ;;[1 1 1] Create save file
  (bind _returnvalue (SaveGame|CreateSaveGameObject "/Game/TECH/Mitz/Blueprints/BP_SaveGame.BP_SaveGame_C"))
  (bind _output_get (Variables|Default|SetSaveGame _returnvalue))
  (SaveGame|SaveGametoSlot _output_get (Variables|Default|GetSaveSlotName))
  ;;;[0 0.2846 1] Sent to character
  (Variables|/Game/TECH/Jay/BP_BaseCharacter.BP_BaseCharacter_C|SetSaveGameRef (Variables|Default|GetPlayerCharacter) (Variables|Default|GetSaveGame))
  (if (not (Variables|/Game/TECH/Mitz/Blueprints/BP_SaveGame.BP_SaveGame_C|GetuseSavedLocation? (Variables|Default|GetSaveGame)))
    (CallFunction|FFirstSave)
    (CallFunction|FCheckLevel)
    (CallFunction|Init)
    (CallFunction|SaveCurrentLevel)))

(event Custom|LoadSaveFile
  ;[1 1 1] Load Game
  (bind _returnvalue (SaveGame|LoadGamefromSlot (Variables|Default|GetSaveSlotName)))
  (bind _saveslot (Class|ISaveGame|IConvertSaveSlot(Message) _returnvalue))
  (Variables|Default|SetSaveGame _saveslot)
  (Utilities|FlowControl|Sequence
    (:then_0
      (bind _returnvalue_2 (Utilities|MCheckLevel))
      (if (not _returnvalue_2)
        (bind _outactors (Actor|GetAllActorsOfClass "/Game/TECH/Mitz/AI/BP_BaseEnemy.BP_BaseEnemy_C"))
        (for _array_element _outactors
          (Class|ISaveGame|IInitEnemies(Message) _array_element)
          (Variables|Default|SetEnemies _outactors))))
    (:then_1
      (bind _returnvalue_3 (Utilities|MCheckLevel))
      (if (not _returnvalue_3)
        (bind _outactors_2 (Actor|GetAllActorsOfClass "/Game/TECH/Mitz/Blueprints/BP_CheckPoint.BP_CheckPoint_C"))
        (for _array_element_2 _outactors_2
          (Class|ISaveGame|IInitCheckPoints(Message) _array_element_2))
        (if (Variables|/Game/TECH/Mitz/Blueprints/BP_SaveGame.BP_SaveGame_C|GetuseSavedLocation? (Variables|Default|GetSaveGame))
          (Utilities|MSpawnSetting))))
    (:then_2
      (CallFunction|SaveGameCharacter))
    (:then_3
      (Class|ISaveGame|IInitTime(Message) (Variables|/Game/TECH/Jay/BP_PlayerController.BP_PlayerController_C|GetHUD (Variables|Default|GetPlayerController))))
    (:then_4
      (CallFunction|FCheckLevel))
    (:then_5
      (Class|ISaveGame|IInitKills(Message) (Variables|Default|GetPlayerCharacter) (Variables|/Game/TECH/Mitz/Blueprints/BP_SaveGame.BP_SaveGame_C|GetKills (Variables|Default|GetSaveGame))))
    (:then_6
      (bind _currentactivecheckpoint (Variables|/Game/TECH/Mitz/Blueprints/BP_SaveGame.BP_SaveGame_C|GetcurrentActiveCheckPoint (Variables|Default|GetSaveGame))
        (:then
          (Class|ISaveGame|IInitActiveCheckPoint(Message) _currentactivecheckpoint (Variables|/Game/TECH/Mitz/Blueprints/BP_SaveGame.BP_SaveGame_C|GetcurrentCheckPointActiveTime (Variables|Default|GetSaveGame)) (Variables|Default|GetPlayerCharacter)))
        (:else)))
    (:then_7
      (Class|ISaveGame|ISettings(Message) (Variables|Default|GetPlayerCharacter) (Variables|/Game/TECH/Mitz/Blueprints/BP_SaveGame.BP_SaveGame_C|GetSettings (Variables|Default|GetSaveGame))))
    (:then_8
      (CallFunction|FAudio))
    (:then_9
      (CallFunction|SaveCurrentLevel))))

(event Custom|SaveGameCharacter
  ;[0.1714 1 0] Save Game
  ;;[1 1 1] Create save file
  ;;;[0 0.2846 1] Sent to character
  (Variables|/Game/TECH/Jay/BP_BaseCharacter.BP_BaseCharacter_C|SetSaveGameRef (Variables|Default|GetPlayerCharacter) (Variables|Default|GetSaveGame))
  (if (not (Variables|/Game/TECH/Mitz/Blueprints/BP_SaveGame.BP_SaveGame_C|GetuseSavedLocation? (Variables|Default|GetSaveGame)))
    (CallFunction|FFirstSave)
    (CallFunction|FCheckLevel)
    (CallFunction|Init)
    (CallFunction|SaveCurrentLevel)))

(event Custom|SaveCurrentLevel
  (bind _savegame (Variables|Default|GetSaveGame))
  ;[0.1714 1 0] Save Game
  ;;[1 1 1] Save Current Level
  (bind _returnvalue (Game|GetCurrentLevelName true))
  (Variables|/Game/TECH/Mitz/Blueprints/BP_SaveGame.BP_SaveGame_C|SetCurrentLevel _savegame (Utilities|String|StringToName _returnvalue))
  (SaveGame|SaveGametoSlot _savegame (Variables|Default|GetSaveSlotName)))

(event Custom|SaveGameStart
  ;[0.1714 1 0] Save Game
  ;;[1 1 1] Checks if a save exists
  (bind _returnvalue (SaveGame|DoesSaveGameExist (Variables|Default|GetSaveSlotName)))
  (if _returnvalue
    (CallFunction|LoadSaveFile)
    (else
      (CallFunction|CreateSaveFile))))

(event EventIInitCurrentGamemode
  (params (Controller :type BP%20Player%20Controller%20Object%20Reference) (Pawn :type Pawn%20Object%20Reference))
  ;[0 0.2846 1] Init
  (Variables|Default|SetPlayerController Controller)
  (CallFunction|FStoreReferences Pawn)
  (CallFunction|SaveGameStart))

(event EventIChangeLevel
  (bind _saveslotname (Variables|Default|GetSaveSlotName))
  ;[0.1714 1 0] Save Game
  ;;[1 1 1] Change level
  (bind _returnvalue (SaveGame|LoadGamefromSlot _saveslotname))
  (bind _saveslot (Class|ISaveGame|IConvertSaveSlot(Message) _returnvalue))
  (bind _output_get (Variables|Default|SetSaveGame _saveslot))
  (Variables|/Game/TECH/Mitz/Blueprints/BP_SaveGame.BP_SaveGame_C|SetuseSavedLocation? _output_get false)
  (bind _returnvalue_2 (SaveGame|SaveGametoSlot _output_get _saveslotname))
  (if _returnvalue_2
    _))

(event EventISaveGame
  (params (SpawnTransform :type Transform) (CheckPoint :type BP%20Check%20Point%20Object%20Reference) (KilledEnemies :type Array%20of%20Actor%20Object%20References) (Kills :type Integer) (CurrentActiveCP%20Index :type Integer))
  (bind _savegame (Variables|Default|GetSaveGame))
  ;[0.1714 1 0] Save Game
  ;;[1 1 1] Save Game
  (SaveGame|LoadGamefromSlot (Variables|Default|GetSaveSlotName))
  (Utilities|Array|Add (Variables|/Game/TECH/Mitz/Blueprints/BP_SaveGame.BP_SaveGame_C|GetCheckPointsUsed _savegame) CheckPoint)
  (Variables|/Game/TECH/Mitz/Blueprints/BP_SaveGame.BP_SaveGame_C|SetCurrentActiveCheckpointIndex _savegame CurrentActiveCP%20Index)
  (Variables|/Game/TECH/Mitz/Blueprints/BP_SaveGame.BP_SaveGame_C|SetSpawnTransform _savegame SpawnTransform)
  (Variables|/Game/TECH/Mitz/Blueprints/BP_SaveGame.BP_SaveGame_C|SetuseSavedLocation? _savegame true)
  (Variables|/Game/TECH/Mitz/Blueprints/BP_SaveGame.BP_SaveGame_C|SetKills _savegame Kills)
  (bind _returnvalue (UserInterface|CreateWidget "/Game/TECH/Mitz/UI/W_Saving.W_Saving_C" (Variables|Default|GetPlayerController)))
  (UserInterface|Viewport|AddtoViewport _returnvalue 0)
  (for _array_element (Variables|Default|GetEnemy)
    (Utilities|Array|Add (Variables|/Game/TECH/Mitz/Blueprints/BP_SaveGame.BP_SaveGame_C|GetKilledEnemies (Variables|Default|GetSaveGame)) _array_element))
  (Utilities|Array|Clear (Variables|Default|GetEnemy))
  (SaveGame|SaveGametoSlot (Variables|Default|GetSaveGame) (Variables|Default|GetSaveSlotName)))

(event EventILoadGame
  ;[0.1714 1 0] Save Game
  ;;[0 0.2846 1] Load Game (Updated)
  (Development|ExecuteConsoleCommand "RestartLevel" 0))

(event EventIRestartLevel
  ;[0.1714 1 0] Save Game
  ;;[1 1 1] Save Game
  (SaveGame|DeleteGameinSlot (Variables|Default|GetSaveSlotName))
  (Development|ExecuteConsoleCommand "RestartLevel" 0))

(event EventIUpdateLevelData
  ;[0.1714 1 0] Save Game
  ;;[1 1 1] Save Game
  ;;;[0 0.2846 1] SaveLevelData
  (SaveGame|SaveGametoSlot (Variables|Default|GetSaveGame) (Variables|Default|GetSaveSlotName)))

(event EventISaveCurrentActiveCheckPoint
  (params (CheckPoint :type Actor%20Object%20Reference))
  ;[1 1 1] Load Game
  ;;[1 1 1] Save Active Checkpoint
  (Variables|/Game/TECH/Mitz/Blueprints/BP_SaveGame.BP_SaveGame_C|SetcurrentActiveCheckPoint (Variables|Default|GetSaveGame) CheckPoint)
  (SaveGame|SaveGametoSlot (Variables|Default|GetSaveGame) (Variables|Default|GetSaveSlotName)))

(event EventISaveTime
  (params (TimeAmount :type Float%20%28single-precision%29))
  ;[1 1 1] Save the game time
  (bind _output_get (Variables|Default|SetTime TimeAmount))
  (Variables|/Game/TECH/Mitz/Blueprints/BP_SaveGame.BP_SaveGame_C|SetTimer (Variables|Default|GetSaveGame) _output_get))

(event EventISaveCheckPointTimer
  ;[1 1 1] Load Game
  ;;[1 1 1] Save Checkpoint timer
  (bind _currentactivecheckpoint (Variables|/Game/TECH/Mitz/Blueprints/BP_SaveGame.BP_SaveGame_C|GetcurrentActiveCheckPoint (Variables|Default|GetSaveGame))
    (:then
      (bind _time (Class|ISaveGame|IGetCheckPointActiveTime(Message) _currentactivecheckpoint))
      (Variables|/Game/TECH/Mitz/Blueprints/BP_SaveGame.BP_SaveGame_C|SetcurrentCheckPointActiveTime (Variables|Default|GetSaveGame) _time)
      (SaveGame|SaveGametoSlot (Variables|Default|GetSaveGame) (Variables|Default|GetSaveSlotName)))
    (:else)))

(event EventIAddKilledEnemy
  (params (Enemy :type Actor%20Object%20Reference))
  ;[1 1 1] Add enemy (to gamemode)
  (Utilities|Array|Add (Variables|Default|GetEnemy) Enemy))

(fn ConstructionScript)

(fn FStoreReferences
  (params (Character :type Pawn%20Object%20Reference))
  (bind _asbp_base_character (Utilities|Casting|CastToBP_BaseCharacter Character))
  (Variables|Default|SetPlayerCharacter _asbp_base_character)
  (bind _returnvalue (Actor|GetActorOfClass "/Game/TECH/Mitz/Blueprints/BP_SpawnManager.BP_SpawnManager_C"))
  (Variables|Default|SetSpawnManager _returnvalue))

(fn FFirstSave
  (bind _playercharacter (Variables|Default|GetPlayerCharacter))
  (bind _returnvalue (Actor|GetActorOfClass "/Game/TECH/Mitz/Blueprints/BP_PlayerStart.BP_PlayerStart_C"))
  (Transformation|SetActorLocation _playercharacter (.location (Transformation|GetWorldTransform (Variables|/Game/TECH/Mitz/Blueprints/BP_PlayerStart.BP_PlayerStart_C|GetForwardDirection _returnvalue))) false false)
  (Pawn|SetControlRotation (Pawn|GetController _playercharacter) (.rotation (Transformation|GetWorldTransform (Variables|/Game/TECH/Mitz/Blueprints/BP_PlayerStart.BP_PlayerStart_C|GetForwardDirection _returnvalue))))
  (Class|ISaveGame|IInitTime(Message) (Variables|Default|GetPlayerController)))

(fn FCheckLevel
  (bind _playercharacter (Variables|Default|GetPlayerCharacter))
  (bind _returnvalue (SaveGame|LoadGamefromSlot (Variables|Default|GetSaveSlotName)))
  (Class|ISaveGame|IConvertSaveSlot(Message) _returnvalue)
  (bind (_returnvalue_2 _previouslevel) (Utilities|MCheckLevel))
  (if _returnvalue_2
    (Variables|/Game/TECH/Mitz/Blueprints/BP_SaveGame.BP_SaveGame_C|SetPreviousLevel (Variables|Default|GetSaveGame) _previouslevel)
    (bind _returnvalue_3 (Actor|GetActorOfClass "/Game/TECH/Mitz/Blueprints/BP_PlayerStart.BP_PlayerStart_C"))
    (Transformation|SetActorLocation _playercharacter (.location (Transformation|GetWorldTransform (Variables|/Game/TECH/Mitz/Blueprints/BP_PlayerStart.BP_PlayerStart_C|GetForwardDirection _returnvalue_3))) false false)
    (Pawn|SetControlRotation (Pawn|GetController _playercharacter) (.rotation (Transformation|GetWorldTransform (Variables|/Game/TECH/Mitz/Blueprints/BP_PlayerStart.BP_PlayerStart_C|GetForwardDirection _returnvalue_3))))
    (Variables|/Game/TECH/Mitz/Blueprints/BP_SaveGame.BP_SaveGame_C|SetSpawnTransform (Variables|Default|GetSaveGame) (Math|Transform|MakeTransform (.location (Transformation|GetWorldTransform (Variables|/Game/TECH/Mitz/Blueprints/BP_PlayerStart.BP_PlayerStart_C|GetForwardDirection _returnvalue_3))) (.rotation (Transformation|GetWorldTransform (Variables|/Game/TECH/Mitz/Blueprints/BP_PlayerStart.BP_PlayerStart_C|GetForwardDirection _returnvalue_3))) "1,1,1"))))

(fn FAudio
  (bind _savegame (Variables|Default|GetSaveGame))
  (bind _settings (Variables|/Game/TECH/Mitz/Blueprints/BP_SaveGame.BP_SaveGame_C|GetSettings _savegame))
  (bind (_fov _mousesensitivity _maxvolume _maxmusicvolume _maxsfxvolume) (Utilities|Struct|Breaks_Settings _settings))
  (Variables|Default|SetMaxVolume _maxvolume)
  (Variables|Default|SetMusicVolume _maxmusicvolume)
  (Variables|Default|SetSFXVolume _maxsfxvolume))

(fn IConvertSaveSlot
  (return 0))

(fn ICurrentGamemode
  (return (Variables|Default|GetCurrentGamemode)))

(fn ICurrentRound
  (return 0))

(fn IGetCheckPointActiveTime
  (return 0.0))

(fn IGetKilledEnemies
  (return (Variables|Default|GetEnemy)))

(fn IGetPlayerController
  (return 0))

(fn IGetTime
  (return 0.0))

(fn IRoundStartDelay
  (return 0.0))