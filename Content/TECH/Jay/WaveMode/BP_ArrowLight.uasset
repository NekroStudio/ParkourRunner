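; BP_ArrowLight is an arrow light actor in the WaveMode folder whose indicator colour other objects can switch between red, green, white and off.
; Four toggle events, apparently from an interface, each swap the material in slot 1 of its mesh.
; A LevelEndLightColour switch in the construction script is disconnected, so it never runs, and its white material differs from the event's.
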(event EventBeginPlay
  (|CallParentFunction) ; This node is disabled and will not be called.\nDrag off pins to build functionality.
)

(event Collision|EventActorBeginOverlap
  (params (OtherActor :type Actor%20Object%20Reference))
  (|CallParentFunction OtherActor) ; This node is disabled and will not be called.\nDrag off pins to build functionality.
)

(event EventTick
  (params (DeltaSeconds :type Float%20%28single-precision%29))
  (|CallParentFunction DeltaSeconds) ; This node is disabled and will not be called.\nDrag off pins to build functionality.
)

(event EventIToggleLightGreen
  (Rendering|Material|SetMaterial (Variables|Character|GetMesh) 1 "/Game/TECH/Jay/Materials/MI_Light_03.MI_Light_03"))

(event EventIToggleLightOff
  (Rendering|Material|SetMaterial (Variables|Character|GetMesh) 1 "/Game/ART/James/Shaders/Master_Materials/MI_Light_02_A_INST.MI_Light_02_A_INST"))

(event EventIToggleLightRed
  (Rendering|Material|SetMaterial (Variables|Character|GetMesh) 1 "/Game/TECH/Jay/Materials/MI_Light_04.MI_Light_04"))

(event EventIToggleLightWhite
  (Rendering|Material|SetMaterial (Variables|Character|GetMesh) 1 "/Game/TECH/Jay/Materials/MI_Light_05.MI_Light_05"))

(fn ConstructionScript
  (|CallParentFunction))