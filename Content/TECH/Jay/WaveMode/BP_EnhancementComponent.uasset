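; Component that tracks the player's enhancements, applies each on pickup, and manages the shield they grant.
; Round setup checks the list for shield tiers to set the shield flag and start its effect.
; The shield is a dynamic post-process material on the character camera, with looping timers animating its Radius on build and break.
; Breaking a tier-two shield also temporarily stops enemy shooting and clears enemy projectiles.
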(event Custom|StoreRefs
  (params (EnhancementManager :type BP%20Enhancement%20Manager%20Object%20Reference))
  ;[1 1 1] Store Manager
  (Variables|Default|SetEnhancement%20Manager EnhancementManager))

(event Custom|AddEnhancement
  (params (AddedEnhancement :type BP%20Base%20Enhancement%20Object%20Reference))
  ;[1 1 1] Add enhancement to player array
  (Utilities|Array|Add (Variables|Default|GetCurrentEnhancements) AddedEnhancement)
  (bind _output_get (Variables|Default|SetNewlyAddedEnhancement AddedEnhancement))
  (Class|BPIEnhancements|IApplyEnhancementEffect(Message) _output_get (Variables|Default|GetCharacter)))

(event Custom|BuildupShieldFX
  ;[0.8924 0 1] Build Shield
  (bind _output_get (Variables|Shield|SetShieldWeightAmount (+ (Variables|Shield|GetShieldWeightAmount) 0.01)))
  (if (>= _output_get 0.5)
    (Utilities|Time|ClearandInvalidateTimerbyHandle (Variables|Shield|GetShieldBuilderHandle)))
  (Rendering|Material|SetScalarParameterValue (Variables|Shield|GetShieldMat) "Radius" (Variables|Shield|GetShieldWeightAmount) :!class /Script/Engine.MaterialInstanceDynamic))

(event Custom|SetupRoundPersistantEnhancements
  ;[0.8924 0 1] Shield setup
  (bind _returnvalue (CallFunction|FCheckforEnhancement "/Game/TECH/Jay/WaveMode/UpgradesAndAbilities/BP_Shield.BP_Shield_C"))
  (if _returnvalue
    (Variables|Shield|SetHasShield true)
    (bind _returnvalue_2 (CallFunction|FCheckforEnhancement "/Game/TECH/Jay/WaveMode/UpgradesAndAbilities/BP_Shield2.BP_Shield2_C"))
    (if _returnvalue_2
      (Variables|Shield|SetShieldColourInstance "/Game/TECH/Jay/Materials/M_Shield2.M_Shield2")
      (CallFunction|SetupShield))
    (CallFunction|TriggerShieldFX)))

(event Custom|InitEnhancementComponent
  (params (Character :type BP%20Base%20Character%20Object%20Reference))
  ;[1 1 1] Store character - INIT
  (Variables|Default|SetCharacter Character))

(event Custom|SetupShield
  ;[0.8924 0 1] Setup shield
  (bind _currentgamemode (Class|BPIGamemodeElements|ICurrentGamemode(Message) (Game|GetGameMode)))
  (switch Utilities|FlowControl|Switch|SwitchonE_CurrentGamemode _currentgamemode
    (:NewEnumerator1
      (bind _returnvalue (Rendering|Material|CreateDynamicMaterialInstance (Variables|Shield|GetShieldColourInstance) "None" "None" :!class /Script/Engine.KismetMaterialLibrary))
      (bind _output_get (Variables|Shield|SetShieldMat _returnvalue))
      (Utilities|Struct|SetmembersinPostProcessSettings (Variables|/Script/Engine.CameraComponent|GetPostProcessSettings (Variables|/Game/TECH/Jay/BP_BaseCharacter.BP_BaseCharacter_C|GetCamera (Variables|Default|GetCharacter))) (Utilities|Struct|MakeWeightedBlendables (Utilities|Array|MakeArray (Utilities|Struct|MakeWeightedBlendable 1.0 _output_get)))))))

(event Custom|TriggerBrokenShieldFX
  ;[0.8924 0 1] Break Shield
  (bind _returnvalue (Utilities|Time|SetTimerbyEvent (delegate Custom|ShieldBreakFX) 0.005 true))
  (Variables|Shield|SetShieldBuilderHandle _returnvalue))

(event Custom|ShieldBreakFX
  ;[0.8924 0 1] Break Shield
  (bind _output_get (Variables|Shield|SetShieldWeightAmount (- (Variables|Shield|GetShieldWeightAmount) 0.01)))
  (if (<= _output_get -0.5)
    (Utilities|Time|ClearandInvalidateTimerbyHandle (Variables|Shield|GetShieldBuilderHandle)))
  (Rendering|Material|SetScalarParameterValue (Variables|Shield|GetShieldMat) "Radius" (Variables|Shield|GetShieldWeightAmount) :!class /Script/Engine.MaterialInstanceDynamic))

(event Custom|TriggerShieldFX
  ;[0.8924 0 1] Build Shield
  (bind _returnvalue (Utilities|Time|SetTimerbyEvent (delegate Custom|BuildupShieldFX) 0.005 true))
  (Variables|Shield|SetShieldBuilderHandle _returnvalue))

(event EventIDisableShield
  ;[0.8924 0 1] Disable shield
  (Variables|Shield|SetHasShield false)
  (CallFunction|TriggerBrokenShieldFX)
  (bind _returnvalue (CallFunction|FCheckforEnhancement "/Game/TECH/Jay/WaveMode/UpgradesAndAbilities/BP_Shield2.BP_Shield2_C"))
  (if _returnvalue
    (bind _outactors (Actor|GetAllActorsOfClass "/Game/TECH/Mitz/AI/BP_BaseEnemy.BP_BaseEnemy_C"))
    (for _array_element _outactors
      (Default|TempDisableShooting _array_element))
    (bind _outactors_2 (Actor|GetAllActorsOfClass "/Game/TECH/Mitz/AI/BP_EnemyProectile.BP_EnemyProectile_C"))
    (for _array_element_2 _outactors_2
      (Actor|SetLifeSpan _array_element_2 0.001))))

(fn FCheckforEnhancement
  (params (Enhancement :type Object%20Class%20Reference))
  (bind _currentenhancements (Variables|Default|GetCurrentEnhancements))
  (if (> (Utilities|Array|Length _currentenhancements) 0)
    (bind _array_element (Utilities|Array|ForEachLoopwithBreak _currentenhancements :!label _label)
      (:LoopBody
        (if (== (Utilities|Struct|BreakS_EnhancementButtonValues (Variables|/Game/TECH/Jay/WaveMode/BP_BaseEnhancement.BP_BaseEnhancement_C|GetEnhancementButtonValues _array_element)) Enhancement)
          (goto _label Break)))
      (:Completed
        (return (== (Utilities|Struct|BreakS_EnhancementButtonValues (Variables|/Game/TECH/Jay/WaveMode/BP_BaseEnhancement.BP_BaseEnhancement_C|GetEnhancementButtonValues _array_element)) Enhancement))))))

(fn ICheckShield
  (return (Variables|Shield|GetHasShield)))