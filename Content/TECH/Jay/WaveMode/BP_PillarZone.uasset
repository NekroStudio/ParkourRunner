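; BP_PillarZone is a zone actor that grants temporary bullet time when the player enters its sphere.
; It stays hidden until an enhancement effect stores the character and enables interaction.
; Overlap slows global time and inversely speeds the character's custom dilation for PillarDuration.
; If dash dilation is active at expiry, a delay loop adjusts character dilation once and waits before restoring both time scales.
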(event OnComponentBeginOverlap(Sphere)
  (params (OverlappedComponent :type Primitive%20Component%20Object%20Reference) (OtherActor :type Actor%20Object%20Reference) (OtherComp :type Primitive%20Component%20Object%20Reference) (OtherBodyIndex :type Integer) (bFromSweep :type Boolean) (SweepResult :type Hit%20Result%20Structure%20%28by%20ref%29))
  (bind _character (Variables|Default|GetCharacter))
  ;[1 1 1] Overlapping pullar zone causes time dilation
  (Utilities|MIsPlayer OtherActor
    (:true
      (if (Variables|Default|GetCanInteract)
        (if (not (Variables|Default|GetIsCurrentlyActive))
          (Variables|Default|SetIsCurrentlyActive true)
          (Variables|Default|SetBaseCustomTD (Variables|/Script/Engine.Actor|GetCustomTimeDilation _character))
          (Utilities|Time|SetGlobalTimeDilation 0.25)
          (Variables|/Script/Engine.Actor|SetCustomTimeDilation _character 4.0)
          (Utilities|FlowControl|Delay (Variables|Default|GetPillarDuration))
          (if (Variables|/Game/TECH/Jay/BP_BaseCharacter.BP_BaseCharacter_C|GetDashDilationActive _character) :!label _label
            (Utilities|FlowControl|Delay 0.01)
            (Utilities|FlowControl|Sequence
              (:then_0
                (Utilities|FlowControl|DoOnce false
                  (:Completed
                    (Variables|/Script/Engine.Actor|SetCustomTimeDilation _character 0.25))))
              (:then_1
                (goto _label)))
            (else
              (Utilities|Time|SetGlobalTimeDilation 1.0)
              (Variables|/Script/Engine.Actor|SetCustomTimeDilation _character (Variables|Default|GetBaseCustomTD))
              (Variables|Default|SetIsCurrentlyActive false))))))))

(event EventBeginPlay
  (|CallParentFunction)
  (Rendering|SetActorHiddenInGame true))

(event Collision|EventActorBeginOverlap
  (params (OtherActor :type Actor%20Object%20Reference))
  (|CallParentFunction OtherActor) ; This node is disabled and will not be called.\nDrag off pins to build functionality.
)

(event EventTick
  (params (DeltaSeconds :type Float%20%28single-precision%29))
  (|CallParentFunction DeltaSeconds) ; This node is disabled and will not be called.\nDrag off pins to build functionality.
)

(event EventIApplyEnhancementEffect
  (params (Character :type BP%20Base%20Character%20Object%20Reference))
  (Variables|Default|SetCharacter Character)
  (Variables|Default|SetCanInteract true)
  (Rendering|SetActorHiddenInGame false))

(fn ConstructionScript
  (|CallParentFunction))

(fn ICheckShield
  (return false))