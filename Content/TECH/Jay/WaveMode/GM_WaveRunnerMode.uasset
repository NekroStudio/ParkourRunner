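; Game mode for the wave runner mode, managing rounds of timer-spawned enemies, enhancement selection between rounds and the win screen.
; Each round grows the enemy quota up to a cap and randomises enemy types after round three.
; The final kill triggers brief slow motion, then unlocks the exit door, switches arrow lights and notifies listeners.
; Player death clears enemies and replays the round at the same quota; most checkpoint save logic is disconnected.
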(event Custom|Win%20Condition
  (bind _playercontroller (Variables|CoreReferences|GetPlayerController))
  (bind _playercontroller_2 (Variables|CoreReferences|GetPlayerController))
  (bind _playercharacter (Variables|CoreReferences|GetPlayerCharacter))
  (bind _savegameref (Variables|/Game/TECH/Jay/BP_BaseCharacter.BP_BaseCharacter_C|GetSaveGameRef _playercharacter))
  ;[0 0.2846 1] Show win screen
  (bind _returnvalue (UserInterface|CreateWidget "/Game/TECH/Jay/UI/W_WaveModeEndScreen.W_WaveModeEndScreen_C" _playercontroller (Variables|/Game/TECH/Mitz/Blueprints/BP_SaveGame.BP_SaveGame_C|GetKills _savegameref) (Variables|/Game/TECH/Mitz/Blueprints/BP_SaveGame.BP_SaveGame_C|GetDeaths _savegameref) (Variables|/Game/TECH/Mitz/Blueprints/BP_SaveGame.BP_SaveGame_C|GetTimer _savegameref) (Variables|/Game/TECH/Mitz/Blueprints/BP_SaveGame.BP_SaveGame_C|GetPlayerScore _savegameref) "NewEnumerator7" _playercontroller _playercharacter))
  (UserInterface|Viewport|AddtoViewport _returnvalue 0)
  (Input|SetInputModeUIOnly _playercontroller_2 _returnvalue "DoNotLock")
  (Variables|/Script/Engine.PlayerController|SetbShowMouseCursor _playercontroller_2 true)
  (Default|PlayAnim _returnvalue))

(event Custom|TriggerTimeSlow
  ;[0 0.2846 1] Round end elements (pre start new round)
  (Utilities|Time|SetGlobalTimeDilation 0.1)
  (Utilities|FlowControl|Delay 0.05)
  (CallFunction|TriggerResetTime))

(event Custom|EndOfRound
  (bind _playercontroller (Variables|CoreReferences|GetPlayerController))
  (bind _hud (Variables|/Game/TECH/Jay/BP_PlayerController.BP_PlayerController_C|GetHUD _playercontroller))
  (bind _w_enhancementselectscreen (Variables|/Game/TECH/Jay/UI/W_BaseHUD.W_BaseHUD_C|GetW_EnhancementSelectScreen _hud))
  ;[0 0.2846 1] Round End
  (bind _result (Math|Integer|IncrementInt (Variables|CoreRoundValues|GetCurrentRoundNumber))
    (:%20%20
      (CallFunction|FDisableMovement)
      (CallFunction|IUpdateAISpawnPoints)
      (if (not (>= _result (Variables|CoreRoundValues|GetMaxRoundCap)))
        (Default|ToggleEnhancementScreenON _hud)
        (Default|RefreshEnhancementtoSelect _w_enhancementselectscreen)
        (Default|RefreshCurrentEnhancements _w_enhancementselectscreen)))))

(event Custom|TriggerResetTime
  ;[0 0.2846 1] Round end elements (pre start new round)
  (Utilities|Time|SetGlobalTimeDilation 1.0)
  (CallFunction|FCheckforActivePillar)
  (CallFunction|TriggerDoortoOpen)
  (CallFunction|FToggleLightsonEnd)
  (Default|CallEDCurrentWaveCompleted))

(event Custom|TriggerDoorToOpen
  ;[0 0.2846 1] Round end elements (pre start new round)
  (Class|BPIEnvironmentalInteractions|IUnlockDoor(WM)(Message) (Variables|CoreReferences|GetRoundEndDoor) self)
  (if (>= (Variables|CoreRoundValues|GetCurrentRoundNumber) (Variables|CoreRoundValues|GetMaxRoundCap))
    (bind _returnvalue (Actor|GetActorOfClass "/Game/TECH/Jay/Blueprints/BP_WaveModeEndVolume.BP_WaveModeEndVolume_C"))
    (Variables|/Game/TECH/Jay/Blueprints/BP_WaveModeEndVolume.BP_WaveModeEndVolume_C|SetCompletedAllWaves _returnvalue true)))

(event Custom|TriggerSpawningAI
  ;[0 0.2846 1] AI Spawn Loop
  (bind _returnvalue (Utilities|Time|SetTimerbyEvent (delegate Custom|AISpwningLoop) (Variables|SpawningEnemies|GetDelayBetweenAISpawns) true))
  (Variables|SpawningEnemies|SetAISpawnLoopHandle _returnvalue))

(event Custom|AISpwningLoop
  (bind _aitospawn (Variables|SpawningEnemies|GetAIToSpawn))
  ;[0 0.2846 1] AI Spawn Loop
  (if (<= (Variables|CoreRoundValues|GetCurrentSpawnedEnemies) (- (Variables|CoreRoundValues|GetMaxEnemiesToSpawnInRound) 1))
    (Game|SpawnActorfromClass (Utilities|Array|Get(acopy) _aitospawn (Math|Integer|SelectInt 0 (Math|Random|RandomInteger (Utilities|Array|Length _aitospawn)) (<= (Variables|CoreRoundValues|GetCurrentRoundNumber) 3))) (Utilities|MGetSpawnPointTransforms) "AdjustIfPossibleButAlwaysSpawn" 0 0)
    (Math|Integer|IncrementInt (Variables|CoreRoundValues|GetCurrentSpawnedEnemies))
    (else
      (Utilities|Time|ClearandInvalidateTimerbyHandle (Variables|SpawningEnemies|GetAISpawnLoopHandle))
      (Default|CallEDUpdateRemainingEnemies (Variables|CoreRoundValues|GetCurrentNumberOfEnemiesKilled) (Variables|CoreRoundValues|GetCurrentSpawnedEnemies)))))

(event Custom|SaveGameStart
  ;[0.1714 1 0] Save Game
  ;;[1 1 1] Checks if a save exists
)

(event Custom|RoundStarted
  ;[0 0.2846 1] Start new round
  (Default|SetupRoundPersistantEnhancements (Variables|/Game/TECH/Jay/BP_BaseCharacter.BP_BaseCharacter_C|GetBP_EnhancementComponent (Variables|CoreReferences|GetPlayerCharacter)))
  (CallFunction|FSetupNumOfEnemiestoSpawn)
  (Variables|CoreRoundValues|SetPlayerDied false)
  (for _array_element (Variables|SpawningEnemies|GetAISpawnPoints)
    (Variables|/Game/TECH/Jay/WaveMode/BP_AISpawnLocation.BP_AISpawnLocation_C|SetOccupied _array_element false))
  (CallFunction|TriggerSpawningAI)
  (CallFunction|FToggleLightsonStart))

(event EventILoadGame
  ;[0 0.2846 1] Load Game (Updated) - Player death
  (Variables|CoreRoundValues|SetPlayerDied true)
  (bind _outactors (Actor|GetAllActorsOfClass "/Game/TECH/Mitz/AI/BP_BaseEnemy.BP_BaseEnemy_C"))
  (for _array_element _outactors
    (Actor|DestroyActor _array_element))
  (Utilities|Time|ClearandInvalidateTimerbyHandle (Variables|SpawningEnemies|GetAISpawnLoopHandle))
  (CallFunction|FResetCharacterLocation)
  (CallFunction|IStartRound))

(event EventIChangeLevel
  ;[0.1714 1 0] Save Game
  ;;[1 1 1] Change level
)

(event EventBeginPlay
  ;[0 0.2846 1] Begin play
  (bind _returnvalue (SaveGame|LoadGamefromSlot (Variables|CoreReferences|GetSaveSlotName)))
  (bind _saveslot (Class|ISaveGame|IConvertSaveSlot(Message) _returnvalue))
  (Default|FClearVariables _saveslot)
  (bind _asbp_base_character (Utilities|Casting|CastToBP_BaseCharacter (Game|GetPlayerCharacter 0)))
  (Variables|CoreReferences|SetPlayerCharacter _asbp_base_character)
  (CallFunction|FFirstSave))

(event EventISaveGame
  (params (SpawnTransform :type Transform) (CheckPoint :type BP%20Check%20Point%20Object%20Reference) (KilledEnemies :type Array%20of%20Actor%20Object%20References) (Kills :type Integer) (CurrentActiveCP%20Index :type Integer))
  ;[0.1714 1 0] Save Game
  ;;[1 1 1] Save Game
)

(event EventIUpdateAISpawnPoints
  ;[0 0.2846 1] Updates AI spawn points (usually when environment expansion enhancement is activated)
  (Utilities|Array|Clear (Variables|SpawningEnemies|GetAISpawnPoints))
  (Utilities|FlowControl|Delay 0.01)
  (bind _outactors (Actor|GetAllActorsOfClass "/Game/TECH/Jay/WaveMode/BP_AISpawnLocation.BP_AISpawnLocation_C"))
  (for _array_element _outactors
    (Utilities|Array|Add (Variables|SpawningEnemies|GetAISpawnPoints) _array_element)))

(event EventIRestartLevel
  ;[0.1714 1 0] Save Game
  ;;[1 1 1] Save Game
)

(event EventIUpdateLevelData
  ;[0.1714 1 0] Save Game
  ;;[1 1 1] Save Game
  ;;;[0 0.2846 1] SaveLevelData
  (SaveGame|SaveGametoSlot (Variables|CoreReferences|GetSaveGame) (Variables|CoreReferences|GetSaveSlotName)))

(event EventIAddKilledEnemy
  (params (Enemy :type Actor%20Object%20Reference))
  (bind _currentnumberofenemieskilled (Variables|CoreRoundValues|GetCurrentNumberOfEnemiesKilled))
  ;[0 0.2846 1] Add enemy to variable
  (Utilities|Array|Add (Variables|CoreReferences|GetEnemy) Enemy)
  (Math|Integer|IncrementInt _currentnumberofenemieskilled
    (:%20%20
      (Utilities|MCanApplySpeedBoost)
      (Default|CallEDUpdateRemainingEnemies _currentnumberofenemieskilled (Variables|CoreRoundValues|GetCurrentSpawnedEnemies))
      (if (>= (Variables|CoreRoundValues|GetCurrentNumberOfEnemiesKilled) (Variables|CoreRoundValues|GetNeededNumberOfEnemiesKilled))
        (CallFunction|TriggerTimeSlow)))))

(event EventISaveTime
  (params (TimeAmount :type Float%20%28single-precision%29))
  ;[0.07998 1 0] Save the game time
  (bind _output_get (Variables|GameTime|SetTime TimeAmount))
  (Variables|/Game/TECH/Mitz/Blueprints/BP_SaveGame.BP_SaveGame_C|SetTimer (Variables|CoreReferences|GetSaveGame) _output_get))

(event EventIInitCurrentGamemode
  (params (Controller :type BP%20Player%20Controller%20Object%20Reference) (Pawn :type Pawn%20Object%20Reference))
  ;[0 0.2846 1] Init
  (Variables|CoreReferences|SetPlayerController Controller)
  (CallFunction|FStoreReferences Pawn)
  (CallFunction|SaveGameStart)
  (CallFunction|FAISpawnPoints)
  (Default|CallEDToggleWaveHudon))

(event EventIStartRound
  ;[0 0.2846 1] Trigger Round Start
  (Utilities|MEnableInput)
  (CallFunction|FResetVariables)
  (CallFunction|FResetCharacterLocation)
  (CallFunction|RoundStarted)
  (Default|CallEDNewWaveStarted))

(fn ConstructionScript)

(fn FStoreReferences
  (params (Charcter :type Pawn%20Object%20Reference))
  (bind _asbp_base_character (Utilities|Casting|CastToBP_BaseCharacter Charcter))
  (Variables|CoreReferences|SetPlayerCharacter _asbp_base_character)
  (bind _returnvalue (Actor|GetActorOfClass "/Game/TECH/Mitz/Blueprints/BP_SpawnManager.BP_SpawnManager_C"))
  (Variables|CoreReferences|SetSpawnManager _returnvalue)
  (bind _returnvalue_2 (Actor|GetActorOfClass "/Game/TECH/Jay/Blueprints/EnvironmentalInteractions/BP_OpeningDoor.BP_OpeningDoor_C"))
  (Variables|CoreReferences|SetRoundEndDoor _returnvalue_2)
  (bind _outactors (Actor|GetAllActorsOfClass "/Game/TECH/Jay/WaveMode/BP_ArrowLight.BP_ArrowLight_C"))
  (for _array_element _outactors
    (Utilities|Array|Add (Variables|Default|GetArrowLights) _array_element)))

(fn FFirstSave
  (bind _playercharacter (Variables|CoreReferences|GetPlayerCharacter))
  (bind _returnvalue (Actor|GetActorOfClass "/Game/TECH/Mitz/Blueprints/BP_PlayerStart.BP_PlayerStart_C"))
  (Transformation|SetActorLocation _playercharacter (.location (Transformation|GetWorldTransform (Variables|/Game/TECH/Mitz/Blueprints/BP_PlayerStart.BP_PlayerStart_C|GetForwardDirection _returnvalue))) false false)
  (Pawn|SetControlRotation (Pawn|GetController _playercharacter) (.rotation (Transformation|GetWorldTransform (Variables|/Game/TECH/Mitz/Blueprints/BP_PlayerStart.BP_PlayerStart_C|GetForwardDirection _returnvalue)))))

(fn FAISpawnPoints
  (bind _outactors (Actor|GetAllActorsOfClass "/Game/TECH/Jay/WaveMode/BP_AISpawnLocation.BP_AISpawnLocation_C"))
  (for _array_element _outactors
    (Utilities|Array|Add (Variables|SpawningEnemies|GetAISpawnPoints) _array_element)))

(fn FResetVariables
  (Variables|CoreRoundValues|SetCurrentSpawnedEnemies 0)
  (Variables|CoreRoundValues|SetCurrentNumberOfEnemiesKilled 0))

(fn FResetCharacterLocation
  (bind _returnvalue (Actor|GetActorOfClass "/Game/TECH/Mitz/Blueprints/BP_PlayerStart.BP_PlayerStart_C"))
  (Pawn|SetControlRotation (Variables|CoreReferences|GetPlayerController) (.rotation (Transformation|GetActorTransform _returnvalue)))
  (Transformation|SetActorLocation (Variables|CoreReferences|GetPlayerCharacter) (.location (Transformation|GetActorTransform _returnvalue)) false false))

(fn FSetupNumOfEnemiestoSpawn
  (if (not (Variables|CoreRoundValues|GetPlayerDied))
    (bind _output_get (Variables|CoreRoundValues|SetMaxEnemiesToSpawnInRound (Math|Integer|Clamp(Integer) (+ (Variables|CoreRoundValues|GetMaxEnemiesToSpawnInRound) (Math|Random|RandomIntegerinRange 1 2)) 0 (Variables|SpawningEnemies|GetClampedMaxSpawnFoes))))
    (Variables|CoreRoundValues|SetNeededNumberOfEnemiesKilled _output_get)))

(fn FDisableMovement
  (Class|NavMovementComponent|StopActiveMovement (Variables|/Script/Engine.Character|GetCharacterMovement (Variables|CoreReferences|GetPlayerCharacter)))
  (Input|DisableInput (Variables|CoreReferences|GetPlayerCharacter) (Variables|CoreReferences|GetPlayerController)))

(fn FCheckforEnhancement
  (params (EnhancementToCheck :type Object%20Class%20Reference))
  (bind _playercharacter (Variables|CoreReferences|GetPlayerCharacter)
    (:then
      (bind _array_element (Utilities|Array|ForEachLoopwithBreak (Variables|/Game/TECH/Jay/WaveMode/BP_EnhancementComponent.BP_EnhancementComponent_C|GetCurrentEnhancements (Variables|/Game/TECH/Jay/BP_BaseCharacter.BP_BaseCharacter_C|GetBP_EnhancementComponent _playercharacter)) :!label _label)
        (:LoopBody
          (if (== (Utilities|Struct|BreakS_EnhancementButtonValues (Variables|/Game/TECH/Jay/WaveMode/BP_BaseEnhancement.BP_BaseEnhancement_C|GetEnhancementButtonValues _array_element)) EnhancementToCheck)
            (goto _label Break)))
        (:Completed
          (Utilities|IsValid _array_element
            (:Is%20Valid
              ;[1 1 1] Prevent error
              (if (== (Utilities|Struct|BreakS_EnhancementButtonValues (Variables|/Game/TECH/Jay/WaveMode/BP_BaseEnhancement.BP_BaseEnhancement_C|GetEnhancementButtonValues _array_element)) EnhancementToCheck)
                (return true)
                (else
                  _)))
            (:Is%20Not%20Valid
              _))
          (return false))))
    (:else)))

(fn FCheckforActivePillar
  (bind _containsenhancement (CallFunction|FCheckforEnhancement "/Game/TECH/Jay/WaveMode/UpgradesAndAbilities/BP_PillarTemporalZone.BP_PillarTemporalZone_C"))
  (if _containsenhancement
    (bind _returnvalue (Actor|GetActorOfClass "/Game/TECH/Jay/WaveMode/UpgradeEffects/BP_PillarZone.BP_PillarZone_C"))
    (if (Variables|/Game/TECH/Jay/WaveMode/UpgradeEffects/BP_PillarZone.BP_PillarZone_C|GetIsCurrentlyActive _returnvalue)
      (Default|IDisablePillarZone _returnvalue)
      (return)
      (else
        (return)))
    (else
      (return))))

(fn FToggleLightsonEnd
  (for _array_element (Variables|Default|GetArrowLights)
    (switch Utilities|FlowControl|Switch|SwitchonE_ArrowLightColour (Variables|/Game/TECH/Jay/WaveMode/BP_ArrowLight.BP_ArrowLight_C|GetLevelEndLightColour _array_element)
      (:NewEnumerator0
        (Default|IToggleLightOff _array_element))
      (:NewEnumerator1
        (Default|IToggleLightRed _array_element))
      (:NewEnumerator2
        (Default|IToggleLightGreen _array_element))
      (:NewEnumerator3
        (Default|IToggleLightWhite _array_element))))
  (return))

(fn FToggleLightsonStart
  (for _array_element (Variables|Default|GetArrowLights)
    (switch Utilities|FlowControl|Switch|SwitchonE_ArrowLightColour (Variables|/Game/TECH/Jay/WaveMode/BP_ArrowLight.BP_ArrowLight_C|GetLevelStartLightColour _array_element)
      (:NewEnumerator0
        (Default|IToggleLightOff _array_element))
      (:NewEnumerator1
        (Default|IToggleLightRed _array_element))
      (:NewEnumerator2
        (Default|IToggleLightGreen _array_element))
      (:NewEnumerator3
        (Default|IToggleLightWhite _array_element))))
  (return))

(fn IConvertSaveSlot
  (return 0))

(fn ICurrentGamemode
  (return (Variables|CoreReferences|GetCurrentGamemode)))

(fn ICurrentRound
  (return (Variables|CoreRoundValues|GetCurrentRoundNumber)))

(fn IGetCheckPointActiveTime
  (return 0.0))

(fn IGetKilledEnemies
  (return 0))

(fn IGetPlayerController
  (return 0))

(fn IGetTime
  (return 0.0))

(fn IRoundStartDelay
  (return (Variables|CoreRoundValues|GetDelayTillNewRound)))