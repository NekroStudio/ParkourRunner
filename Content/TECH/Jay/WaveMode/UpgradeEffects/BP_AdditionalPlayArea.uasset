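; Wave Mode upgrade effect actor that provides an additional play area, built from six mesh pieces.
; The construction script shows or hides the meshes according to IsVisible, while BeginPlay always disables the actor's collision.
; ActivatePlayArea makes all six meshes visible and enables collision, turning the area solid.
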(event Custom|ActivatePlayArea
  (Rendering|SetVisibility (Variables|Character|GetMesh) true false)
  (Collision|SetActorEnableCollision true))

(event EventBeginPlay
  (|CallParentFunction)
  (Collision|SetActorEnableCollision false))

(event Collision|EventActorBeginOverlap
  (params (OtherActor :type Actor%20Object%20Reference))
  (|CallParentFunction OtherActor) ; This node is disabled and will not be called.\nDrag off pins to build functionality.
)

(event EventTick
  (params (DeltaSeconds :type Float%20%28single-precision%29))
  (|CallParentFunction DeltaSeconds) ; This node is disabled and will not be called.\nDrag off pins to build functionality.
)

(fn ConstructionScript
  (bind _mesh (Variables|Character|GetMesh))
  (|CallParentFunction)
  (if (Variables|Default|GetIsVisible)
    (Rendering|SetVisibility _mesh true false)
    (else
      (Rendering|SetVisibility _mesh false false))))