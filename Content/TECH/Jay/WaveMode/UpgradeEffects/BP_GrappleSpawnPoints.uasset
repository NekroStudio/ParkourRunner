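; Grapple spawn point among the Wave Mode upgrade effects, holding a child-actor grapple point and two optional meshes.
; Construction and a delayed BeginPlay show or hide the grapple from IsActive, and construction sets mesh visibility from HasMesh.
; SpawnGrapple assigns BP_GrapplePoint as the child class, sends blocking-size and visibility interface messages, and reveals the grapple, plus meshes if HasMesh or WantsMesh.
; ShouldRotate gives a slow random spin on all axes.
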(event Custom|SpawnGrapple
  (bind _grapple (Variables|Default|GetGrapple))
  (bind _mesh (Variables|Character|GetMesh))
  ;[1 1 1] Toggle visibility of grapple points
  (ChildActorComponent|SetChildActorClass _grapple "/Game/TECH/Jay/Blueprints/GrappleElements/GrapplePoints/BP_GrapplePoint.BP_GrapplePoint_C")
  (Class|BPIGrapplePointElements|ITweakBlockingGrappleSize(Message) _grapple 2.5e+02)
  (Class|BPIGrapplePointElements|IToggleVisibility(Message) (Variables|/Script/Engine.ChildActorComponent|GetChildActor (Variables|Default|GetGrapple)) "NewEnumerator1")
  (Rendering|SetVisibility (Variables|Default|GetGrapple) true true)
  (if (Variables|Default|GetHasMesh)
    (Rendering|SetVisibility _mesh true true)
    (else
      (Rendering|SetVisibility _mesh false false)))
  (if (Variables|Default|GetWantsMesh)
    (Rendering|SetVisibility (Variables|Character|GetMesh) true true)))

(event EventBeginPlay
  (bind _grapple (Variables|Default|GetGrapple))
  ;[1 1 1] Begin play
  (|CallParentFunction)
  (Rendering|SetVisibility (Variables|Default|GetGrapple) true true)
  (Utilities|FlowControl|Delay 0.2)
  (if (Variables|Default|GetIsActive)
    (Rendering|SetVisibility _grapple true true)
    (else
      (Rendering|SetVisibility _grapple false true)))
  (if (Variables|Default|GetShouldRotate)
    (CallFunction|FSetRandomRotationMovement)
    (else
      (Variables|/Script/Engine.RotatingMovementComponent|SetRotationRate (Variables|Default|GetRotatingMovement) "0.0,0.0,0.0"))))

(fn ConstructionScript
  (bind _grapple (Variables|Default|GetGrapple))
  (bind _mesh (Variables|Character|GetMesh))
  (|CallParentFunction)
  (if (Variables|Default|GetHasMesh)
    (Rendering|SetVisibility _mesh true false)
    (else
      (Rendering|SetVisibility _mesh false false)))
  (if (Variables|Default|GetIsActive)
    (Rendering|SetVisibility _grapple true true)
    (else
      (Rendering|SetVisibility _grapple false true))))

(fn FSetRandomRotationMovement
  (bind _returnvalue (Math|Random|RandomBool))
  (bind _returnvalue_2 (Math|Float|SelectFloat 1.0 -1.0 _returnvalue))
  (Variables|/Script/Engine.RotatingMovementComponent|SetRotationRate (Variables|Default|GetRotatingMovement) (Math|Rotator|MakeRotator (* (Math|Random|RandomFloatinRange -5.0 5.0) _returnvalue_2) (* (Math|Random|RandomFloatinRange -5.0 5.0) _returnvalue_2) (* (Math|Random|RandomFloatinRange -5.0 5.0) _returnvalue_2))))