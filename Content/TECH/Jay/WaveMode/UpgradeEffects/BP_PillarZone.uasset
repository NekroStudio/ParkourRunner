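; Wave-mode upgrade pillar, hidden until its enhancement is applied, that slows global time when the player touches its sphere.
; The player's custom dilation and grapple hook speed are scaled up to offset the slowdown.
; After PillarDuration, or an interface disable, it restores time, hook speed and visuals, with timed expiry waiting out an active dash dilation.
; M_SpawnFX respawns the Niagara effect, using variant visuals with the additional-time enhancement.
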(event OnComponentBeginOverlap(Sphere)
  (params (OverlappedComponent :type Primitive%20Component%20Object%20Reference) (OtherActor :type Actor%20Object%20Reference) (OtherComp :type Primitive%20Component%20Object%20Reference) (OtherBodyIndex :type Integer) (bFromSweep :type Boolean) (SweepResult :type Hit%20Result%20Structure%20%28by%20ref%29))
  (bind _character (Variables|Default|GetCharacter))
  ;[1 1 1] Overlapping pullar zone causes time dilation
  (Utilities|MIsPlayer OtherActor
    (:true
      (if (Variables|Default|GetCanInteract)
        (if (not (Variables|Default|GetIsCurrentlyActive))
          (Variables|Default|SetIsCurrentlyActive true)
          (Variables|Default|SetBaseCustomTD (Variables|/Script/Engine.Actor|GetCustomTimeDilation _character))
          (Utilities|Time|SetGlobalTimeDilation 0.25)
          (Variables|/Script/Engine.Actor|SetCustomTimeDilation _character 4.0)
          (Rendering|Material|SetMaterial (Variables|Character|GetMesh) 0 "/Game/TECH/Jay/Materials/M_BaseFresnelMat_Inst1.M_BaseFresnelMat_Inst1")
          (Components|Activation|Deactivate (Variables|Default|GetSpawnedFX))
          (Utilities|FlowControl|Delay (Variables|Default|GetPillarDuration))
          (if (Variables|/Game/TECH/Jay/BP_BaseCharacter.BP_BaseCharacter_C|GetDashDilationActive _character) :!label _label
            (Utilities|FlowControl|Delay 0.01)
            (Utilities|FlowControl|Sequence
              (:then_0
                (Utilities|FlowControl|DoOnce false
                  (:Completed
                    (Variables|/Script/Engine.Actor|SetCustomTimeDilation _character 0.25))))
              (:then_1
                (goto _label)))
            (else
              (Utilities|Time|SetGlobalTimeDilation 1.0)
              (Variables|/Script/Engine.Actor|SetCustomTimeDilation _character (Variables|Default|GetBaseCustomTD))
              (Variables|Default|SetIsCurrentlyActive false)
              (CallFunction|ResetGrappleHookSpeed)
              (Rendering|Material|SetMaterial (Variables|Character|GetMesh) 0 "/Game/TECH/Jay/Materials/M_TemporalZoneMat_Inst.M_TemporalZoneMat_Inst")
              (Utilities|MSpawnFX))))))))

(event Custom|UpdateGrappleHookSpeed
  (params (GrappleHook :type BP%20Grapple%20Hook%20Object%20Reference))
  ;[1 1 1] Update hook speed - done in grapple hook if pillar is active
  (Variables|Default|SetBaseGHSpeed (Variables|/Game/TECH/Jay/Blueprints/GrappleElements/BP_GrappleHook.BP_GrappleHook_C|GetGrappleHookSpeed GrappleHook))
  (Variables|/Game/TECH/Jay/Blueprints/GrappleElements/BP_GrappleHook.BP_GrappleHook_C|SetGrappleHookSpeed GrappleHook (* (Variables|/Game/TECH/Jay/Blueprints/GrappleElements/BP_GrappleHook.BP_GrappleHook_C|GetGrappleHookSpeed GrappleHook) 4.0)))

(event Custom|SpawnFX
  ;[1 1 1] Set actor to visible
  (Utilities|MSpawnFX))

(event Custom|ResetGrappleHookSpeed
  ;[1 1 1] Only reset grapple hook speed if still valid when pillar deactivates
  (Utilities|IsValid (stale Custom|UpdateGrappleHookSpeed GrappleHook)
    (:Is%20Valid
      (Variables|/Game/TECH/Jay/Blueprints/GrappleElements/BP_GrappleHook.BP_GrappleHook_C|SetGrappleHookSpeed (stale Custom|UpdateGrappleHookSpeed GrappleHook) (Variables|Default|GetBaseGHSpeed)))))

(event EventBeginPlay
  ;[1 1 1] Begin play - hide
  (|CallParentFunction)
  (Rendering|SetActorHiddenInGame true))

(event EventIDisablePillarZone
  ;[1 1 1] Overlapping pullar zone causes time dilation
  (Utilities|Time|SetGlobalTimeDilation 1.0)
  (Variables|/Script/Engine.Actor|SetCustomTimeDilation (Variables|Default|GetCharacter) (Variables|Default|GetBaseCustomTD))
  (Variables|Default|SetIsCurrentlyActive false)
  (CallFunction|ResetGrappleHookSpeed)
  (Rendering|Material|SetMaterial (Variables|Character|GetMesh) 0 "/Game/TECH/Jay/Materials/M_TemporalZoneMat_Inst.M_TemporalZoneMat_Inst")
  (Utilities|MSpawnFX))

(event EventIApplyEnhancementEffect
  (params (Character :type BP%20Base%20Character%20Object%20Reference))
  ;[1 1 1] Set actor to visible
  (Variables|Default|SetCharacter Character)
  (Variables|Default|SetCanInteract true)
  (Rendering|SetActorHiddenInGame false)
  (Utilities|MSpawnFX))

(fn ConstructionScript
  (|CallParentFunction))

(fn ICheckShield
  (return false))