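; BP_UpgradeFloor is a wave mode upgrade floor piece that starts without collision and opens extra play area when activated.
; ActivatePlayArea shows the mesh, enables collision and spawns a BP_AISpawnLocation at the EnemySpawnLocation transform.
; After a very short delay it messages the game mode to update its AI spawn points.
; The construction script sets initial mesh visibility from the IsVisible flag.
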(event Custom|ActivatePlayArea
  (bind _enemyspawnlocation (Variables|Default|GetEnemySpawnLocation))
  (bind _returnvalue (Transformation|GetWorldTransform _enemyspawnlocation))
  (Rendering|SetVisibility (Variables|Character|GetMesh) true false)
  (Collision|SetActorEnableCollision true)
  (Game|SpawnActorfromClass "/Game/TECH/Jay/WaveMode/BP_AISpawnLocation.BP_AISpawnLocation_C" (Math|Transform|MakeTransform (.location _returnvalue) (.rotation _returnvalue) "1,1,1") "Undefined" 0 0)
  (Utilities|FlowControl|Delay 0.01)
  (Class|BPIGamemodeElements|IUpdateAISpawnPoints(Message) (Game|GetGameMode)))

(event EventBeginPlay
  (Collision|SetActorEnableCollision false))

(fn ConstructionScript
  (bind _mesh (Variables|Character|GetMesh))
  (|CallParentFunction)
  (if (Variables|Default|GetIsVisible)
    (Rendering|SetVisibility _mesh true false)
    (else
      (Rendering|SetVisibility _mesh false false))))