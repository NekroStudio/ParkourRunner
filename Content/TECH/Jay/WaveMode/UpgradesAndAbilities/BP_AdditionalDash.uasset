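; BP_AdditionalDash is a Wave Mode upgrade that grants a character one additional dash.
; When the IApplyEnhancementEffect event fires, it increments the passed-in character's NumberOfDashes and sets TempRemainingDashes to the new total, refilling the available dashes.
; All other events are unused defaults, so the upgrade's logic lives entirely in that one event.
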(event EventBeginPlay
  (|CallParentFunction) ; This node is disabled and will not be called.\nDrag off pins to build functionality.
)

(event Collision|EventActorBeginOverlap
  (params (OtherActor :type Actor%20Object%20Reference))
  (|CallParentFunction OtherActor) ; This node is disabled and will not be called.\nDrag off pins to build functionality.
)

(event EventTick
  (params (DeltaSeconds :type Float%20%28single-precision%29))
  (|CallParentFunction DeltaSeconds) ; This node is disabled and will not be called.\nDrag off pins to build functionality.
)

(event EventIApplyEnhancementEffect
  (params (Character :type BP%20Base%20Character%20Object%20Reference))
  ;[1 1 1] Increase number of dashes
  (bind _output_get (Variables|Default|SetCharacter Character))
  (Math|Integer|IncrementInt (Variables|/Game/TECH/Jay/BP_BaseCharacter.BP_BaseCharacter_C|GetNumberOfDashes _output_get)
    (:%20%20
      (Variables|/Game/TECH/Jay/BP_BaseCharacter.BP_BaseCharacter_C|SetTempRemainingDashes _output_get (Variables|/Game/TECH/Jay/BP_BaseCharacter.BP_BaseCharacter_C|GetNumberOfDashes _output_get)))))

(fn ConstructionScript
  (|CallParentFunction))