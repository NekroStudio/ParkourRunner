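; BP_EnvironmentExpansion is a wave mode upgrade that expands the playable environment when its enhancement effect is applied.
; On IApplyEnhancementEffect, it finds every BP_UpgradeFloor in the level and calls ActivatePlayArea on each, then does the same for every BP_AdditionalPlayArea.
; The Blueprint holds no other active logic and leaves the actual activation to those actors.
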(event EventBeginPlay
  (|CallParentFunction) ; This node is disabled and will not be called.\nDrag off pins to build functionality.
)

(event Collision|EventActorBeginOverlap
  (params (OtherActor :type Actor%20Object%20Reference))
  (|CallParentFunction OtherActor) ; This node is disabled and will not be called.\nDrag off pins to build functionality.
)

(event EventTick
  (params (DeltaSeconds :type Float%20%28single-precision%29))
  (|CallParentFunction DeltaSeconds) ; This node is disabled and will not be called.\nDrag off pins to build functionality.
)

(event EventIApplyEnhancementEffect
  (params (Character :type BP%20Base%20Character%20Object%20Reference))
  (Utilities|FlowControl|Sequence
    (:then_0
      (bind _outactors (Actor|GetAllActorsOfClass "/Game/TECH/Jay/WaveMode/UpgradeEffects/BP_UpgradeFloor.BP_UpgradeFloor_C"))
      (for _array_element _outactors
        (Default|ActivatePlayArea _array_element)))
    (:then_1
      (bind _outactors_2 (Actor|GetAllActorsOfClass "/Game/TECH/Jay/WaveMode/UpgradeEffects/BP_AdditionalPlayArea.BP_AdditionalPlayArea_C"))
      (for _array_element_2 _outactors_2
        (Default|ActivatePlayArea _array_element_2)))))

(fn ConstructionScript
  (|CallParentFunction))