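; BP_Instinct is a wave-mode upgrade that lengthens how long a character can use time dilation.
; When the ApplyEnhancementEffect interface event fires, it stores the passed-in character and multiplies that character's maximum time dilation time by one and a half.
; The multiplier works on the current value, and the Blueprint has no other active logic.
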(event EventBeginPlay
  (|CallParentFunction) ; This node is disabled and will not be called.\nDrag off pins to build functionality.
)

(event Collision|EventActorBeginOverlap
  (params (OtherActor :type Actor%20Object%20Reference))
  (|CallParentFunction OtherActor) ; This node is disabled and will not be called.\nDrag off pins to build functionality.
)

(event EventTick
  (params (DeltaSeconds :type Float%20%28single-precision%29))
  (|CallParentFunction DeltaSeconds) ; This node is disabled and will not be called.\nDrag off pins to build functionality.
)

(event EventIApplyEnhancementEffect
  (params (Character :type BP%20Base%20Character%20Object%20Reference))
  (bind _output_get (Variables|Default|SetCharacter Character))
  (Variables|/Game/TECH/Jay/BP_BaseCharacter.BP_BaseCharacter_C|SetMaxTimeDilationTime _output_get (* (Variables|/Game/TECH/Jay/BP_BaseCharacter.BP_BaseCharacter_C|GetMaxTimeDilationTime _output_get) 1.5)))

(fn ConstructionScript
  (|CallParentFunction))