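; BP_SharpEdged is a wave-mode upgrade that extends the reach of a character's sword.
; When the enhancement effect interface event fires, it queries the character's weapon child actor through an interface for the sword and its collision half height.
; It then doubles the sword collision capsule's half height and the sword's attack range.
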(event EventBeginPlay
  (|CallParentFunction) ; This node is disabled and will not be called.\nDrag off pins to build functionality.
)

(event Collision|EventActorBeginOverlap
  (params (OtherActor :type Actor%20Object%20Reference))
  (|CallParentFunction OtherActor) ; This node is disabled and will not be called.\nDrag off pins to build functionality.
)

(event EventIApplyEnhancementEffect
  (params (Character :type BP%20Base%20Character%20Object%20Reference))
  ;[1 1 1] adjust collision for sword (increased half height)
  (bind (_sword _halfheight) (Class|BPiCombat|ISwordCollisionHalfHeight(Message) (Variables|/Script/Engine.ChildActorComponent|GetChildActor (Variables|/Game/TECH/Jay/BP_BaseCharacter.BP_BaseCharacter_C|GetWeapon Character))))
  (Components|Capsule|SetCapsuleHalfHeight (Variables|/Game/TECH/Mitz/Blueprints/BP_Sword.BP_Sword_C|GetSwordCollision _sword) (* _halfheight 2.0) true)
  (Variables|/Game/TECH/Mitz/Blueprints/BP_Sword.BP_Sword_C|SetAttackRange _sword (* (Variables|/Game/TECH/Mitz/Blueprints/BP_Sword.BP_Sword_C|GetAttackRange _sword) 2.0)))

(fn ConstructionScript
  (|CallParentFunction))