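; BP_Stimulated is a wave mode enhancement that raises a character's movement speed.
; When applied through IApplyEnhancementEffect, it stores the character and scales walk, wall-run and grapple speeds by one shared multiplier.
; Three helper functions write to the CharacterMovement, parkour and grapple components, each saving the original value first, though nothing here restores it.
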(event EventBeginPlay
  (|CallParentFunction) ; This node is disabled and will not be called.\nDrag off pins to build functionality.
)

(event Collision|EventActorBeginOverlap
  (params (OtherActor :type Actor%20Object%20Reference))
  (|CallParentFunction OtherActor) ; This node is disabled and will not be called.\nDrag off pins to build functionality.
)

(event EventTick
  (params (DeltaSeconds :type Float%20%28single-precision%29))
  (|CallParentFunction DeltaSeconds) ; This node is disabled and will not be called.\nDrag off pins to build functionality.
)

(event EventIApplyEnhancementEffect
  (params (Character :type BP%20Base%20Character%20Object%20Reference))
  ;[1 1 1] Increases movement speed
  (Variables|Default|SetCharacter Character)
  (Utilities|MUpdateCharMovementSpeed)
  (Utilities|MUpdateWallRunMovSpeed)
  (Utilities|MUpdateCharGrappleSpeed))

(fn ConstructionScript
  (|CallParentFunction))