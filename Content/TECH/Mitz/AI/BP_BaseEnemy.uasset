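; Base enemy Blueprint that hands its Behaviour Tree to the AI controller and leaves Shoot, Death and Reload for children.
; Any damage kills it: AI stops, the mesh ragdolls, the damage causer gets score and the linked door deducts the enemy.
; Kills persist via game mode and save slot, so init destroys already-killed enemies or registers survivors with their door.
; Gun jamming temporarily pauses AI logic, and a gated flip rotates the capsule 180 degrees.
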(event Custom|Shoot
  (params (Target :type Actor%20Object%20Reference))
  ;[1 1 1] Tells the child actors to shoot depending on if the target is valid
)

(event Custom|Reload
  ;[1 1 1] Tells the child actors to shoot depending on if the target is valid
)

(event Custom|AllowRotation
  ;[1 1 1] Once the enemy rotates a certain amount, flip them 180 so that they face th player again
  (Utilities|FlowControl|DoOnce false) ; enters at Reset
)

(event Custom|Death
  ;[1 1 1] Tells the child actors to shoot depending on if the target is valid
)

(event Custom|TempDisableShooting
  (bind _self self)
  (bind _returnvalue (AI|GetAIController _self))
  (bind _braincomponent (Variables|/Script/AIModule.AIController|GetBrainComponent _returnvalue))
  ;[0 0.2846 1] Jam Shooting
  (Variables|Default|SetGunDisabled true)
  (Variables|Default|SetTarget 0)
  (bind _returnvalue_2 (Niagara|SpawnSystemAttached "/Game/TECH/Mitz/Particles/NS_Smoke_System.NS_Smoke_System" (Variables|Default|GetGunMesh) "Muzzle" "0, 0, 0" "0, 0, 0" "KeepRelativeOffset" true))
  (AI|Logic|StopLogic _braincomponent "")
  (Utilities|FlowControl|Delay (Variables|Default|GetJammedDuration))
  (Components|Activation|Deactivate _returnvalue_2)
  (Variables|Default|SetGunDisabled false)
  (AI|Logic|StartLogic _braincomponent))

(event EventIShoot
  (params (Target :type Actor%20Object%20Reference))
  ;[1 1 1] Tells the child actors to shoot depending on if the target is valid
  (if (not (Variables|Default|Getdead?))
    (if (not (Variables|Default|GetGunDisabled))
      (Variables|Default|SetTarget Target)
      (Utilities|IsValid Target
        (:Is%20Valid
          (CallFunction|Shoot Target))
        (:Is%20Not%20Valid
          (CallFunction|Shoot))))))

(event EventBeginPlay
  ;[1 1 1] Sends the Behaviour Tree to the AI Controller
  (Class|BPiAI|ISendBT(Message) (AI|GetAIController self) (Variables|Default|GetBTAsset)))

(event EventIFlip
  ;[1 1 1] Once the enemy rotates a certain amount, flip them 180 so that they face th player again
  (Utilities|FlowControl|DoOnce false
    (:Completed
      (Transformation|AddRelativeRotation (Variables|Collision|GetCapsuleComponent) "0,-180.000000, 0" false false)
      (Utilities|FlowControl|Delay 0.2)
      (CallFunction|AllowRotation))))

(event EventIInitEnemies
  ;[1 1 1] Init
  ;;[1 1 1] Loads the save slot
  (Utilities|FlowControl|Sequence
    (:then_0
      ;[1 1 1] Sends the Behaviour Tree to the AI Controller
      (Class|BPiAI|ISendBT(Message) (AI|GetAIController self) (Variables|Default|GetBTAsset)))
    (:then_1
      (bind _returnvalue (SaveGame|LoadGamefromSlot "Save1"))
      (bind _saveslot (Class|ISaveGame|IConvertSaveSlot(Message) _returnvalue))
      ;;[1 1 1] Checks if the check point is contained
      (if (Utilities|Array|ContainsItem (Variables|/Game/TECH/Mitz/Blueprints/BP_SaveGame.BP_SaveGame_C|GetKilledEnemies _saveslot) self)
        ;;[1 1 1] If it is, destroy the enemy
        (Actor|DestroyActor)
        (else
          ;;[0 0.2846 1] If not, setup the connected door (if valid)
          (bind _connecteddoor (Variables|Default|GetConnectedDoor)
            (:then
              (Class|BPIEnvironmentalInteractions|ISetupDoor(Message) _connecteddoor self))
            (:else)))))))

(event Game|Damage|EventAnyDamage
  (params (Damage :type Float%20%28single-precision%29) (DamageType :type Damage%20Type%20Object%20Reference) (InstigatedBy :type Controller%20Object%20Reference) (DamageCauser :type Actor%20Object%20Reference))
  (bind _self self)
  ;[1 1 1] Saves the checkpoint
  ;;[1 1 1] When the enemy takes damage
  (Variables|Default|Setdead? true)
  ;;[0 0.2846 1] Stop brain function
  (CallFunction|Death)
  ;;[1 1 1] Sets the spawn point in the spawn manager
  (Utilities|MStopAILogic) ; Prevents shootings after death
  (bind _returnvalue (SaveGame|LoadGamefromSlot "Save1"))
  (bind _saveslot (Class|ISaveGame|IConvertSaveSlot(Message) _returnvalue))
  ;;[1 1 1] Checks if it is contained
  (if (Utilities|Array|ContainsItem (Variables|/Game/TECH/Mitz/Blueprints/BP_SaveGame.BP_SaveGame_C|GetKilledEnemies _saveslot) self)
    ;;[1 1 1] Saves the game and sets the spawn point and destroys the checkpoint
    (CallFunction|FDead :!label _label)
    (Class|BPiCombat|IGiveKill(Message) DamageCauser (Variables|Default|GetScoreOnKilled) _self)
    ;;;[0 0.2846 1] Deduct enemy from door
    (bind _connecteddoor (Variables|Default|GetConnectedDoor)
      (:then
        (Class|BPIEnvironmentalInteractions|IDeductEnemy(Message) _connecteddoor _self))
      (:else
        _))
    (Components|Activation|Activate (Variables|Default|GetDeathFX) true)
    (Utilities|FlowControl|Delay 1.0)
    (Rendering|SetVisibility (Variables|Character|GetMesh) false false)
    (Utilities|FlowControl|Sequence
      (:then_0
        (Components|Activation|Deactivate (Variables|Default|GetDeathFX)))
      (:then_1
        (Utilities|FlowControl|Delay 1.0)
        (Actor|DestroyActor)))
    (else
      (Class|ISaveGame|IAddKilledEnemy(Message) (Game|GetGameMode) self)
      (bind _returnvalue_2 (SaveGame|SaveGametoSlot _saveslot "Save1"))
      (if _returnvalue_2
        (goto _label)))))

(fn ConstructionScript)

(fn FUpdateBBKeys)

(fn FDead
  (bind _mesh (Variables|Character|GetMesh))
  (Collision|SetCollisionEnabled _mesh "QueryAndPhysics")
  (Physics|SetSimulatePhysics _mesh true)
  (Collision|SetCollisionEnabled (Variables|Collision|GetCapsuleComponent) "NoCollision")
  (Class|BPiAI|IStopBehaviour(Message) (AI|GetAIController self))
  (Collision|SetCollisionResponsetoChannel (Variables|Character|GetMesh) "ECC_GameTraceChannel3" "ECR_Ignore")
  (Audio|PlaySound2D "/Game/TECH/Jay/Sounds/SC_RandomKillLine.SC_RandomKillLine" 1.0 1.0 0.0 0 0))

(fn IAnimationVaribales
  (return (Variables|Default|GetTarget)))

(fn IConvertSaveSlot
  (return 0))

(fn IGetCheckPointActiveTime
  (return 0.0))

(fn IGetKilledEnemies
  (return 0))

(fn IGetPlayerController
  (return 0))

(fn IGetRotationSpeed
  (return (Variables|Default|GetrotationSpeed)))

(fn IGetShootDelay
  (return 0.0))

(fn IGetTarget
  (return (Variables|Default|GetTarget)))

(fn IGetTime
  (return 0.0))