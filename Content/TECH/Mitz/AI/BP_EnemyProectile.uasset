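; Enemy projectile Blueprint that damages the player unless blocked, in which case it bounces back.
; Blocking reverses its velocity with random spread, after which its overlaps can damage non-player actors too.
; Damaging overlaps spawn Niagara blood using hit data from a looping forward sphere trace that starts upon reflection.
; A looping timer line-traces ahead, destroying the projectile on hits other than BP_BaseCharacter.
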(event OnComponentBeginOverlap(Box)
  (params (OverlappedComponent :type Primitive%20Component%20Object%20Reference) (OtherActor :type Actor%20Object%20Reference) (OtherComp :type Primitive%20Component%20Object%20Reference) (OtherBodyIndex :type Integer) (bFromSweep :type Boolean) (SweepResult :type Hit%20Result%20Structure%20%28by%20ref%29))
  (Utilities|MIsPlayer OtherActor
    (:true
      (bind _blocking_ (Class|BPiCombat|ICheckBlocking(Message) OtherActor))
      (if _blocking_
        (CallFunction|IReflectBullet)
        (else
          (Niagara|SpawnSystemAttached "/Game/TECH/Mitz/Particles/NS_Blood.NS_Blood" (Variables|Default|GetHit%20Component) "None" (Variables|Default|GetImpact%20Point) (Math|Conversions|RotationFromXVector (Variables|Default|GetImpact%20Normal)) "KeepWorldPosition" false :!label _label)
          (Game|Damage|ApplyDamage OtherActor 1.0 0 self))))
    (:false
      (if (Variables|Default|GetReflected)
        (goto _label)))))

(event Custom|Trace
  (CallFunction|FTraceforWall))

(event Custom|CheckForHIt
  (bind _returnvalue (Transformation|GetActorLocation))
  (bind (_outhit _returnvalue_2) (Collision|SphereTraceByChannel _returnvalue (+ _returnvalue (* (Transformation|GetActorForwardVector) 2.5e+02)) 64.0 "TraceTypeQuery4" false 0 "None"))
  (if _returnvalue_2
    (Variables|Default|SetImpact%20Point (.ImpactPoint (Collision|BreakHitResult _outhit)))
    (Variables|Default|SetImpact%20Normal (.ImpactNormal (Collision|BreakHitResult _outhit)))
    (Variables|Default|SetHit%20Component (.HitComponent (Collision|BreakHitResult _outhit)))))

(event EventIReflectBullet
  (bind _projectilemovement (Variables|Default|GetProjectileMovement))
  (Variables|Default|SetReflected true)
  (Variables|/Script/Engine.MovementComponent|SetVelocity _projectilemovement (+ (* (Variables|/Script/Engine.MovementComponent|GetVelocity _projectilemovement) -1.0) (Math|Vector|MakeVector (Math|Random|RandomFloatinRange -2e+02 2e+02) (Math|Random|RandomFloatinRange -2e+02 2e+02) (Math|Random|RandomFloatinRange -2e+02 2e+02))))
  (bind _returnvalue (Utilities|Time|SetTimerbyEvent (delegate Custom|CheckForHIt) 0.01 true))
  (Variables|Default|SetTraceForBlood _returnvalue))

(event EventBeginPlay
  (bind _returnvalue (Utilities|Time|SetTimerbyEvent (EventDispatchers|CreateEvent :!event Custom|Trace) 0.01 true))
  (Variables|Default|SetTraceTimer _returnvalue))

(fn ConstructionScript)

(fn FCheckWall
  (params (hasHit? :type Boolean) (Result :type Hit%20Result%20Structure%20%28by%20ref%29))
  (if hasHit?
    (if (!= (Utilities|GetClass (.HitActor (Collision|BreakHitResult Result))) "/Game/TECH/Jay/BP_BaseCharacter.BP_BaseCharacter_C")
      (Actor|DestroyActor))))

(fn FTraceforWall
  (bind (_start _end) (Utilities|MVectorMath))
  (bind (_outhit _returnvalue) (Collision|LineTraceByChannel _start _end "TraceTypeQuery1" false (Utilities|Array|MakeArray self) "None"))
  (CallFunction|FCheckWall _returnvalue _outhit))

(fn ICheckBlocking
  (return false))

(fn IGetKills
  (return 0))

(fn ISwordCollisionHalfHeight
  (return 0 0.0))