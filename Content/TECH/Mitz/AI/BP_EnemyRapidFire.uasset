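; BP_EnemyRapidFire is an enemy that sprays projectiles at a target until its ammo runs out, then reloads.
; Shoot passes a DoOnce gate to start a looping timer, which re-aims ProjectileArrow and spawns BP_EnemyProectile each tick while not Dead.
; An empty magazine stops the timer, prints a debug message and refills after a delay.
; Reload completion or an invalid target reopens the gate.
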(event Custom|Shooting
  (params (Target :type Actor%20Object%20Reference))
  (Variables|Default|SetTarget Target)
  (bind _returnvalue (Utilities|Time|SetTimerbyEvent (delegate Custom|RapidFire) (Variables|Default|GetBulletDelay) true))
  (Variables|Default|SetSprayTimer _returnvalue))

(event Custom|RapidFire
  (bind _target (Variables|Default|GetTarget))
  (bind _projectilearrow (Variables|Default|GetProjectileArrow))
  (bind _returnvalue (Transformation|GetWorldLocation _projectilearrow))
  (Utilities|IsValid _target
    (:Is%20Valid
      (if (not (Variables|Default|Getdead?))
        (Transformation|SetWorldRotation (Variables|Default|GetProjectileArrow) (Math|Rotator|FindLookatRotation _returnvalue (Transformation|GetActorLocation _target)) false false)
        (Game|SpawnActorfromClass "/Game/TECH/Mitz/AI/BP_EnemyProectile.BP_EnemyProectile_C" (Math|Transform|MakeTransform _returnvalue (Math|Conversions|RotationFromXVector (Math|Vector|GetForwardVector (Variables|Default|GetProjectileArrow))) "0.300000,0.300000,0.300000") "Undefined" 0 0)
        (bind _result (Math|Integer|DecrementInt (Variables|Default|GetAmmo))
          (:%20%20
            (if (<= _result 0)
              (Utilities|Time|ClearandInvalidateTimerbyHandle (Variables|Default|GetSprayTimer))
              (CallFunction|Reload))))))
    (:Is%20Not%20Valid
      (Utilities|Time|ClearandInvalidateTimerbyHandle (Variables|Default|GetSprayTimer))
      (CallFunction|ResetShootDoOnce))))

(event Custom|ResetShootDoOnce
  (Utilities|FlowControl|DoOnce false) ; enters at Reset
)

(event EventBeginPlay
  (|CallParentFunction) ; This node is disabled and will not be called.\nDrag off pins to build functionality.
)

(event Collision|EventActorBeginOverlap
  (params (OtherActor :type Actor%20Object%20Reference)))

(event EventTick
  (params (DeltaSeconds :type Float%20%28single-precision%29)))

(event EventShoot
  (params (Target :type Actor%20Object%20Reference))
  (Utilities|FlowControl|DoOnce false
    (:Completed
      (CallFunction|Shooting Target))))

(event EventReload
  (Development|PrintString (Utilities|String|Append (Utilities|GetDisplayName self) ":" "Reloading") true true "(R=1.000000,G=0.000000,B=0.000000,A=1.000000)")
  (Utilities|FlowControl|Delay (Variables|Default|GetReloadDelay))
  (Variables|Default|SetAmmo (Variables|Default|GetMaxammo))
  (CallFunction|ResetShootDoOnce))

(fn ConstructionScript
  (|CallParentFunction)
  (Variables|Default|SetAmmo (Variables|Default|GetMaxammo)))