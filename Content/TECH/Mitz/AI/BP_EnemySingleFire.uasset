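; Enemy Blueprint for a single-shot attacker that charges, then fires one projectile at its target.
; Shoot attaches a charge Niagara effect to the gun muzzle once per cycle while a delay runs.
; After the delay, if still alive with a valid target, it aims an arrow component, spawns the projectile, alerts the target's indicator through an interface call and resets the charge.
; Death destroys the charge effect.
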(event Custom|ResetCharge
  (Utilities|FlowControl|DoOnce false) ; enters at Reset
)

(event EventBeginPlay
  (|CallParentFunction) ; This node is disabled and will not be called.\nDrag off pins to build functionality.
)

(event Collision|EventActorBeginOverlap
  (params (OtherActor :type Actor%20Object%20Reference)))

(event EventTick
  (params (DeltaSeconds :type Float%20%28single-precision%29)))

(event EventShoot
  (params (Target :type Actor%20Object%20Reference))
  (bind _projectilearrow (Variables|Default|GetProjectileArrow))
  (bind _returnvalue (Transformation|GetWorldLocation _projectilearrow))
  (Utilities|FlowControl|Sequence
    (:then_0
      (Utilities|FlowControl|Delay (Variables|Default|GetShootDelay))
      (Utilities|IsValid Target
        (:Is%20Valid
          (if (not (Variables|Default|Getdead?))
            (Transformation|SetWorldRotation (Variables|Default|GetProjectileArrow) (Math|Rotator|FindLookatRotation _returnvalue (Transformation|GetActorLocation Target)) false false)
            (Game|SpawnActorfromClass "/Game/TECH/Mitz/AI/BP_EnemyProectile.BP_EnemyProectile_C" (Math|Transform|MakeTransform _returnvalue (Math|Conversions|RotationFromXVector (Math|Vector|GetForwardVector (Variables|Default|GetProjectileArrow))) "0.300000,0.300000,0.300000") "Undefined" 0 0)
            (Class|BPiCombat|IShowIndicator(Message) Target (Transformation|GetActorLocation))
            (CallFunction|ResetCharge)))))
    (:then_1
      (Utilities|FlowControl|DoOnce false
        (:Completed
          (if (not (Variables|Default|Getdead?))
            (bind _returnvalue_2 (Niagara|SpawnSystemAttached "/Game/TECH/Mitz/Particles/NS_ChargeBallSingle.NS_ChargeBallSingle" (Variables|Default|GetGunMesh) "Muzzle" "0, 0, 0" "0, 0, 0" "KeepRelativeOffset" true))
            (Variables|Default|SetEmitter _returnvalue_2)))))))

(event EventDeath
  (bind _emitter (Variables|Default|GetEmitter))
  (Utilities|IsValid _emitter
    (:Is%20Valid
      (Components|DestroyComponent _emitter))))

(fn ConstructionScript
  (|CallParentFunction))