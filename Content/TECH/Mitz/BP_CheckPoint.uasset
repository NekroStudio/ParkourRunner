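; BP_CheckPoint is a checkpoint trigger that updates the spawn point when the character enters it.
; On box overlap by an actor whose class is exactly BP_BaseCharacter, it finds BP_SpawnManager and sends it the Billboard's world transform through the ISetSpawnPointMessage interface call.
; The construction script sizes the trigger box from the Extent variable, while the Billboard marks the respawn transform.
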(event OnComponentBeginOverlap(Box)
  (params (OverlappedComponent :type Primitive%20Component%20Object%20Reference) (OtherActor :type Actor%20Object%20Reference) (OtherComp :type Primitive%20Component%20Object%20Reference) (OtherBodyIndex :type Integer) (bFromSweep :type Boolean) (SweepResult :type Hit%20Result%20Structure%20%28by%20ref%29))
  (if (== (Utilities|GetClass OtherActor) "/Game/TECH/Jay/BP_BaseCharacter.BP_BaseCharacter_C")
    (bind _returnvalue (Actor|GetActorOfClass "/Game/TECH/Mitz/BP_SpawnManager.BP_SpawnManager_C"))
    (Class|BPiSpawning|ISetSpawnPoint(Message) _returnvalue (Transformation|GetWorldTransform (Variables|Default|GetBillboard)))))

(fn ConstructionScript
  (Components|Box|SetBoxExtent (Variables|Default|GetBox) (Variables|Default|GetExtent) true))