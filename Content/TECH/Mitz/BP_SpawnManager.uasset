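; BP_SpawnManager spawns the player character and tracks the point where that player respawns.
; On BeginPlay it finds the BP_PlayerStart, spawns the character at its transform and has player controller 0 possess it.
; Interface-style events update the stored spawn transform and respawn by moving the existing pawn to its location and rotation, without creating a new one.
; IGetController is an empty stub.
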(event Custom|Spawn
  (bind _playerstart (Variables|Default|GetPlayerStart))
  (bind _returnvalue (Transformation|GetActorTransform _playerstart))
  (Variables|Default|SetSpawnLoc _returnvalue)
  (bind _returnvalue_2 (Game|SpawnActorfromClass (Variables|Default|GetPlayerCharacter) _returnvalue "Undefined" 0 0))
  (Variables|Default|SetPlayer _returnvalue_2)
  (Pawn|Possess (Game|GetPlayerController 0) _returnvalue_2))

(event EventBeginPlay
  (bind _returnvalue (Actor|GetActorOfClass "/Game/TECH/Mitz/BP_PlayerStart.BP_PlayerStart_C"))
  (Utilities|IsValid _returnvalue
    (:Is%20Valid
      (Variables|Default|SetPlayerStart _returnvalue)
      (CallFunction|Spawn))))

(event EventIPlayerSpawn
  (bind _spawnloc (Variables|Default|GetSpawnLoc))
  (Transformation|SetActorTransform (Variables|Default|GetPlayer) (Math|Transform|MakeTransform (.location _spawnloc) (.rotation _spawnloc) "1,1,1")))

(event EventISetSpawnPoint
  (params (SpawnLoc :type Transform))
  (Variables|Default|SetSpawnLoc SpawnLoc))

(fn ConstructionScript)

(fn IGetController
  (return 0))