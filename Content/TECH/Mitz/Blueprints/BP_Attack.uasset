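; BP_Attack handles a character's two-step melee attack combo, driven through combat interface events.
; Attacks play animations on the owning character, buffer input pressed mid-swing for the combo event, and reset on completion or via a two-second retriggerable fail-safe.
; A separate effects event spawns Niagara blood on the hit actor if the save's Gore setting is enabled.
; The camera sphere-trace damage is disconnected, and the blocking, kills and sword-collision getters are stubs.
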(event Custom|ContinueAttackEffects
  (params (ImpactPoint :type Vector) (ImpactNormal :type Vector) (HitComponent :type Primitive%20Component%20Object%20Reference) (HitActor :type Actor%20Object%20Reference))
  (bind _rootcomponent (Variables|/Script/Engine.Actor|GetRootComponent HitActor))
  (bind _returnvalue (Transformation|GetWorldLocation _rootcomponent))
  ;[0.07998 1 0] Attack Trace from the camera
  ;[0.07998 1 0] Blood Spawn
  (bind _returnvalue_2 (SaveGame|LoadGamefromSlot "Save1"))
  (bind _saveslot (Class|ISaveGame|IConvertSaveSlot(Message) _returnvalue_2))
  (if (Variables|/Game/TECH/Mitz/Blueprints/BP_SaveGame.BP_SaveGame_C|GetGore? _saveslot)
    (Variables|Default|SetImpact%20Point ImpactPoint)
    (Variables|Default|SetImpact%20Normal ImpactNormal)
    (Variables|Default|SetHit%20Component HitComponent)
    (Niagara|SpawnSystemAttached "/Game/TECH/Mitz/Particles/NS_Blood.NS_Blood" _rootcomponent "None" _returnvalue (Math|Conversions|RotationFromXVector (* (Variables|Default|GetImpact%20Normal) -1.0)) "KeepWorldPosition" false)
    (Niagara|SpawnSystemAttached "/Game/TECH/Mitz/Particles/NS_Blood.NS_Blood" _rootcomponent "None" _returnvalue (Math|Conversions|RotationFromXVector (Variables|Default|GetImpact%20Normal)) "KeepWorldPosition" false)))

(event Custom|FailSafeAttack
  ;[0.07998 1 0] Fail safe for the attacks
  (Utilities|FlowControl|RetriggerableDelay 2.0)
  (CallFunction|FResetAttacks))

(event EventIAttackTraceON
  (params (Character :type BP%20Base%20Character%20Object%20Reference)))

(event EventICharacterCombat
  (params (Character :type BP%20Base%20Character%20Object%20Reference))
  ;[0.07998 1 0] Init and set the character
  (Variables|Default|SetCharacter Character))

(event EventIAttackCombat
  ;[0.07998 1 0] Combo system
  ;;[0.3203 1 0.1892] Checks if the player is already attacking
  (if (Variables|Default|GetAttacking?)
    ;;[0.3203 1 0.1892] If they are save the attack
    (Variables|Default|SetSaveAttack? true)
    (else
      ;;[0.3203 1 0.1892] If they are not set attacking to true and switch on the attack counter
      (Variables|Default|SetAttacking? true)
      (switch int (Variables|Default|GetAttackCounter)
        (:0
          ;;[0.3203 1 0.1892] Play the animation and set the attack counter and then begin the fail safe
          (Default|IPlayAnimation (Variables|Default|GetCharacter) (Variables|Default|GetAttackCounter))
          (Math|Integer|IncrementInt (Variables|Default|GetAttackCounter)
            (:%20%20
              _)))
        (:1
          (Default|IPlayAnimation (Variables|Default|GetCharacter) (Variables|Default|GetAttackCounter))
          (Variables|Default|SetAttackCounter 0)))
      (CallFunction|FailSafeAttack))))

(event EventIAttackComboCombat
  ;[0.07998 1 0] Combo system
  ;;[0.3203 1 0.1892] Checks if save attack is set and if it is set it to false and if it is not reset the attacks
  (if (Variables|Default|GetSaveAttack?)
    (Variables|Default|SetSaveAttack? false)
    ;;[0.3203 1 0.1892] If they are not set attacking to true and switch on the attack counter
    (switch int (Variables|Default|GetAttackCounter)
      (:0
        ;;[0.3203 1 0.1892] Play the animation and set the attack counter and then begin the fail safe
        (Default|IPlayAnimation (Variables|Default|GetCharacter) (Variables|Default|GetAttackCounter))
        (Math|Integer|IncrementInt (Variables|Default|GetAttackCounter)
          (:%20%20
            _)))
      (:1
        (Default|IPlayAnimation (Variables|Default|GetCharacter) (Variables|Default|GetAttackCounter))
        (Variables|Default|SetAttackCounter 0)))
    (CallFunction|FailSafeAttack)
    (else
      (CallFunction|FResetAttacks))))

(fn FResetAttacks
  ;[0.3203 1 0.1892] Reset the attack counter and set attacking to false and save attack to false
  (Variables|Default|SetAttackCounter 0)
  (Variables|Default|SetAttacking? false)
  (Variables|Default|SetSaveAttack? false))

(fn ICheckBlocking
  (return false))

(fn IGetKills
  (return 0))

(fn ISwordCollisionHalfHeight
  (return 0 0.0))