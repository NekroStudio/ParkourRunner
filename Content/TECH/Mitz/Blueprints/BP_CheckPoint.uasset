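; BP_CheckPoint is a chained checkpoint actor that times how long it stays active and saves progress when the player reaches it.
; On init it destroys itself if Save1 lists it as used, or starts its 0.01-second looping timer if it is current.
; Player overlap reports times to the character, starts the next checkpoint, saves spawn transform and kills through the GameMode, then destroys the actor.
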(event OnComponentBeginOverlap(Box)
  (params (OverlappedComponent :type Primitive%20Component%20Object%20Reference) (OtherActor :type Actor%20Object%20Reference) (OtherComp :type Primitive%20Component%20Object%20Reference) (OtherBodyIndex :type Integer) (bFromSweep :type Boolean) (SweepResult :type Hit%20Result%20Structure%20%28by%20ref%29))
  (bind _returnvalue (Game|GetGameMode))
  ;[1 1 1] Saves the checkpoint
  ;;[1 1 1] Checks if the player is overlapping
  (Utilities|MIsPlayer OtherActor
    (:true
      (Variables|Default|SetCharacter OtherActor)
      ;;[1 1 1] Sets the spawn point in the spawn manager
      (bind _returnvalue_2 (SaveGame|LoadGamefromSlot "Save1"))
      (bind _saveslot (Class|ISaveGame|IConvertSaveSlot(Message) _returnvalue_2))
      ;;[1 1 1] Checks if it is contained
      (if (not (Utilities|Array|ContainsItem (Variables|/Game/TECH/Mitz/Blueprints/BP_SaveGame.BP_SaveGame_C|GetCheckPointsUsed _saveslot) self))
        ;;[1 1 1] Saves the game and sets the spawn point and destroys the checkpoint
        (Utilities|Time|ClearandInvalidateTimerbyHandle (Variables|ScoreElements|GetCheckpointTimerHandle))
        ;;;[0 0.2846 1] Send to player
        (Class|BPIEnvironmentalInteractions|IOverlappedCheckpoint(Message) (Variables|Default|GetCharacter) (Variables|ScoreElements|GetCurrentActiveTime) (Variables|Default|GetAverageTimeToReach) (Variables|Default|GetCheckpointIndex))
        ;;;[0 0.2846 1] Triggers next checkpoint timer
        (bind _nextcheckpoint (Variables|Default|GetNextCheckpoint)
          (:then
            (Class|ISaveGame|ITriggerNewCheckpointTimer(Message) _nextcheckpoint (Variables|Default|GetCheckpointIndex)))
          (:else
            _))
        (bind _killedenemies (Class|ISaveGame|IGetKilledEnemies(Message) _returnvalue))
        (bind _kills (Class|BPiCombat|IGetKills(Message) (Variables|Default|GetCharacter)))
        (Class|ISaveGame|ISaveGame(Message) _returnvalue (Transformation|GetWorldTransform (Variables|Default|GetArrow)) self _killedenemies _kills (Variables|Default|GetCheckpointIndex))
        (Class|ISaveGame|ISaveCurrentActiveCheckPoint(Message) (Game|GetGameMode) _nextcheckpoint)
        (Actor|DestroyActor)))))

(event Custom|TriggerCheckpointTimer
  ;[0 0.2846 1] Checkpoint timer
  (bind _returnvalue (Utilities|Time|SetTimerbyEvent (delegate Custom|UpdateCurrentActiveTime) 0.01 true))
  (Variables|ScoreElements|SetCheckpointTimerHandle _returnvalue)
  (Rendering|Material|SetMaterial (Variables|Default|GetStaticMesh1) 0 "/Game/TECH/Jay/Materials/M_testmat.M_testmat"))

(event Custom|UpdateCurrentActiveTime
  ;[0 0.2846 1] Checkpoint timer
  (Variables|ScoreElements|SetCurrentActiveTime (+ (Variables|ScoreElements|GetCurrentActiveTime) 0.01)))

(event EventITriggerNewCheckpointTimer
  (params (OldCheckpointIndex :type Integer))
  ;[0.4226 0 1] Shit don't work bruh
  (Math|Integer|IncrementInt (Variables|/Game/TECH/Mitz/Blueprints/BP_SaveGame.BP_SaveGame_C|GetCurrentActiveCheckpointIndex (Variables|Default|GetSave%20Slot))
    (:%20%20
      (CallFunction|TriggerCheckpointTimer))))

(event EventIInitCheckPoints
  ;[1 1 1] Init
  ;;[1 1 1] Loads the save slot
  (bind _returnvalue (SaveGame|LoadGamefromSlot "Save1"))
  (bind _saveslot (Class|ISaveGame|IConvertSaveSlot(Message) _returnvalue))
  (bind _output_get (Variables|Default|SetSave%20Slot _saveslot))
  ;;[1 1 1] Checks if the check point is contained
  (if (Utilities|Array|ContainsItem (Variables|/Game/TECH/Mitz/Blueprints/BP_SaveGame.BP_SaveGame_C|GetCheckPointsUsed _output_get) self)
    ;;[1 1 1] If it is destroy the check point
    (Actor|DestroyActor)
    (else
      ;;[0 0.2846 1] If not, trigger checkpoint timer
      (if (== (Variables|Default|GetCheckpointIndex) (Variables|/Game/TECH/Mitz/Blueprints/BP_SaveGame.BP_SaveGame_C|GetCurrentActiveCheckpointIndex (Variables|Default|GetSave%20Slot)))
        (CallFunction|TriggerCheckpointTimer)))))

(event EventIInitActiveCheckPoint
  (params (Time :type Float%20%28single-precision%29) (Character :type Actor%20Object%20Reference))
  ;[1 1 1] Init
  ;;[1 1 1] Initilize if current checkpoint
  (Variables|ScoreElements|SetCurrentActiveTime Time)
  (Variables|Default|SetCharacter Character)
  (CallFunction|TriggerCheckpointTimer))

(fn ConstructionScript
  (Components|Box|SetBoxExtent (Variables|Default|GetBox) (Variables|Default|GetExtent) true))

(fn IConvertSaveSlot
  (return 0))

(fn IGetCheckPointActiveTime
  (return (Variables|ScoreElements|GetCurrentActiveTime)))

(fn IGetKilledEnemies
  (return 0))

(fn IGetTime
  (return 0.0))