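; BP_MovingActorEnvironment is an environment prop wrapper that slowly rotates a chosen actor class at a random rate.
; The construction script assigns SelectedClass to a ChildActor component, so the displayed actor is configurable.
; On BeginPlay, it sets the RotatingMovement component's rate, giving each axis enabled by CanMoveX, CanMoveY or CanMoveZ a small random speed in either direction and zeroing the others.
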(event EventBeginPlay
  (Variables|/Script/Engine.RotatingMovementComponent|SetRotationRate (Variables|Default|GetRotatingMovement) (Math|Rotator|MakeRotator (Math|Float|SelectFloat (* (Math|Random|RandomFloatinRange -5.0 5.0) (Math|Float|SelectFloat 1.0 -1.0 (Math|Random|RandomBool))) 0.0 (Variables|Default|GetCanMoveX)) (Math|Float|SelectFloat (* (Math|Random|RandomFloatinRange -5.0 5.0) (Math|Float|SelectFloat 1.0 -1.0 (Math|Random|RandomBool))) 0.0 (Variables|Default|GetCanMoveY)) (Math|Float|SelectFloat (* (Math|Random|RandomFloatinRange -5.0 5.0) (Math|Float|SelectFloat 1.0 -1.0 (Math|Random|RandomBool))) 0.0 (Variables|Default|GetCanMoveZ)))))

(fn ConstructionScript
  (ChildActorComponent|SetChildActorClass (Variables|Default|GetChildActor) (Variables|Default|GetSelectedClass)))