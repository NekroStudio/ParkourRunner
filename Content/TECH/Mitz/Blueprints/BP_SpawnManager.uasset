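; Spawn manager that creates the player character at the level's BP_PlayerStart on BeginPlay, possesses it and passes it a reference to itself.
; Interface messages store the current spawn transform and checkpoint, and move the player back to that transform with matching control rotation.
; Phantom ghost logic for recording, loading from a save and replaying movement remains, but is disconnected and never runs.
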(event Custom|Spawn
  (bind _playerstart (Variables|Default|GetPlayerStart))
  (bind _returnvalue (Transformation|GetActorTransform _playerstart))
  ;[0.07998 1 0] Begin play - Spawn character
  (Variables|Default|SetSpawnLoc _returnvalue)
  (bind _returnvalue_2 (Game|SpawnActorfromClass (Variables|Default|GetPlayerCharacter) _returnvalue "Undefined" 0 0))
  (bind _character (Class|BPiSpawning|ICharacterRef(Message) _returnvalue_2))
  (Variables|Default|SetPlayer _character)
  (Pawn|Possess (Game|GetPlayerController 0) _returnvalue_2)
  (Class|BPiSpawning|IStoreSpawnManager(Message) _returnvalue_2 self))

(event Custom|TriggerRecording)

(event Custom|LoopingRecording)

(event Custom|OpenGate)

(event Custom|CloseGate)

(event Custom|NewReset)

(event EventBeginPlay
  ;[0.07998 1 0] Begin play - Spawn character
  (bind _returnvalue (Actor|GetActorOfClass "/Game/TECH/Mitz/Blueprints/BP_PlayerStart.BP_PlayerStart_C"))
  (Utilities|IsValid _returnvalue
    (:Is%20Valid
      (Variables|Default|SetPlayerStart _returnvalue)
      (CallFunction|Spawn))))

(event EventIPlayerSpawn
  (bind _player (Variables|Default|GetPlayer))
  (bind _spawnloc (Variables|Default|GetSpawnLoc))
  ;[0.07998 1 0] Moves the player to the spawn and rotates the player
  (Transformation|SetActorLocation _player (.location _spawnloc) false false)
  (Pawn|SetControlRotation (Pawn|GetController _player) (.rotation _spawnloc)))

(event EventISetSpawnPoint
  (params (SpawnLoc :type Transform) (CurrentCheckpoint :type BP%20Check%20Point%20Object%20Reference))
  ;[0.07998 1 0] Store current spawn transform and spawn checkpoint
  (Variables|Default|SetSpawnLoc SpawnLoc)
  (Variables|Default|SetCurrent%20Checkpoint CurrentCheckpoint))

(fn ConstructionScript)

(fn FRecordPhantom)

(fn FReplayPhantom
  (params (CurrentSpawnedPhantom :type BP%20Phantom%20Character%20Object%20Reference)))

(fn FSpawnPhantom
  (params (CanSpawn :type Boolean)))

(fn FLoadGamePhantom)

(fn FCheckifSaveGameIsValid)

(fn ICharacterRef
  (return 0))

(fn IGetController
  (return 0))