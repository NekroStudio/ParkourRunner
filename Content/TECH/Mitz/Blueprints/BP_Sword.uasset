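; Sword weapon actor whose capsule hit box deals damage to non-player actors during its owner's attack.
; Attack-trace interface events toggle the collision and the owning Character's Blocking flag together.
; On overlap, it applies damage, then passes impact data from a debug-drawn forward line trace from the Character to its BPAttack for hit effects.
; An interface getter exposes the capsule half height, while the length update is empty.
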(event OnComponentBeginOverlap(SwordCollision)
  (params (OverlappedComponent :type Primitive%20Component%20Object%20Reference) (OtherActor :type Actor%20Object%20Reference) (OtherComp :type Primitive%20Component%20Object%20Reference) (OtherBodyIndex :type Integer) (bFromSweep :type Boolean) (SweepResult :type Hit%20Result%20Structure%20%28by%20ref%29))
  (bind _character (Variables|Default|GetCharacter))
  ;[1 1 1] Attack hit box for sword
  (Variables|Default|SetHitActor OtherActor)
  (Utilities|MIsPlayer OtherActor
    (:false
      (Utilities|IsValid _character
        (:Is%20Valid
          (bind (_impactpoint _impactnormal _hitcomponent) (CallFunction|FTraceforFX))
          (Game|Damage|ApplyDamage (Variables|Default|GetHitActor) 1.0 0 _character)
          (Default|ContinueAttackEffects (Variables|/Game/TECH/Jay/BP_BaseCharacter.BP_BaseCharacter_C|GetBP_Attack _character) _impactpoint _impactnormal _hitcomponent))))))

(event EventIAttackTraceON
  (params (Character :type BP%20Base%20Character%20Object%20Reference))
  ;[1 1 1] Toggle collision (alongside blocking)
  (Variables|Default|SetCharacter Character)
  (Collision|SetCollisionEnabled (Variables|Default|GetSwordCollision) "QueryAndPhysics")
  (Variables|/Game/TECH/Jay/BP_BaseCharacter.BP_BaseCharacter_C|Setblocking? (Variables|Default|GetCharacter) true))

(event EventIAttackTraceOFF
  ;[1 1 1] Toggle collision (alongside blocking)
  (Collision|SetCollisionEnabled (Variables|Default|GetSwordCollision) "NoCollision")
  (Variables|/Game/TECH/Jay/BP_BaseCharacter.BP_BaseCharacter_C|Setblocking? (Variables|Default|GetCharacter) false)
  (Variables|Default|SetHitActor 0))

(fn ConstructionScript)

(fn FTraceforFX
  (bind _character (Variables|Default|GetCharacter))
  (bind _returnvalue (Transformation|GetActorLocation _character))
  ;[1 1 1] Line trace for attack collision
  (bind (_outhit _returnvalue_2) (Collision|LineTraceByChannel _returnvalue (+ _returnvalue (* (Transformation|GetActorForwardVector _character) 1.5e+02)) "TraceTypeQuery4" false 0 "ForDuration"))
  (if _returnvalue_2
    (return (.ImpactPoint (Collision|BreakHitResult _outhit)) (.ImpactNormal (Collision|BreakHitResult _outhit)) (.HitComponent (Collision|BreakHitResult _outhit)))))

(fn FUpdateSwordLength)

(fn ICheckBlocking
  (return false))

(fn IGetKills
  (return 0))

(fn ISwordCollisionHalfHeight
  (return self (Variables|/Script/Engine.CapsuleComponent|GetCapsuleHalfHeight (Variables|Default|GetSwordCollision))))