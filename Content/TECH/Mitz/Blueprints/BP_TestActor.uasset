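; BP_TestActor is a test trigger that removes itself once the player touches it, using the killed-enemy save list to stay removed.
; On box overlap by the player, if unlisted, it reports itself to the GameMode as killed, saves the "Save1" slot object and destroys itself on success.
; On the InitEnemies interface event, it loads that slot and destroys itself if listed.
; Despite checkpoint comments, no spawn point is set here.
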(event OnComponentBeginOverlap(Box)
  (params (OverlappedComponent :type Primitive%20Component%20Object%20Reference) (OtherActor :type Actor%20Object%20Reference) (OtherComp :type Primitive%20Component%20Object%20Reference) (OtherBodyIndex :type Integer) (bFromSweep :type Boolean) (SweepResult :type Hit%20Result%20Structure%20%28by%20ref%29))
  ;[1 1 1] Saves the checkpoint
  ;;[1 1 1] Checks if the player is overlapping
  (Utilities|MIsPlayer OtherActor
    (:true
      ;;[1 1 1] Sets the spawn point in the spawn manager
      (bind _returnvalue (SaveGame|LoadGamefromSlot "Save1"))
      (bind _saveslot (Class|ISaveGame|IConvertSaveSlot(Message) _returnvalue))
      ;;[1 1 1] Checks if it is contained
      (if (not (Utilities|Array|ContainsItem (Variables|/Game/TECH/Mitz/Blueprints/BP_SaveGame.BP_SaveGame_C|GetKilledEnemies _saveslot) self))
        (Class|ISaveGame|IAddKilledEnemy(Message) (Game|GetGameMode) self)
        ;;[1 1 1] Saves the game and sets the spawn point and destroys the checkpoint
        (bind _returnvalue_2 (SaveGame|SaveGametoSlot _saveslot "Save1"))
        (if _returnvalue_2
          (Actor|DestroyActor))))))

(event EventIInitEnemies
  ;[1 1 1] Init
  ;;[1 1 1] Loads the save slot
  (bind _returnvalue (SaveGame|LoadGamefromSlot "Save1"))
  (bind _saveslot (Class|ISaveGame|IConvertSaveSlot(Message) _returnvalue))
  ;;[1 1 1] Checks if the check point is contained
  (if (Utilities|Array|ContainsItem (Variables|/Game/TECH/Mitz/Blueprints/BP_SaveGame.BP_SaveGame_C|GetKilledEnemies _saveslot) self)
    ;;[1 1 1] If it is destroy the check point
    (Actor|DestroyActor)))

(fn ConstructionScript)

(fn IConvertSaveSlot
  (return 0))